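; Player controller for the multiplayer lobby that loads the local player's account data and shows the lobby menu.
; On BeginPlay it registers five default loadouts with the GISS multiplayer system, then copies the account's name, background, level, rank icon and loadouts into its variables.
; It then creates the lobby widget with the mouse cursor visible.
; Player list updates forward to that widget, retrying on a short delay until it is valid.
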(event `self.ReceiveBeginPlay`
  (`/Engine/EditorBlueprintResources/ActorMacros.Switch Has Authority`
    (:`Authority`
      _)
    (:`Remote`
      _))
  (`self.GetAllUserAttributes`)
  (`self.CreateLobbyMenu`))

(event `CreateLobbyMenu`
  (set `self.bShowMouseCursor` true)
  (bind _returnvalue (`|CreateWidget` "/Game/GameplayAbilities/Maps/UtilityMaps/Blueprints/UI/WBP_LobbyMenu.WBP_LobbyMenu_C" self))
  (bind _output_get (set `self.LobbyMenu` _returnvalue))
  (`UserWidget.AddToViewport` _output_get 0))

(event `UpdateCurrentPlayers`
  (bind _lobbymenu (`self.LobbyMenu`))
  (`/Engine/EditorBlueprintResources/StandardMacros.IsValid` _lobbymenu :!label _label
    (:`Is Valid`
      (`/Game/GameplayAbilities/Maps/UtilityMaps/Blueprints/UI/WBP_LobbyMenu.UpdateCurrentPlayers` _lobbymenu))
    (:`Is Not Valid`
      (`KismetSystemLibrary.RetriggerableDelay` 0.1)
      (goto _label))))

(fn `GetAllUserAttributes`
  (locals (AccountInfo :type "BPUserOnlineAccount Structure"))
  (`GISS_Multiplayer.SetDefaultLoadouts` (subsystem `GISS_Multiplayer`) (`|MakeArray` "/Game/GameplayAbilities/Blueprints/UI/InfiniteWarfare/Loadout/DefaultLoadouts/Loadout_Assault.Loadout_Assault_C" "/Game/GameplayAbilities/Blueprints/UI/InfiniteWarfare/Loadout/DefaultLoadouts/Loadout_Predator.Loadout_Predator_C" "/Game/GameplayAbilities/Blueprints/UI/InfiniteWarfare/Loadout/DefaultLoadouts/Loadout_Phantom.Loadout_Phantom_C" "/Game/GameplayAbilities/Blueprints/UI/InfiniteWarfare/Loadout/DefaultLoadouts/Loadout_Stronghold.Loadout_Stronghold_C" "/Game/GameplayAbilities/Blueprints/UI/InfiniteWarfare/Loadout/DefaultLoadouts/Loadout_Outlaw.Loadout_Outlaw_C" :!type "MultiplayerLoadout Class Reference"))
  (bind _attributes (`GISS_Multiplayer.GetUserAccountAttributes` (subsystem `GISS_Multiplayer`)))
  (bind (_displayname _clanname _title _experience _level _prestige _rankicon _background _portrait _emblemicon _equippedcallingcards _loadouts) (break `AccountAttributes` _attributes))
  (setmembers `/Game/GameplayAbilities/Maps/UtilityMaps/Blueprints/Framework/ST_LobbyPlayerInfo` :`StructRef` (`self.PlayerLobbyInfo`) :`Name` _displayname :`PlayerBackground` _background :`Level` _level :`Rank` _rankicon)
  (set `self.Loadouts` _loadouts)
  (return))

(fn `UserConstructionScript`)