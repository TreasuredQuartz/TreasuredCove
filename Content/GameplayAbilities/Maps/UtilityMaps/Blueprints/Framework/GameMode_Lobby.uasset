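; Lobby game mode that registers joining and leaving players and maintains a shared multiplayer map pool from their map preferences.
; On login it notifies the lobby game state and adds the player's preferred maps; on logout it refreshes the player list and removes them.
; The pool maps each DT_MultiplayerMaps row to a preference count, incremented per player and deleted when it reaches zero.
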(event `self.ReceiveBeginPlay`)

(event `self.K2_PostLogin`
  (params (NewPlayer :type "PlayerController Object Reference"))
  (`KismetSystemLibrary.LogString` "GameMode: PostLogin")
  (bind _asplayer_controller_lobby (cast `/Game/GameplayAbilities/Maps/UtilityMaps/Blueprints/Framework/PlayerController_Lobby` NewPlayer))
  (`/Game/GameplayAbilities/Maps/UtilityMaps/Blueprints/Framework/GameState_Lobby.NewPlayerAddedToLobby` (cast `/Game/GameplayAbilities/Maps/UtilityMaps/Blueprints/Framework/GameState_Lobby` (`GameplayStatics.GetGameState`) :!pure true) _asplayer_controller_lobby)
  (`self.AddPlayerMapPoolToLobby` (`Controller.PlayerState` _asplayer_controller_lobby)))

(event `self.K2_OnLogout`
  (params (ExitingController :type "Controller Object Reference"))
  (bind _playerstate (`Controller.PlayerState` ExitingController))
  (`/Game/GameplayAbilities/Maps/UtilityMaps/Blueprints/Framework/GameState_Lobby.UpdateCurrentPlayers` (cast `/Game/GameplayAbilities/Maps/UtilityMaps/Blueprints/Framework/GameState_Lobby` (`GameplayStatics.GetGameState`) :!pure true))
  (`/Engine/EditorBlueprintResources/StandardMacros.IsValid` _playerstate
    (:`Is Valid`
      (`self.RemovePlayerMapPoolFromLobby` _playerstate))))

(event `self.K2_OnSetMatchState`
  (params (NewState :type Name)))

(fn `AddPlayerMapPoolToLobby`
  (params (NewPlayerState :type "PlayerState Object Reference"))
  (for _array_element (`/Game/GameplayAbilities/Maps/UtilityMaps/Blueprints/Framework/BP_PlayerState_Lobby.GetMapPreferences` (cast `/Game/GameplayAbilities/Maps/UtilityMaps/Blueprints/Framework/BP_PlayerState_Lobby` NewPlayerState :!pure true))
    (bind _returnvalue (`|GetDataTableRow` "/Game/Multiplayer/MultiplayerMaps/DT_MultiplayerMaps.DT_MultiplayerMaps" _array_element)
      (:`then`
        (`KismetSystemLibrary.LogString` (`KismetTextLibrary.Conv_TextToString` (`|FormatText` "Adding Map: {Name}" (`.MapName` (break `MultiplayerMapInfo` _returnvalue)))))
        (bind (_value _returnvalue_2) (`BlueprintMapLibrary.Map_Find` (`self.MultiplayerMapPool`) _returnvalue))
        (if _returnvalue_2
          (`BlueprintMapLibrary.Map_Add` (`self.MultiplayerMapPool`) _returnvalue (+ _value 1))
          (else
            (`BlueprintMapLibrary.Map_Add` (`self.MultiplayerMapPool`) _returnvalue 1)))))))

(fn `GetCurrentMapPool`
  (returns (MapPool :type "Map of MultiplayerMapInfo Structure to Integer"))
  (return (`self.MultiplayerMapPool`)))

(fn `RemovePlayerMapPoolFromLobby`
  (params (LeavingPlayer :type "PlayerState Object Reference"))
  (for _array_element (`/Game/GameplayAbilities/Maps/UtilityMaps/Blueprints/Framework/BP_PlayerState_Lobby.GetMapPreferences` (cast `/Game/GameplayAbilities/Maps/UtilityMaps/Blueprints/Framework/BP_PlayerState_Lobby` LeavingPlayer :!pure true))
    (bind _returnvalue (`|GetDataTableRow` "/Game/Multiplayer/MultiplayerMaps/DT_MultiplayerMaps.DT_MultiplayerMaps" _array_element)
      (:`then`
        (bind (_value _returnvalue_2) (`BlueprintMapLibrary.Map_Find` (`self.MultiplayerMapPool`) _returnvalue))
        (if _returnvalue_2
          (bind _returnvalue_3 (+ _value -1))
          (if (> _returnvalue_3 0)
            (`BlueprintMapLibrary.Map_Add` (`self.MultiplayerMapPool`) _returnvalue _returnvalue_3)
            (else
              (`BlueprintMapLibrary.Map_Remove` (`self.MultiplayerMapPool`) _returnvalue))))))))

(fn `UserConstructionScript`)