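; Lobby player state Blueprint that holds each player's profile display data, map preferences and map vote.
; On BeginPlay it initializes user account attributes through the multiplayer subsystem and copies them into lobby info (name, background, level, rank, clan) and player card structs.
; Vote events record a map index only while voting is allowed, and getters expose the lobby, portrait and map preference data.
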(event `self.ReceiveBeginPlay`
  (`KismetSystemLibrary.PrintString` "Player State: Begin Play")
  (`GISS_Multiplayer.InitializeUserAccountAttributes` (subsystem `GISS_Multiplayer`) (make `BPUserOnlineAccount`))
  (bind _attributes (`GISS_Multiplayer.GetUserAccountAttributes` (subsystem `GISS_Multiplayer`)))
  (bind (_displayname _clanname _title _experience _level _prestige _rankicon _background _portrait _emblemicon _equippedcallingcards) (break `AccountAttributes` _attributes))
  (setmembers `/Game/GameplayAbilities/Maps/UtilityMaps/Blueprints/Framework/ST_LobbyPlayerInfo` :`StructRef` (`self.PlayerInfo`) :`Name` _displayname :`PlayerBackground` _background :`Level` _level :`Rank` _rankicon :`ClanName` _clanname)
  (setmembers `/Game/GameplayAbilities/Maps/UtilityMaps/Blueprints/Framework/ST_PlayerCardInfo` :`StructRef` (`self.PlayerPortrait`) :`CallingCards` _equippedcallingcards :`Portrait` _portrait :`Title` _title))

(event `CastVote`
  (params (Index :type Integer))
  (if (`self.bCanVote`)
    (set `self.MapVote` Index)))

(event `SetCanVote`
  (params (CanVote :type Boolean))
  (set `self.bCanVote` CanVote))

(fn `GetLobbyInfo`
  (returns (PlayerInfo :type "/Game/GameplayAbilities/Maps/UtilityMaps/Blueprints/Framework/ST_LobbyPlayerInfo Structure"))
  (return (`self.PlayerInfo`)))

(fn `GetMapPreferences`
  (returns (OutPreferrences :type "Array of Name"))
  (return (`self.MapPreferences`)))

(fn `GetPortraitInfo`
  (returns (PlayerPortrait :type "/Game/GameplayAbilities/Maps/UtilityMaps/Blueprints/Framework/ST_PlayerCardInfo Structure"))
  (return (`self.PlayerPortrait`)))

(fn `UserConstructionScript`)