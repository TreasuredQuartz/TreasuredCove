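; Tower of Owen dungeon actor: a player pawn overlapping the entrance trigger enters a chain of stacked rooms, shown one at a time.
; BeginPlay spawns and attaches the room actors, binding their next/previous events to room switching; going back from the first room exits.
; Entering restricts movement moves, locks look and viewpoint, and switches to the tower's spring-arm camera attached to the player.
; Local players also get fog and a hidden exterior; exiting reverses most changes.
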(event `self.ReceiveBeginPlay`
  (`self.GenerateRooms`))

(event `self.EntranceTrigger.OnComponentBeginOverlap`
  (params (OverlappedComponent :type "PrimitiveComponent Object Reference") (OtherActor :type "Actor Object Reference") (OtherComp :type "PrimitiveComponent Object Reference") (OtherBodyIndex :type Integer) (bFromSweep :type Boolean) (SweepResult :type "HitResult Structure (by ref)"))
  (`KismetSystemLibrary.PrintString` (`KismetSystemLibrary.GetDisplayName` OtherComp))
  (bind _aspawn (cast `Pawn` OtherActor))
  (if (`Pawn.IsPlayerControlled` _aspawn)
    (`self.EnterDungeon` _aspawn)))

(fn `DisableCharacterMovementOptions`
  (params (User :type "Object Object Reference"))
  (bind _asgacharacter (cast `GACharacter` User :!pure true))
  (`GACharacter.SetJumpAllowed` _asgacharacter false)
  (`GACharacter.SetWallRunAllowed` _asgacharacter false)
  (`GACharacter.SetClimbAllowed` _asgacharacter false)
  (`GACharacter.SetSlideAllowed` _asgacharacter false))

(fn `EnableCharacterMovementOptions`
  (params (User :type "Actor Object Reference"))
  (bind _asgacharacter (cast `GACharacter` User :!pure true))
  (`GACharacter.SetJumpAllowed` _asgacharacter true)
  (`GACharacter.SetWallRunAllowed` _asgacharacter true)
  (`GACharacter.SetClimbAllowed` _asgacharacter true)
  (`GACharacter.SetSlideAllowed` _asgacharacter true))

(fn `EnterDungeon`
  (params (`New User` :type "Pawn Object Reference"))
  (locals (NewUserIndex :type Integer :default 0))
  (bind _outsidemesh (`self.OutsideMesh`))
  (bind _springarm (`self.SpringArm`))
  (`|ExecutionSequence`
    (:`then_0`
      (bind _returnvalue (`KismetArrayLibrary.Array_Add` (`self.Users`) (`local.New User`)))
      (set `local.NewUserIndex` _returnvalue))
    (:`then_1`
      (`self.DisableCharacterMovementOptions` (`local.New User`))
      (bind _asplayer_controller (cast `PlayerController` (`Pawn.GetController` (`local.New User`))))
      (`Controller.SetIgnoreLookInput` _asplayer_controller true)
      (`Controller.SetControlRotation` _asplayer_controller (`KismetMathLibrary.ComposeRotators` (`SceneComponent.K2_GetComponentRotation` (`self.DefaultSceneRoot`)) (struct :`Yaw` 180.0)))
      (`ActorComponent.Activate` (`self.Camera`) false)
      (`PlayerController.SetViewTargetWithBlend` _asplayer_controller self 0.0 "VTBlend_Linear" 0.0 false)
      (bind _asgacharacter (cast `GACharacter` (`local.New User`))
        (:`then`
          (`GACharacter.ChangeViewpoint` _asgacharacter false)
          (set `GACharacter.bLockedViewpoint` true _asgacharacter))
        (:`CastFailed`
          _))
      (`SceneComponent.K2_AttachToComponent` _springarm (`Actor.RootComponent` (`local.New User`)) "None" "SnapToTarget" "KeepRelative" "KeepRelative" true)
      (set `SceneComponent.bAbsoluteRotation` true _springarm))
    (:`then_2`
      (if (`Pawn.IsLocallyControlled` (`local.New User`))
        (`|ExecutionSequence`
          (:`then_0`
            (`/Game/GameplayAbilities/Blueprints/Environment/Planet/GA_SunSky.SetViewDistanceFog` :`self` (`self.SunSky`) :`Blend` 1.0 :`FogStrength` 1.0 :`FogStart` 1500.0)
            (`PrimitiveComponent.SetCollisionEnabled` _outsidemesh "NoCollision")
            (`SceneComponent.SetHiddenInGame` _outsidemesh true false))
          (:`then_1`
            (`self.EnterRoom` (`local.New User`) 1)))))))

(fn `EnterRoom`
  (params (InUser :type "Pawn Object Reference") (Room :type Byte))
  (set `self.CurrentLevel` (`local.Room`))
  (`/Game/GameplayAbilities/Maps/MainWorld/TowerOfOwen/BP_TowerOfOwen_Room.EnterRoom` (`|GetArrayItem` (`self.Rooms`) (- (`KismetMathLibrary.Conv_ByteToInt` (`local.Room`)) 1)) InUser)
  (`self.UpdateCurrentLevelVisibility`))

(fn `ExitDungeon`
  (params (OldUser :type "Pawn Object Reference"))
  (bind _olduser (`local.OldUser`))
  (bind _outsidemesh (`self.OutsideMesh`))
  (bind _springarm (`self.SpringArm`))
  (`|ExecutionSequence`
    (:`then_0`
      (`KismetArrayLibrary.Array_RemoveItem` (`self.Users`) (`local.OldUser`)))
    (:`then_1`
      (`self.EnableCharacterMovementOptions` (`local.OldUser`))
      (`self.K2_SetActorLocation` (`local.OldUser`) (`SceneComponent.K2_GetComponentLocation` (`self.EntranceLocation`)) false true))
    (:`then_2`
      (bind _asplayer_controller (cast `PlayerController` (`Pawn.GetController` _olduser)))
      (`PlayerController.SetViewTargetWithBlend` _asplayer_controller _olduser 0.0 "VTBlend_Linear" 0.0 false)
      (`Controller.SetControlRotation` _asplayer_controller (`KismetMathLibrary.ComposeRotators` (`self.K2_GetActorRotation` (`local.OldUser`)) (struct :`Yaw` 180.0)))
      (`Controller.SetIgnoreLookInput` _asplayer_controller false)
      (`ActorComponent.Deactivate` (`self.Camera`))
      (`SceneComponent.K2_DetachFromComponent` _springarm "KeepRelative" "KeepRelative" "KeepRelative" true)
      (set `SceneComponent.bAbsoluteRotation` true _springarm))
    (:`then_3`
      (if (`Pawn.IsLocallyControlled` (`local.OldUser`))
        (`/Game/GameplayAbilities/Blueprints/Environment/Planet/GA_SunSky.SetViewDistanceFog` :`self` (`self.SunSky`))
        (`self.SetActorHiddenInGame` (`|GetArrayItem` (`self.Rooms`) (`KismetMathLibrary.Conv_ByteToInt` (`self.CurrentLevel`))) true)
        (`PrimitiveComponent.SetCollisionEnabled` _outsidemesh "QueryAndPhysics")
        (`SceneComponent.SetHiddenInGame` _outsidemesh false false)))))

(fn `GenerateRooms`
  (`KismetArrayLibrary.Array_Clear` (`self.Rooms`))
  (for _index (range 1 (+ (`self.MaxRoomCount`) 1))
    (bind _returnvalue (`|SpawnActorFromClass` (select `int` _index :`0` null :`1` "/Game/GameplayAbilities/Maps/MainWorld/TowerOfOwen/TO_Room_01.TO_Room_01_C" :`2` "/Game/GameplayAbilities/Maps/MainWorld/TowerOfOwen/TO_Room_02.TO_Room_02_C" :`3` "/Game/GameplayAbilities/Maps/MainWorld/TowerOfOwen/TO_Room_03.TO_Room_03_C" :`4` "/Game/GameplayAbilities/Maps/MainWorld/TowerOfOwen/TO_Room_04.TO_Room_04_C" :`5` "/Game/GameplayAbilities/Maps/MainWorld/TowerOfOwen/TO_Room_05.TO_Room_05_C" :`6` "/Game/GameplayAbilities/Maps/MainWorld/TowerOfOwen/TO_Room_06.TO_Room_06_C" :`7` "/Game/GameplayAbilities/Maps/MainWorld/TowerOfOwen/TO_Room_07.TO_Room_07_C" :`8` "/Game/GameplayAbilities/Maps/MainWorld/TowerOfOwen/TO_Room_08.TO_Room_08_C" :`9` "/Game/GameplayAbilities/Maps/MainWorld/TowerOfOwen/TO_Room_09.TO_Room_09_C" :`10` "/Game/GameplayAbilities/Maps/MainWorld/TowerOfOwen/TO_Room_10.TO_Room_10_C" :`11` "/Game/GameplayAbilities/Maps/MainWorld/TowerOfOwen/TO_Room_11.TO_Room_11_C" :!type "Actor Class Reference") (`self.GetTransform`) "AlwaysSpawn" "SelectDefaultAtRuntime" self null))
    (bind _asbp_tower_of_owen_room (cast `/Game/GameplayAbilities/Maps/MainWorld/TowerOfOwen/BP_TowerOfOwen_Room` _returnvalue :!pure true))
    (`KismetArrayLibrary.Array_Add` (`self.Rooms`) _asbp_tower_of_owen_room)
    (`self.K2_AttachToActor` _asbp_tower_of_owen_room self "None" "KeepWorld" "KeepWorld" "KeepWorld" true)
    (add `/Game/GameplayAbilities/Maps/MainWorld/TowerOfOwen/BP_TowerOfOwen_Room.MoveToNextRoom` _asbp_tower_of_owen_room (`|CreateDelegate` :!event `MoveToNextRoom`))
    (add `/Game/GameplayAbilities/Maps/MainWorld/TowerOfOwen/BP_TowerOfOwen_Room.MoveToPreviousRoom` _asbp_tower_of_owen_room (`|CreateDelegate` :!event `MoveToPreviousRoom`))))

(fn `MoveToNextRoom`
  (params (User :type "Pawn Object Reference"))
  (`self.EnterRoom` (`local.User`) (+ (`self.CurrentLevel`) 1)))

(fn `MoveToPreviousRoom`
  (params (User :type "Pawn Object Reference"))
  (bind _currentlevel (`self.CurrentLevel`))
  (bind _user (`local.User`))
  (if (== _currentlevel 1)
    (`self.ExitDungeon` _user)
    (else
      (`self.EnterRoom` _user (- _currentlevel 1)))))

(fn `UpdateCurrentLevelVisibility`
  (for (_array_element _array_index) (`self.Rooms`)
    (bind _returnvalue (!= _array_index (- (`self.CurrentLevel`) 1)))
    (`self.SetActorHiddenInGame` _array_element _returnvalue)
    (`self.SetActorEnableCollision` (not _returnvalue))))

(fn `UserConstructionScript`)