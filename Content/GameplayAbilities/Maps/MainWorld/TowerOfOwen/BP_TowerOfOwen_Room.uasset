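; Tower of Owen room actor that moves a pawn in and out through enter and exit triggers.
; Two timelines lerp the pawn between trigger and end-location transforms, playing in reverse for backtracking.
; Forward exit completion calls the move to the next room, reversed entry the previous one after a short delay.
; Transition events block player move input and retriggering, and toggle trigger collision.
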(event `OnRoom_BeginEnter`
  (bind _movingpawn (`self.MovingPawn`))
  (bind (_asplayer_controller _bsuccess) (cast `PlayerController` (`Pawn.GetController` _movingpawn) :!pure true))
  (set `self.bPerformingTransition` true :!label _label)
  (`/Engine/EditorBlueprintResources/StandardMacros.IsValid` _movingpawn
    (:`Is Valid`
      (if _bsuccess
        (if (not (`Controller.IsMoveInputIgnored` _asplayer_controller))
          (`Controller.SetIgnoreMoveInput` _asplayer_controller true))
        (else
          (`KismetSystemLibrary.PrintString` "Shit failed" true true (struct :`G` 0.66 :`B` 1.0 :`A` 1.0) 5.0 :!label _label_2))))
    (:`Is Not Valid`
      (goto _label_2))))

(event `OnRoom_BeginExit`
  (`self.SetEnableOverlapEvents` "NoCollision")
  (goto _label))

(event `OnRoom_EndEnter`
  (bind _movingpawn (`self.MovingPawn`))
  (bind (_asplayer_controller _bsuccess) (cast `PlayerController` (`Pawn.GetController` _movingpawn) :!pure true))
  (`self.SetEnableOverlapEvents` "QueryOnly")
  (set `self.bPerformingTransition` false :!label _label_3)
  (`/Engine/EditorBlueprintResources/StandardMacros.IsValid` _movingpawn
    (:`Is Valid`
      (if _bsuccess
        (`Controller.ResetIgnoreMoveInput` _asplayer_controller)
        (else
          (`KismetSystemLibrary.PrintString` "Shit failed" true true (struct :`G` 0.66 :`B` 1.0 :`A` 1.0) 5.0 :!label _label_4))))
    (:`Is Not Valid`
      (goto _label_4))))

(event `OnRoom_EndExit`
  (goto _label_3))

(event `EnterRoom`
  (params (InPawn :type "Pawn Object Reference"))
  ;[1 1 1] Transition movement
  (if (not (`KismetSystemLibrary.IsValid` InPawn))
    (`KismetSystemLibrary.PrintString` "In Room Pawn cast failed" true true (struct :`G` 0.66 :`B` 1.0 :`A` 1.0) 5.0))
  (set `self.MovingPawn` InPawn)
  (`self.OnRoom_BeginEnter`)
  (bind (_direction _leveltransitiontrack) (`Timeline|LevelEnterTimeline` :!via `PlayFromStart` :!label _label_5)
    (:`Update`
      (`self.K2_SetActorTransform` (`self.MovingPawn`) (`KismetMathLibrary.TLerp` (`self.GetEnterStartTransform`) (`self.GetEnterEndTransform`) _leveltransitiontrack) false true))
    (:`Finished`
      (`self.OnRoom_EndEnter`)
      (`KismetSystemLibrary.Delay` 0.5)
      (switch `ETimelineDirection` _direction
        (:`Forward`
          _)
        (:`Backward`
          (`self.MoveToPreviousRoom` (`self.MovingPawn`))))
      (set `self.MovingPawn` null))))

(event `ReturnFrom`
  (params (InPawn :type "Pawn Object Reference"))
  ;[1 1 1] Transition movement
  (if (`KismetSystemLibrary.IsValid` InPawn)
    (set `self.MovingPawn` InPawn)
    (`self.OnRoom_BeginEnter`)
    (goto _label_5 :!via `ReverseFromEnd`)))

(event `ExitRoom`
  (params (InPawn :type "Pawn Object Reference"))
  ;[1 1 1] Transition movement
  (if (`KismetSystemLibrary.IsValid` InPawn)
    (set `self.MovingPawn` InPawn)
    (`self.OnRoom_BeginExit`)
    (bind (_direction _leveltransitiontrack) (`Timeline|LevelExitTimeline` :!via `PlayFromStart` :!label _label_6)
      (:`Update`
        (`self.K2_SetActorTransform` (`self.MovingPawn`) (`KismetMathLibrary.TLerp` (`self.GetExitStartTransform`) (`self.GetExitEndTransform`) _leveltransitiontrack) false false))
      (:`Finished`
        (`self.OnRoom_EndExit`)
        (switch `ETimelineDirection` _direction
          (:`Forward`
            (`self.MoveToNextRoom` (`self.MovingPawn`)))
          (:`Backward`
            _))
        (set `self.MovingPawn` null)))))

(event `ReturnTo`
  (params (InPawn :type "Pawn Object Reference"))
  ;[1 1 1] Transition movement
  (if (`KismetSystemLibrary.IsValid` InPawn)
    (set `self.MovingPawn` InPawn)
    (`self.OnRoom_BeginExit`)
    (goto _label_6 :!via `ReverseFromEnd`)))

(event `self.EnterTrigger.OnComponentBeginOverlap`
  (params (OverlappedComponent :type "PrimitiveComponent Object Reference") (OtherActor :type "Actor Object Reference") (OtherComp :type "PrimitiveComponent Object Reference") (OtherBodyIndex :type Integer) (bFromSweep :type Boolean) (SweepResult :type "HitResult Structure (by ref)"))
  (cast `/Game/GameplayAbilities/Maps/MainWorld/TowerOfOwen/BP_Room` OtherActor
    (:`CastFailed`
      (if (not (`self.bPerformingTransition`))
        (bind _aspawn (cast `Pawn` OtherActor))
        (`self.ReturnFrom` _aspawn)))))

(event `self.ExitTrigger.OnComponentBeginOverlap`
  (params (OverlappedComponent :type "PrimitiveComponent Object Reference") (OtherActor :type "Actor Object Reference") (OtherComp :type "PrimitiveComponent Object Reference") (OtherBodyIndex :type Integer) (bFromSweep :type Boolean) (SweepResult :type "HitResult Structure (by ref)"))
  (cast `/Game/GameplayAbilities/Maps/MainWorld/TowerOfOwen/BP_Room` OtherActor
    (:`CastFailed`
      (if (not (`self.bPerformingTransition`))
        (bind _aspawn (cast `Pawn` OtherActor))
        (`self.ExitRoom` _aspawn)))))

(fn `GetEnterEndTransform`
  (returns (Transform :type "Transform Structure"))
  (return (`SceneComponent.K2_GetComponentToWorld` (`self.EnterEndLocation`))))

(fn `GetEnterStartTransform`
  (returns (Transform :type "Transform Structure"))
  (return (`SceneComponent.K2_GetComponentToWorld` (`self.EnterTrigger`))))

(fn `GetExitEndTransform`
  (returns (Transform :type "Transform Structure"))
  (return (`SceneComponent.K2_GetComponentToWorld` (`self.ExitEndLocation`))))

(fn `GetExitStartTransform`
  (returns (Transform :type "Transform Structure"))
  (return (`SceneComponent.K2_GetComponentToWorld` (`self.ExitTrigger`))))

(fn `SetEnableOverlapEvents`
  (params (NewType :type "ECollisionEnabled Enum" :default "NoCollision"))
  (`PrimitiveComponent.SetCollisionEnabled` (`self.EnterTrigger`) NewType)
  (`PrimitiveComponent.SetCollisionEnabled` (`self.ExitTrigger`) NewType))

(fn `UserConstructionScript`)