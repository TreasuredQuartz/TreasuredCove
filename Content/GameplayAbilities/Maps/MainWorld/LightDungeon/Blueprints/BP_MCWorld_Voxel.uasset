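; Voxel world actor for the LightDungeon map that places voxels as randomized instanced static meshes.
; The construction script clears existing instances, then runs the parent's construction script.
; AddVoxelInstance adds an instance half a voxel below the given location, with X/Y jitter and per-axis scale drawn from a random stream and bounded by voxel size.
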(event `self.AddVoxelInstance`
  (params (Location :type "Vector Structure") (InstanceType :type Integer))
  (bind _randomstream (`self.RandomStream`))
  (bind _voxelsize (`self.VoxelSize`))
  (bind _returnvalue (`KismetMathLibrary.RandomFloatInRangeFromStream` _randomstream 4.0 (* (`self.VoxelSize`) 0.05)))
  (`InstancedStaticMeshComponent.AddInstance` (`self.InstancedStaticMesh`) (`KismetMathLibrary.MakeTransform` (`KismetMathLibrary.MakeVector` (+ (.x Location) (/ (* (* (- (`KismetMathLibrary.RandomFloatFromStream` _randomstream) 0.5) 2.0) _voxelsize) (/ _returnvalue 2.0))) (+ (.y Location) (/ (* (* (- (`KismetMathLibrary.RandomFloatFromStream` _randomstream) 0.5) 2.0) _voxelsize) (/ _returnvalue 2.0))) (- (.z Location) (`self.VoxelSizeHalf`) 0.0)) (struct) (`KismetMathLibrary.MakeVector` _returnvalue _returnvalue _returnvalue)) false))

(fn `UserConstructionScript`
  (`InstancedStaticMeshComponent.ClearInstances` (`self.InstancedStaticMesh`))
  (`parent.UserConstructionScript`))