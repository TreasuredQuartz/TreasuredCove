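; Room Blueprint for the King's Bedroom in the Quartz Palace dungeon, which sets up its entrances at runtime.
; On BeginPlay, it treats three courtyard door-frame components as placeholders, spawning a FrontEntrance actor at each one's world transform.
; Each spawned entrance attaches to the Entrances component with its world transform kept, and the placeholder is destroyed.
; The construction script only calls the parent room's version.
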(event `self.ReceiveBeginPlay`
  (for _array_element (`|MakeArray` (`self.SM_CourtyardDoorFrame`) (`self.SM_CourtyardDoorFrame1`) (`self.SM_CourtyardDoorFrame2`))
    (bind _returnvalue (`|SpawnActorFromClass` "/Game/GameplayAbilities/Maps/MainWorld/QuartzDungeon/Blueprints/Palace/Tools/FrontEntrance.FrontEntrance_C" (`SceneComponent.K2_GetComponentToWorld` _array_element) "AlwaysSpawn" "OverrideRootScale" null null))
    (`self.K2_AttachToComponent` _returnvalue (`self.Entrances`) "None" "KeepWorld" "KeepWorld" "KeepWorld" true)
    (`ActorComponent.K2_DestroyComponent` _array_element)))

(fn `UserConstructionScript`
  (`parent.UserConstructionScript`))