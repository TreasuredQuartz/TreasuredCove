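; Hex tile selector for the hex city builder that shows selection state by color and stores a tile index and grid.
; BeginPlay creates dynamic materials for the selector mesh and an emissive sphere, leaving the sphere cyan.
; ChangeSelected tints both red when selected or blue otherwise, creating the sphere material if missing.
; ChangeIndex only stores the new index and grid.
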(event `self.ReceiveBeginPlay`
  (bind _returnvalue (`PrimitiveComponent.CreateDynamicMaterialInstance` (`self.HexTileSelector`) 0 "/Game/GameplayAbilities/Blueprints/Abilities/HexCityBuilder/HexTiles/M_HexSelector.M_HexSelector" "None"))
  (set `self.MID` _returnvalue)
  (`self.ChangeSelected` (`self.bSelected`))
  (bind _returnvalue_2 (`PrimitiveComponent.CreateDynamicMaterialInstance` (`self.Sphere`) 0 "/Game/GameplayAbilities/Materials/Originals/M_OnlyEmissive.M_OnlyEmissive" "Light"))
  (set `self.LightMID` _returnvalue_2)
  (`MaterialInstanceDynamic.SetScalarParameterValue` (`self.LightMID`) "Intensity" 10.0)
  (`MaterialInstanceDynamic.SetVectorParameterValue` (`self.LightMID`) "Color" (struct :`G` 0.753621 :`B` 1.0 :`A` 1.0)))

(event `ChangeIndex`
  (params (NewIndex :type Integer) (NewGrid :type "HexGrid Object Reference"))
  (set `self.SelectedIndex` NewIndex)
  (set `self.SelectedGrid` NewGrid))

(event `ChangeSelected`
  (params (bSelected :type Boolean))
  (bind _output_get (set `self.bSelected` bSelected))
  (`MaterialInstanceDynamic.SetVectorParameterValue` (`self.MID`) "Color" (`KismetMathLibrary.SelectColor` (struct :`R` 1.0 :`A` 1.0) (struct :`R` 0.191202 :`G` 0.450786 :`B` 1.0 :`A` 1.0) _output_get))
  (`self.LightMID`
    (:`then`
      _)
    (:`else`
      (bind _returnvalue (`PrimitiveComponent.CreateDynamicMaterialInstance` (`self.Sphere`) 0 "/Game/GameplayAbilities/Materials/Originals/M_OnlyEmissive.M_OnlyEmissive" "Light"))
      (set `self.LightMID` _returnvalue)
      (`MaterialInstanceDynamic.SetScalarParameterValue` (`self.LightMID`) "Intensity" 10.0)))
  (`MaterialInstanceDynamic.SetVectorParameterValue` (`self.LightMID`) "Color" (`KismetMathLibrary.SelectColor` (struct :`R` 1.0 :`A` 1.0) (struct :`R` 0.191202 :`G` 0.450786 :`B` 1.0 :`A` 1.0) (`self.bSelected`))))

(event `self.ReceiveTick`
  (params (DeltaSeconds :type "Float (single-precision)")))

(fn `UserConstructionScript`)