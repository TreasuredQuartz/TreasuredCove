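; Tile selector for the hex city builder that resolves which hex tile lies under the player's mouse cursor.
; BPCheckSelectingTile deprojects the owning controller's mouse position and line traces along that ray on a custom game trace channel.
; When the hit actor is a HexGrid, it stores the grid and the hit item index, then returns the grid's tile for that index.
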(fn `BP_CheckSelectingTile`
  (returns (ReturnValue :type "HexTile Object Reference"))
  (locals (LocStart :type "Vector Structure") (LocEnd :type "Vector Structure") (HitIndex :type Integer :default 0) (HitHexGrid :type "HexGrid Object Reference"))
  (bind (_outhit _returnvalue) (`self.WorldSingleLineTrace` (`local.LocStart`) (`local.LocEnd`) "ECC_GameTraceChannel2"))
  (bind (_worldlocation _worlddirection) (`PlayerController.DeprojectMousePositionToWorld` (`self.OwningController`)))
  (bind (_bblockinghit _binitialoverlap _time _distance _location _impactpoint _normal _impactnormal _physmat _hitactor _hitcomponent _hitbonename _bonename _hititem) (`GameplayStatics.BreakHitResult` _outhit))
  (bind _output_get (set `local.LocStart` _worldlocation))
  (set `local.LocEnd` (+ _output_get (* _worlddirection (`self.LineTraceLength`))))
  (if _returnvalue
    (bind _ashex_grid (cast `HexGrid` _hitactor))
    (bind _output_get_2 (set `local.HitHexGrid` _ashex_grid))
    (bind _output_get_3 (set `local.HitIndex` _hititem))
    (return (`HexGrid.GetTileFromIndex` _output_get_2 _output_get_3))))