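; Game state Blueprint that sets the game clock's speed at BeginPlay and can hand a set of items to the player.
; SetPlayerInventory casts the first player's pawn to BP_Character and has it pick up each item passed in.
; A disconnected chain that would spawn the configured starting items after a short delay and feed them to SetPlayerInventory never runs.
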(event `self.ReceiveBeginPlay`
  (`GameTimeInterface.UpdateGameSpeed` (`self.GameClock`) 0.5))

(event `SetPlayerInventory`
  (params (NewInventory :type "Array of GAActor Object Reference"))
  (bind _asbp_character (cast `/Game/GameplayAbilitiesBP/Blueprint/Actors/Characters/BP_Character` (`GameplayStatics.GetPlayerCharacter` 0)))
  (for _array_element NewInventory
    (`GACharacter.PickupItem` _asbp_character _array_element)))

(fn `UserConstructionScript`)