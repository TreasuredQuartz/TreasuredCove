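; Pause Studio pawn that the player controller possesses on enter, presenting a hex-tile grid with an orbit camera, and hands control back on exit.
; It spawns the grid manager, rotates the spring arm on right-drag, and scales spotlight intensity with wheel zoom.
; Mouse traces drive hover and selection marker actors and tile events; selecting halts the RotatingMovement spin, deselecting re-targets it.
; Fog of war and move/look axes are empty stubs.
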(event `self.ReceiveTick`
  (params (DeltaSeconds :type "Float (single-precision)"))
  ;[1 1 1] Begin Play And Tick
  (`self.RotateCamera` DeltaSeconds)
  (`self.HoverOverTiles`))

(event `self.ReceiveBeginPlay`
  ;[1 1 1] Begin Play And Tick
  (bind _output_get (set `self.OwningPawn` (cast `Pawn` (`self.GetOwner`) :!pure true)))
  (set `self.OwningControler` (cast `PlayerController` (`self.GetController` _output_get) :!pure true))
  (`self.InitializeGrid`)
  (`self.InitializeFogOfWar`)
  (set `self.CameraRotation` (`SceneComponent.RelativeRotation` (`self.SpringArm`))))

(event `InitializeFogOfWar`)

(event `self.OnEnter`
  ;[1 1 1] Pause Studio
  (`parent.OnEnter`)
  (`Controller.Possess` (`self.OwningControler`) self)
  (`self.SetActorHiddenInGame` (`self.HexManager`) true))

(event `self.OnExit`
  ;[1 1 1] Pause Studio
  (`parent.OnExit`)
  (`Controller.Possess` (`self.OwningControler`) (`self.OwningPawn`)))

(event `InputAxis|Move Forward / Backward`
  (params (AxisValue :type "Float (single-precision)"))
  ;[1 1 1] Inputs
  (if (!= AxisValue 0.0)
    _))

(event `InputAxis|LookRight`
  (params (AxisValue :type "Float (single-precision)"))
  ;[1 1 1] Inputs
  (if (!= AxisValue 0.0)
    _))

(event `InputAction|Pause`
  (params (Key :type "Key Structure"))
  ;[1 1 1] Inputs
  (:`Pressed`
    (`self.OnExit`)))

(event `InputAxis|LookUp`
  (params (AxisValue :type "Float (single-precision)"))
  ;[1 1 1] Inputs
  (if (!= AxisValue 0.0)
    _))

(event `InputAxisKey|MouseWheelAxis`
  (params (AxisValue :type "Float (single-precision)"))
  ;[1 1 1] Inputs
  (`self.ZoomCamera` AxisValue))

(event `Key|RightMouseButton`
  (params (Key :type "Key Structure"))
  ;[1 1 1] Inputs
  (:`Pressed`
    (set `self.bIsRightMouseButtonDown` true)
    (`self.SetCurrentMousePosition`))
  (:`Released`
    (set `self.bIsRightMouseButtonDown` false)))

(event `Key|LeftMouseButton`
  (params (Key :type "Key Structure"))
  ;[1 1 1] Inputs
  (:`Pressed`
    (`/Engine/EditorBlueprintResources/StandardMacros.IsValid` (`self.HexTileSelector`)
      (:`Is Valid`
        (`self.SelectedTile`)))))

(fn `ChangeHoveredTile`
  (params (InHit :type "HitResult Structure"))
  (locals (LocIndex :type Integer :default 0) (LocGrid :type "HexGrid Object Reference") (SpawnTransform :type "Transform Structure"))
  (bind (_bblockinghit _binitialoverlap _time _distance _location _impactpoint _normal _impactnormal _physmat _hitactor _hitcomponent _hitbonename _bonename _hititem) (`GameplayStatics.BreakHitResult` InHit))
  (bind _hextileselector (`self.HexTileSelector`))
  (bind _hextileselector_2 (`self.HexTileSelector`))
  (if _bblockinghit
    (`/Engine/EditorBlueprintResources/StandardMacros.IsValid` (`self.HexTileSelector`)
      (:`Is Valid`
        _)
      (:`Is Not Valid`
        (bind _returnvalue (`|SpawnActorFromClass` "/Game/GameplayAbilities/Blueprints/Abilities/HexCityBuilder/HexTiles/BP_TileSelector.BP_TileSelector_C" (`local.SpawnTransform`) "AlwaysSpawn" "OverrideRootScale" null 0 false null null))
        (bind _output_get (set `self.HexTileSelector` _returnvalue))
        (`self.K2_AttachToComponent` _output_get (`self.Scene`) "None" "KeepWorld" "KeepWorld" "KeepWorld" true)))
    (set `local.LocIndex` _hititem)
    (set `local.LocGrid` (cast `HexGrid` _hitactor :!pure true))
    (set `local.SpawnTransform` (`HexGrid.GetTileCollisionTransform` (`local.LocGrid`) (`local.LocIndex`)))
    (`self.K2_SetActorRelativeTransform` _hextileselector_2 (`local.SpawnTransform`) false true)
    (`/Game/GameplayAbilities/Blueprints/Abilities/HexCityBuilder/HexTiles/BP_TileSelector.ChangeIndex` _hextileselector_2 (`local.LocIndex`) (`local.LocGrid`))
    (`self.SetActorHiddenInGame` _hextileselector_2 false)
    (`self.OnHoveredTile` (`local.LocIndex`))
    (`HexGrid.SetTileVertexColor` (`local.LocGrid`) (`self.HoveredColor`) (make `HexCoord`))
    (else
      (`/Engine/EditorBlueprintResources/StandardMacros.IsValid` _hextileselector
        (:`Is Valid`
          (`self.SetActorHiddenInGame` _hextileselector true)
          (`HexGrid.SetTileVertexColor` (`/Game/GameplayAbilities/Blueprints/Abilities/HexCityBuilder/HexTiles/BP_TileSelector.SelectedGrid` _hextileselector) (`self.NormalColor`) (make `HexCoord`))
          (set `/Game/GameplayAbilities/Blueprints/Abilities/HexCityBuilder/HexTiles/BP_TileSelector.SelectedIndex` -1 _hextileselector)
          (`self.OnUnHoveredTile`))))))

(fn `CreateDynamicBrushMaterial`)

(fn `HoverOverTiles`
  (locals (LocStart :type "Vector Structure" :default (0.0 0.0 0.0)) (LocEnd :type "Vector Structure"))
  (bind (_worldlocation _worlddirection) (`PlayerController.DeprojectMousePositionToWorld` (`self.OwningControler`)))
  (if (not (`self.bIsRightMouseButtonDown`))
    (`/Engine/EditorBlueprintResources/StandardMacros.IsValid` (`self.GetController`)
      (:`Is Valid`
        (bind _output_get (set `local.LocStart` _worldlocation))
        (set `local.LocEnd` (+ _output_get (* _worlddirection (`SpringArmComponent.TargetArmLength` (`self.SpringArm`)))))
        (bind _outhit (`KismetSystemLibrary.LineTraceSingleForObjects` (`local.LocStart`) (`local.LocEnd`) (`|MakeArray` "ObjectTypeQuery8" :!type "EObjectTypeQuery Enum") true))
        (`self.ChangeHoveredTile` _outhit)))))

(fn `InitializeGrid`
  (`/Engine/EditorBlueprintResources/StandardMacros.IsValid` (`self.HexManager`)
    (:`Is Valid`
      _)
    (:`Is Not Valid`
      (bind _returnvalue (`|SpawnActorFromClass` "/Game/GameplayAbilities/Blueprints/Abilities/HexCityBuilder/HexTiles/BP_HexGridManager.BP_HexGridManager_C" (`self.GetTransform`) "AlwaysSpawn" "MultiplyWithRoot" null null))
      (bind _output_get (set `self.HexManager` _returnvalue))
      (`self.K2_AttachToComponent` _output_get (`self.Scene`) "None" "SnapToTarget" "SnapToTarget" "KeepWorld" true)))
  (return))

(fn `LockCameraOverSelectedTile`
  (`MovementComponent.SetUpdatedComponent` (`self.RotatingMovement`) null))

(fn `RotateCamera`
  (params (DeltaTime :type "Float (single-precision)"))
  (bind (_camerarotation_roll _camerarotation_pitch _camerarotation_yaw) (`KismetMathLibrary.BreakRotator` (`self.CameraRotation`)))
  (if (and (`self.bCanMoveCamera`) (`self.bIsRightMouseButtonDown`))
    (bind _returnvalue (`WidgetLayoutLibrary.GetMousePositionOnViewport`))
    (bind (_returnvalue_x _returnvalue_y) (`KismetMathLibrary.BreakVector2D` (- _returnvalue (`self.PrevMousePosition`))))
    (set `self.CameraRotation` (`KismetMathLibrary.RInterpTo` (`self.CameraRotation`) (`KismetMathLibrary.MakeRotator` 0.0 (- _camerarotation_pitch _returnvalue_y) (+ _camerarotation_yaw _returnvalue_x)) (`local.DeltaTime`) (`self.CameraRotationSpeed`)))
    (`SceneComponent.K2_SetRelativeRotation` (`self.SpringArm`) (`self.CameraRotation`) false false)
    (`self.SetCurrentMousePosition`)))

(fn `SelectedTile`
  (locals (SpawnTransform :type "Transform Structure"))
  (bind _hextileselected (`self.HexTileSelected`))
  (bind _hextileselector (`self.HexTileSelector`))
  (bind _hextileselected_2 (`self.HexTileSelected`))
  (bind _hextileselector_2 (`self.HexTileSelector`))
  (bind _selectedindex (`/Game/GameplayAbilities/Blueprints/Abilities/HexCityBuilder/HexTiles/BP_TileSelector.SelectedIndex` _hextileselector))
  (bind _selectedindex_2 (`/Game/GameplayAbilities/Blueprints/Abilities/HexCityBuilder/HexTiles/BP_TileSelector.SelectedIndex` _hextileselector_2))
  (bind _returnvalue (`HexGrid.GetTileCollisionTransform` (`/Game/GameplayAbilities/Blueprints/Abilities/HexCityBuilder/HexTiles/BP_TileSelector.SelectedGrid` _hextileselector_2) _selectedindex_2))
  (if (> (`/Game/GameplayAbilities/Blueprints/Abilities/HexCityBuilder/HexTiles/BP_TileSelector.SelectedIndex` (`self.HexTileSelector`)) -1)
    (`|ExecutionSequence`
      (:`then_0`
        (`/Engine/EditorBlueprintResources/StandardMacros.IsValid` (`self.HexTileSelected`)
          (:`Is Valid`
            (set `local.SpawnTransform` _returnvalue))
          (:`Is Not Valid`
            (set `local.SpawnTransform` _returnvalue)
            (bind _returnvalue_2 (`|SpawnActorFromClass` "/Game/GameplayAbilities/Blueprints/Abilities/HexCityBuilder/HexTiles/BP_TileSelector.BP_TileSelector_C" (`local.SpawnTransform`) "AlwaysSpawn" "OverrideRootScale" self _selectedindex_2 true null self))
            (bind _output_get (set `self.HexTileSelected` _returnvalue_2))
            (`self.K2_AttachToComponent` _output_get (`self.RootComponent`) "None" "KeepWorld" "KeepWorld" "KeepWorld" true)))
        (`self.K2_SetActorRelativeTransform` _hextileselected_2 (`local.SpawnTransform`) false true)
        (`/Game/GameplayAbilities/Blueprints/Abilities/HexCityBuilder/HexTiles/BP_TileSelector.ChangeIndex` _hextileselected_2 _selectedindex (`/Game/GameplayAbilities/Blueprints/Abilities/HexCityBuilder/HexTiles/BP_TileSelector.SelectedGrid` _hextileselector))
        (`self.SetActorHiddenInGame` _hextileselected_2 false)
        (`self.OnSelectedTile` _selectedindex))
      (:`then_1`
        (`self.LockCameraOverSelectedTile`)))
    (else
      (`/Engine/EditorBlueprintResources/StandardMacros.IsValid` _hextileselected
        (:`Is Valid`
          (`self.SetActorHiddenInGame` _hextileselected true)
          (`MovementComponent.SetUpdatedComponent` (`self.RotatingMovement`) (`self.RootComponent`))
          (`self.OnUnSelectedTile`))))))

(fn `Set Starter Tile`
  (locals (LocStart :type "Vector Structure") (LocEnd :type "Vector Structure") (LocCanvas :type "Canvas Object Reference"))
  (`HexGrid.SetTileVertexColor` (`HexGridManager.GetGridAtIndex` (`self.HexManager`) 0) (`KismetMathLibrary.MakeColor` 0.0) (make `HexCoord`)))

(fn `SetCurrentMousePosition`
  (bind _returnvalue (`WidgetLayoutLibrary.GetMousePositionOnViewport`))
  (set `self.PrevMousePosition` _returnvalue))

(fn `StartGlobeRotation`
  (bind _rotatingmovement (`self.RotatingMovement`))
  (`MovementComponent.SetUpdatedComponent` _rotatingmovement (`self.RootComponent`))
  (`ActorComponent.Activate` _rotatingmovement false))

(fn `UserConstructionScript`)

(fn `ZoomCamera`
  (params (AxisValue :type "Float (single-precision)"))
  (if (and (`self.bCanZoomCamera`) (!= (`local.AxisValue`) 0.0))
    (bind _output_get (set `SpringArmComponent.TargetArmLength` (`KismetMathLibrary.FClamp` (+ (* (`local.AxisValue`) (`self.CameraZoomSpeed`) -1.0) (`SpringArmComponent.TargetArmLength` (`self.SpringArm`))) (`self.MinCameraDistance`) (`self.MaxCameraDistance`)) (`self.SpringArm`)))
    (`LightComponent.SetIntensity` (`self.SpotLight`) (`KismetMathLibrary.MapRangeClamped` _output_get (`self.MinCameraDistance`) (`self.MaxCameraDistance`) (`self.CloseLightIntensity`) (`self.FarLightIntensity`)))))