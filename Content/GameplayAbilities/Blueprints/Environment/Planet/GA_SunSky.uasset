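; Planet sky actor that drives sun, moon, sky light, atmosphere, height fog and volumetric clouds from the GameState's time of day.
; Each tick a day curve sets light intensities, while atmosphere, fog and cloud values interpolate toward weather targets.
; SetAtmosphere selects those targets, though Overcast and Heavy Fog are empty stubs and Default mostly zeroes values.
; SetViewDistanceFog drives a lazily created dynamic post-process material for distance fog.
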(event `self.ReceiveBeginPlay`
  (`self.UpdatePostProcessMaterials`))

(event `self.ReceiveTick`
  (params (DeltaSeconds :type "Float (single-precision)"))
  (bind _returnvalue (message `GameTimeInterface.GetTimeOfDay` (`GameplayStatics.GetGameState`)))
  (set `self.SolarTime` _returnvalue)
  (`parent.ReceiveTick` DeltaSeconds)
  (`self.UpdateSky` DeltaSeconds))

(event `WeatherInterface.SetAtmosphere`
  (params (InAtmosphere :type "EAtmosphereType Enum" :default "NoChange"))
  (switch `EAtmosphereType` InAtmosphere
    (:`Default`
      (`self.DefaultWeather`))
    (:`Overcast`
      (`self.OvercastWeather`))
    (:`HeavyFog`
      (`self.HeavyFogWeather`))))

(event `SetViewDistanceFog`
  (params (Blend :type "Float (double-precision)") (FogStrength :type "Float (double-precision)") (FogStart :type "Float (double-precision)") (FogColor :type "LinearColor Structure"))
  (bind _dynamicfog (`self.GetViewDistanceFogDynamic` Blend))
  (if (not (<= Blend 0.0))
    (`MaterialInstanceDynamic.SetScalarParameterValue` _dynamicfog "FogDistance" FogStrength)
    (`MaterialInstanceDynamic.SetScalarParameterValue` _dynamicfog "FogStartDistance" FogStart)
    (`MaterialInstanceDynamic.SetVectorParameterValue` _dynamicfog "FogColor" FogColor))
  (`self.UpdatePostProcessMaterials`))

(fn `DefaultWeather`
  (set `self.RSSTarget` 0.0)
  (set `self.RSTarget` (struct))
  (set `self.REDTarget` 0.0)
  (set `self.FogDensityTarget` 0.0)
  (set `self.FogFalloffTarget` 0.0)
  (set `self.FogColorTarget` (struct))
  (set `self.CloudHeight` 0.0))

(fn `GetViewDistanceFogDynamic`
  (params (Item_Weight :type "Float (single-precision)"))
  (returns (DynamicFog :type "MaterialInstanceDynamic Object Reference"))
  (bind _output (`|GetArrayItem` (`self.PPM`) 1))
  (bind _asmaterial_instance_dynamic (cast `MaterialInstanceDynamic` (`.Object` (break `WeightedBlendable` _output)))
    (:`then`
      (setmembers `WeightedBlendable` :`StructRef` _output :`Weight` (`local.Item_Weight`))
      (return _asmaterial_instance_dynamic))
    (:`CastFailed`
      (bind _returnvalue (`KismetMaterialLibrary.CreateDynamicMaterialInstance` "/Game/GameplayAbilities/FX/Cascade/PostProcessM/MI_PP_ViewDistanceFog_Default.MI_PP_ViewDistanceFog_Default" "ViewDistanceFogMaterial"))
      (`KismetArrayLibrary.Array_Set` (`self.PPM`) 1 (make `WeightedBlendable` (`local.Item_Weight`) _returnvalue))
      (return _returnvalue))))

(fn `HeavyFogWeather`)

(fn `OvercastWeather`)

(fn `UpdateMoon`
  (`SceneComponent.K2_SetWorldRotation` (`self.MoonLight`) (`KismetMathLibrary.NegateRotator` (`KismetMathLibrary.MakeRotator` 0.0 (`self.CorrectedElevation`) (+ (`self.Azimuth`) (`self.NorthOffset`)))) false false))

(fn `UpdatePostProcessMaterials`
  (setmembers `PostProcessSettings` :`StructRef` (`PostProcessComponent.Settings` (`self.PostProcess`)) :`WeightedBlendables` (make `WeightedBlendables` (`self.PPM`))))

(fn `UpdateSky`
  (params (DeltaTime :type "Float (double-precision)"))
  (locals (LocDeltaTime :type "Float (double-precision)") (LocREDistribution :type "Float (double-precision)" :default 0.0) (LocRScattering :type "LinearColor Structure") (LocRSScale :type "Float (double-precision)" :default 0.0) (LocFogColor :type "LinearColor Structure") (LocFogFalloff :type "Float (double-precision)" :default 0.0) (LocFogDensity :type "Float (double-precision)" :default 0.0) (LocLayerHeight :type "Float (double-precision)" :default 0.0) (LocLayerBottomAltitude :type "Float (double-precision)" :default 0.0) (LocMEDistribution :type "Float (double-precision)" :default 0.0) (LocMScattering :type "LinearColor Structure") (LocMScale :type "Float (double-precision)" :default 0.0) (LocMAbsorbtion :type "LinearColor Structure") (LocMAScale :type "Float (double-precision)" :default 0.0))
  (bind _skyatmosphere (`self.SkyAtmosphere`))
  (bind _exponentialheightfog (`self.ExponentialHeightFog`))
  (bind _volumetriccloud (`self.VolumetricCloud`))
  (bind _directionallight (`self.DirectionalLight`))
  (bind _volumetriccloud_2 (`self.VolumetricCloud`))
  (set `local.LocDeltaTime` DeltaTime)
  (set `local.LocREDistribution` (`SkyAtmosphereComponent.RayleighExponentialDistribution` _skyatmosphere))
  (set `local.LocRScattering` (`SkyAtmosphereComponent.RayleighScattering` _skyatmosphere))
  (set `local.LocRSScale` (`SkyAtmosphereComponent.RayleighScatteringScale` _skyatmosphere))
  (set `local.LocMEDistribution` (`SkyAtmosphereComponent.MieExponentialDistribution` _skyatmosphere))
  (set `local.LocMScattering` (`SkyAtmosphereComponent.MieScattering` _skyatmosphere))
  (set `local.LocMScale` (`SkyAtmosphereComponent.MieScatteringScale` _skyatmosphere))
  (set `local.LocMAbsorbtion` (`SkyAtmosphereComponent.MieAbsorption` _skyatmosphere))
  (set `local.LocMAScale` (`SkyAtmosphereComponent.MieAbsorptionScale` _skyatmosphere))
  (set `local.LocFogDensity` (`ExponentialHeightFogComponent.FogDensity` _exponentialheightfog))
  (set `local.LocFogFalloff` (`ExponentialHeightFogComponent.FogHeightFalloff` _exponentialheightfog))
  (set `local.LocFogColor` (`ExponentialHeightFogComponent.FogInscatteringLuminance` _exponentialheightfog))
  (set `local.LocLayerHeight` (`VolumetricCloudComponent.LayerHeight` _volumetriccloud_2))
  (set `local.LocLayerBottomAltitude` (`VolumetricCloudComponent.LayerBottomAltitude` _volumetriccloud_2))
  (`|ExecutionSequence`
    (:`then_0`
      ;[1 1 1] Atmosphere Details
      (`SkyAtmosphereComponent.SetRayleighExponentialDistribution` (`self.SkyAtmosphere`) (`KismetMathLibrary.FInterpTo` (`local.LocREDistribution`) (`self.REDTarget`) (`local.LocDeltaTime`) 5.0))
      (`SkyAtmosphereComponent.SetRayleighScattering` (`self.SkyAtmosphere`) (`KismetMathLibrary.CInterpTo` (`local.LocRScattering`) (`self.RSTarget`) (`local.LocDeltaTime`) 5.0))
      (`SkyAtmosphereComponent.SetRayleighScatteringScale` (`self.SkyAtmosphere`) (`KismetMathLibrary.FInterpTo` (`local.LocRSScale`) (`self.RSSTarget`) (`local.LocDeltaTime`) 5.0))
      (`SkyAtmosphereComponent.SetMieExponentialDistribution` (`self.SkyAtmosphere`) (`KismetMathLibrary.FInterpTo` (`local.LocMEDistribution`) (`self.MEDTarget`) (`local.LocDeltaTime`) 5.0))
      (`SkyAtmosphereComponent.SetMieScattering` (`self.SkyAtmosphere`) (`KismetMathLibrary.CInterpTo` (`local.LocMScattering`) (`self.MSTarget`) (`local.LocDeltaTime`) 5.0))
      (`SkyAtmosphereComponent.SetMieScatteringScale` (`self.SkyAtmosphere`) (`KismetMathLibrary.FInterpTo` (`local.LocMScale`) (`self.MSSTarget`) (`local.LocDeltaTime`) 5.0))
      (`SkyAtmosphereComponent.SetMieAbsorption` (`self.SkyAtmosphere`) (`KismetMathLibrary.CInterpTo` (`local.LocMAbsorbtion`) (`self.MATarget`) (`local.LocDeltaTime`) 5.0))
      (`SkyAtmosphereComponent.SetMieAbsorptionScale` (`self.SkyAtmosphere`) (`KismetMathLibrary.FInterpTo` (`local.LocMAScale`) (`self.MASTarget`) (`local.LocDeltaTime`) 5.0)))
    (:`then_1`
      ;[1 1 1] Sun Details
      (`LightComponent.SetIntensity` _directionallight (* (`CurveFloat.GetFloatValue` (`self.DayCurve`) (`self.SolarTime`)) (`self.DayLightScale`)))
      (`LightComponent.SetLightColor` _directionallight (`KismetMathLibrary.LinearColorLerp` (`self.HottestColor`) (`self.ColdestColor`) (`self.LightTemperature`)) true))
    (:`then_2`
      ;[1 1 1] Moon Details
      (`LightComponent.SetIntensity` (`self.MoonLight`) (* (- 1.0 (`CurveFloat.GetFloatValue` (`self.DayCurve`) (`self.SolarTime`))) 10.0))
      (`self.UpdateMoon`))
    (:`then_3`
      ;[1 1 1] Fog Details
      (`ExponentialHeightFogComponent.SetFogDensity` (`self.ExponentialHeightFog`) (`KismetMathLibrary.FInterpTo` (`local.LocFogDensity`) (`self.FogDensityTarget`) (`local.LocDeltaTime`) 5.0))
      (`ExponentialHeightFogComponent.SetFogInscatteringColor` (`self.ExponentialHeightFog`) (`KismetMathLibrary.CInterpTo` (`local.LocFogColor`) (`self.FogColorTarget`) (`local.LocDeltaTime`) 5.0))
      (`ExponentialHeightFogComponent.SetFogHeightFalloff` (`self.ExponentialHeightFog`) (`KismetMathLibrary.FInterpTo` (`local.LocFogFalloff`) (`self.FogFalloffTarget`) (`local.LocDeltaTime`) 5.0)))
    (:`then_4`
      ;[1 1 1] Post Process Details
      (`SkyLightComponent.SetIntensity` (`self.SkyLight`) (* (- 1.0 (`CurveFloat.GetFloatValue` (`self.DayCurve`) (`self.SolarTime`))) 3.0)))
    (:`then_5`
      ;[1 1 1] Clouds
      (`VolumetricCloudComponent.SetLayerHeight` _volumetriccloud (`KismetMathLibrary.FInterpTo` (`local.LocLayerHeight`) (`self.CloudHeight`) (`local.LocDeltaTime`) 5.0))
      (`VolumetricCloudComponent.SetLayerBottomAltitude` _volumetriccloud (`KismetMathLibrary.FInterpTo` (`local.LocLayerBottomAltitude`) (`self.CloudBottomAltitude`) (`local.LocDeltaTime`) 5.0)))))

(fn `UserConstructionScript`
  (`parent.UserConstructionScript`))