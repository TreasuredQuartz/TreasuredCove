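; BP_ThumbnailCreator is an editor-only utility that bakes UI thumbnail textures for the Minecraft blocks listed in DT_MinecraftBlockInfo.
; Each RenderThumbnail call applies the current row's block type and material to a preview voxel.
; It saves the scene capture's render target as a static UI-group texture if the row lacks one or regeneration is enabled.
; The row index advances only when a texture is created.
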(event `self.ReceiveBeginPlay`)

(event `RenderThumbnail`
  (bind _voxel (`self.Voxel`))
  (if (`KismetArrayLibrary.Array_IsEmpty` (`self.Out Row Names`))
    (bind _outrownames (`DataTableFunctionLibrary.GetDataTableRowNames` "/Game/GameplayAbilitiesBP/Maps/MainWorld/LightDungeon/Blueprints/Datatables/DT_MinecraftBlockInfo.DT_MinecraftBlockInfo"))
    (set `self.Out Row Names` _outrownames))
  (bind _returnvalue (`|GetDataTableRow` "/Game/GameplayAbilitiesBP/Maps/MainWorld/LightDungeon/Blueprints/Datatables/DT_MinecraftBlockInfo.DT_MinecraftBlockInfo" (`|GetArrayItem` (`self.Out Row Names`) (`self.CurrentIndex`)))
    (:`then`
      (bind (_bistransparent _blocktype _material _uitexture) (break `DTMCBlockInfo` _returnvalue))
      (set `/Game/GameplayAbilities/Environment/Minecraft/Thumbnails/BP_Voxel.BlockType` _blocktype _voxel)
      (set `/Game/GameplayAbilities/Environment/Minecraft/Thumbnails/BP_Voxel.Material` _material _voxel)
      (`/Game/GameplayAbilities/Environment/Minecraft/Thumbnails/BP_Voxel.UpdateMesh` _voxel)
      (`/Engine/EditorBlueprintResources/StandardMacros.IsValid` _uitexture
        (:`Is Valid`
          (if (`self.RegenerateThumbnails`)
            (bind _returnvalue_2 (`KismetRenderingLibrary.RenderTargetCreateStaticTexture2DEditorOnly` (`SceneCaptureComponent2D.TextureTarget` (`/Game/GameplayAbilities/Environment/Minecraft/Thumbnails/BP_CaptureActor.SceneCaptureComponent2D` (`self.CaptureActor`))) "Texture" "TC_Default" "TMGS_Sharpen0" :!label _label))
            (set `Texture.LODGroup` "TEXTUREGROUP_UI" _returnvalue_2)
            (`/Engine/EditorBlueprintResources/StandardMacros.IncrementInt` (`self.CurrentIndex`))))
        (:`Is Not Valid`
          (goto _label))))))

(event `SpawnItem`)

(fn `UserConstructionScript`)