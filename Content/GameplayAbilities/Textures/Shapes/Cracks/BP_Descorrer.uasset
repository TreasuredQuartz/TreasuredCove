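; Construction-script Blueprint that computes geometry for a "rift", a wall-like strip along a spline, for a runtime mesh.
; GenerateRift clears the mesh section, samples world-space spline transforms every segment length, and GetVoxelAtTransform returns a quad for each.
; Quad indices are offset by the triangle-array length rather than vertex count, and vertex-to-index ratios are logged.
; Section creation and material setup are disconnected, so no mesh is built.
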(fn `ClearData`
  (`RuntimeMeshComponentStatic.RemoveSection` (`self.RuntimeMeshComponentStatic`) 0 0))

(fn `GenerateRift`
  (locals (LocVerts :type "Array of Vector Structure") (LocTris :type "Array of Integer"))
  (bind _locverts (`local.LocVerts`))
  (bind _loctris (`local.LocTris`))
  (bind _returnvalue (`KismetArrayLibrary.Array_Length` _loctris))
  (bind _returnvalue_2 (* (`KismetArrayLibrary.Array_Length` _locverts) 1.5))
  (`self.ClearData`)
  (`KismetArrayLibrary.Array_Clear` (`local.LocVerts`))
  (`KismetArrayLibrary.Array_Clear` (`local.LocTris`))
  (for _index (range 1 (`KismetMathLibrary.FTrunc` (/ (`SplineComponent.GetSplineLength` (`self.Spline`)) (`self.WallSegmentLength`))))
    (bind (_verts _tris) (`self.GetVoxelAtTransform` (`SplineComponent.GetTransformAtDistanceAlongSpline` (`self.Spline`) (* _index (`self.WallSegmentLength`)) "World" false) (`KismetArrayLibrary.Array_Length` (`local.LocTris`))))
    (`KismetArrayLibrary.Array_Append` _locverts _verts)
    (`KismetArrayLibrary.Array_Append` _loctris _tris)
    (if (< _returnvalue_2 _returnvalue)
      (`KismetSystemLibrary.LogString` "Verts are less than tris")
      (elif (== _returnvalue_2 _returnvalue)
        (`KismetSystemLibrary.LogString` "Verts == tris")
        (else
          (`KismetSystemLibrary.LogString` "Verts are more than tris"))))))

(fn `GetVoxelAtTransform`
  (params (InTransform :type "Transform Structure (by ref)") (TriangleNum :type Integer))
  (returns (Verts :type "Array of Vector Structure") (Tris :type "Array of Integer"))
  (locals (LocBottomRightVert :type "Vector Structure") (LocBottomLeftVert :type "Vector Structure") (LocTopRightVert :type "Vector Structure") (LocTopLeftVert :type "Vector Structure") (LocVert :type "Array of Vector Structure") (LocTri :type "Array of Integer"))
  (bind _location (.location InTransform))
  (bind _rotation (.rotation InTransform))
  (bind _returnvalue (* (`KismetMathLibrary.Conv_RotatorToVector` _rotation) (* (`self.WallSegmentLength`) 0.5)))
  (bind _returnvalue_2 (* (`KismetMathLibrary.GetUpVector` _rotation) 50.0))
  (bind _returnvalue_3 (+ _location _returnvalue))
  (bind _returnvalue_4 (- _location _returnvalue))
  (set `local.LocBottomRightVert` _returnvalue_3)
  (set `local.LocBottomLeftVert` _returnvalue_4)
  (set `local.LocTopRightVert` (+ _returnvalue_3 _returnvalue_2))
  (set `local.LocTopLeftVert` (+ _returnvalue_4 _returnvalue_2))
  (`KismetArrayLibrary.Array_Add` (`local.LocVert`) (`local.LocBottomRightVert`))
  (`KismetArrayLibrary.Array_Add` (`local.LocVert`) (`local.LocBottomLeftVert`))
  (`KismetArrayLibrary.Array_Add` (`local.LocVert`) (`local.LocTopRightVert`))
  (`KismetArrayLibrary.Array_Add` (`local.LocVert`) (`local.LocTopLeftVert`))
  (`|ExecutionSequence`
    (:`then_0`
      (`KismetArrayLibrary.Array_Add` (`local.LocTri`) (+ (`local.TriangleNum`) 0))
      (`KismetArrayLibrary.Array_Add` (`local.LocTri`) (+ (`local.TriangleNum`) 1))
      (`KismetArrayLibrary.Array_Add` (`local.LocTri`) (+ (`local.TriangleNum`) 2)))
    (:`then_1`
      (`KismetArrayLibrary.Array_Add` (`local.LocTri`) (+ (`local.TriangleNum`) 3))
      (`KismetArrayLibrary.Array_Add` (`local.LocTri`) (+ (`local.TriangleNum`) 1))
      (`KismetArrayLibrary.Array_Add` (`local.LocTri`) (+ (`local.TriangleNum`) 2)))
    (:`then_2`
      (return (`local.LocVert`) (`local.LocTri`)))))

(fn `UserConstructionScript`
  (`self.GenerateRift`))