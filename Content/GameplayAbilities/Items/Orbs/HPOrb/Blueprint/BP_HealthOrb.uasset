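; Health orb pickup that applies the GE_HealthOrb gameplay effect to the actor that collects it, then runs parent pickup logic.
; The construction script randomizes the pickup quantity and, with a separate roll, the mesh scale.
; On pickup it builds a Stats.health SetByCaller spec from the quantity, but applies the effect by class, so that magnitude is not passed on.
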(event `self.ReceiveBeginPlay`
  (`parent.ReceiveBeginPlay`))

(event `PickupInterface.OnPickedUp`
  (params (OtherActor :type "Actor Object Reference"))
  (bind _returnvalue (`|GenericCreateObject` "/Game/GameplayAbilities/Items/Orbs/HPOrb/Ability/GE_HealthOrb.GE_HealthOrb_C"))
  (`AbilitySystemBlueprintLibrary.AssignTagSetByCallerMagnitude` (`AbilitySystemBlueprintLibrary.MakeSpecHandle` _returnvalue (`self.GetInstigator`) self) (struct :`TagName` "stats.health") (`KismetMathLibrary.Conv_IntToDouble` (`.Quantity` (break `ItemKey` (`self.PickupInfo`)))))
  (`AbilitySystemComponent.BP_ApplyGameplayEffectToSelf` :`self` (`AbilitySystemBlueprintLibrary.GetAbilitySystemComponent` OtherActor) :`GameplayEffectClass` "/Game/GameplayAbilities/Items/Orbs/HPOrb/Ability/GE_HealthOrb.GE_HealthOrb_C")
  (`parent.OnPickedUp` OtherActor))

(fn `UserConstructionScript`
  (bind _returnvalue (`KismetMathLibrary.RandomIntegerInRange` 1 10))
  (`parent.UserConstructionScript`)
  (setmembers `ItemKey` :`StructRef` (`self.PickupInfo`) :`Quantity` _returnvalue)
  (`SceneComponent.SetWorldScale3D` (`self.Mesh`) (`KismetMathLibrary.Conv_DoubleToVector` (/ _returnvalue 10.0 2.0))))