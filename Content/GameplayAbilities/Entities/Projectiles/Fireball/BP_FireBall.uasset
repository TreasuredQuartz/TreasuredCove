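; Fireball projectile that applies an ability-supplied gameplay effect to whatever it hits, then explodes.
; Hits come from sphere overlap, ignoring instigator and owner, or a per-tick line trace along velocity until exploding.
; A hit applies the effect spec to the target's ability system component, stops movement and the traveling effect.
; Timelines then expand a sphere mesh, spin it and destroy the actor.
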(event `HitActor`
  (params (HitActor :type "Actor Object Reference"))
  (bind _returnvalue (`AbilitySystemBlueprintLibrary.GetAbilitySystemComponent` HitActor))
  (`/Engine/EditorBlueprintResources/StandardMacros.IsValid` _returnvalue
    (:`Is Valid`
      (`AbilitySystemComponent.BP_ApplyGameplayEffectSpecToSelf` _returnvalue (`self.EffectSpecHandleFromAbility`)))))

(event `self.ReceiveTick`
  (params (DeltaSeconds :type "Float (single-precision)"))
  (if (not (`self.bExploding`))
    (`self.LineTraceCheckCollision`)))

(event `self.Sphere_Collision.OnComponentBeginOverlap`
  (params (OverlappedComponent :type "PrimitiveComponent Object Reference") (OtherActor :type "Actor Object Reference") (OtherComp :type "PrimitiveComponent Object Reference") (OtherBodyIndex :type Integer) (bFromSweep :type Boolean) (SweepResult :type "HitResult Structure (by ref)"))
  (if (and (!= OtherActor (`self.GetInstigator`)) (!= OtherActor (`self.GetOwner`)) (!= OtherActor self))
    (`KismetSystemLibrary.PrintString` (`KismetSystemLibrary.GetDisplayName` OtherActor))
    (`self.HitActor` OtherActor)
    (`self.Explode`)))

(event `Explode`
  (set `self.bExploding` true)
  (`self.SetLifeSpan` 0.0)
  (`self.StopTraveling`)
  (`self.StartExpansion`))

(event `StopTraveling`
  (`ActorComponent.Deactivate` (`self.ProjectileMovementComp`))
  (`ActorComponent.Deactivate` (`self.Fireball_Traveling`)))

(event `StartExpansion`
  (`TimelineComponent.SetPlayRate` (`self.Timeline_Expansion`) (`self.ExpansionRate`))
  (`StaticMeshComponent.SetStaticMesh` (`self.ExplosionMesh`) "/Engine/BasicShapes/Sphere.Sphere")
  (bind (_direction _value) (`Timeline|Timeline_Expansion` :!via `PlayFromStart`)
    (:`Update`
      (`SceneComponent.SetWorldScale3D` (`self.ExplosionMesh`) (+ (1.0 1.0 1.0) (* (5.0 5.0 5.0) _value))))
    (:`Finished`
      (`self.EndExpansion`))))

(event `EndExpansion`
  (`Timeline|Timeline_Rotation` :!via `PlayFromStart`
    (:`Update`
      (`SceneComponent.K2_AddWorldRotation` (`self.ExplosionMesh`) (struct :`Yaw` 7.5) false false))
    (:`Finished`
      (`self.K2_DestroyActor`))))

(fn `LineTraceCheckCollision`
  (bind _returnvalue (`self.K2_GetActorLocation`))
  (bind (_outhit _returnvalue_2) (`KismetSystemLibrary.LineTraceSingle` _returnvalue (+ _returnvalue (* (`self.GetVelocity`) 0.1)) "TraceTypeQuery1"))
  (if _returnvalue_2
    (bind (_bblockinghit _binitialoverlap _time _distance _location _impactpoint _normal _impactnormal _physmat _hitactor) (`GameplayStatics.BreakHitResult` _outhit))
    (`KismetSystemLibrary.PrintString` (`KismetSystemLibrary.GetDisplayName` _hitactor))
    (`self.HitActor` _hitactor)
    (`self.Explode`)))

(fn `UserConstructionScript`
  (`parent.UserConstructionScript`))