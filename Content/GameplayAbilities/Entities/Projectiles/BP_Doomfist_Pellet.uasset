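; BP_Doomfist_Pellet is a projectile actor that displays a pellet spread as a set of Niagara components.
; FireProjectiles destroys the previous components, then adds one per ProjSpreadPattern point at a fixed forward offset, using the point's X/Y as local Y/Z.
; The construction script builds the spread, and a looping one-second timer started on BeginPlay rebuilds it; no movement, collision or damage logic is present.
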(event `self.ReceiveBeginPlay`
  (`parent.ReceiveBeginPlay`)
  (bind _returnvalue (`KismetSystemLibrary.K2_SetTimer` null "FireProjectiles" 1.0 true))
  (set `self.NewVar` _returnvalue))

(fn `ClearProjectiles`
  (for _array_element (`self.ActiveProjectiles`)
    (`ActorComponent.K2_DestroyComponent` _array_element))
  (`KismetArrayLibrary.Array_Clear` (`self.ActiveProjectiles`)))

(fn `FireProjectiles`
  (`self.ClearProjectiles`)
  (for _array_element (`self.ProjSpreadPattern`)
    (bind (_x _y) (`KismetMathLibrary.BreakVector2D` _array_element))
    (bind _returnvalue (`AddComponent|NODE_AddNiagaraComponent-0` :`RelativeTransform` (`KismetMathLibrary.MakeTransform` (`KismetMathLibrary.MakeVector` 25.0 _x _y))))
    (`KismetArrayLibrary.Array_Add` (`self.ActiveProjectiles`) _returnvalue)))

(fn `UserConstructionScript`
  (`parent.UserConstructionScript`)
  (`self.FireProjectiles`))