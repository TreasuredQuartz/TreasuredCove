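; BP_Voxel is an actor that displays a single Minecraft-style block, apparently for thumbnails given its folder.
; The construction script calls UpdateMesh, which clears the procedural mesh and runs CreateFace for six faces using the selected block type's tile data and size.
; The resulting vertices, triangles, normals, UVs and vertex colours form one mesh section with the assigned material.
; A leftover loop copying colours into LinearVertexColor never runs.
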(event `UpdateMesh`
  (bind (_vertices _triangles _normals _uvs _vertexcolors) (break `ProceduralMeshSection` (`self.MeshSection`)))
  (`ProceduralMeshComponent.ClearMeshSection` (`self.ProceduralMesh`) 0)
  (set `self.MeshSection` (struct))
  (`KismetArrayLibrary.Array_Clear` (`self.LinearVertexColor`))
  (set `self.Cur Triangle Num` 0)
  (for _index (range 6)
    (bind (_meshsection _returnvalue) (`GALibrary.CreateFace` (`|GetArrayItem` (`self.BlockTypes`) (`self.BlockType`)) (`self.K2_GetActorLocation`) _index (`self.Cur Triangle Num`) (`self.Size`) 1))
    (set `self.Cur Triangle Num` _returnvalue)
    (set `self.MeshSection` _meshsection))
  (`ProceduralMeshComponent.CreateMeshSection_LinearColor` :`self` (`self.ProceduralMesh`) :`Vertices` _vertices :`Triangles` _triangles :`Normals` _normals :`UV0` _uvs :`VertexColors` _vertexcolors)
  (`PrimitiveComponent.SetMaterial` (`self.ProceduralMesh`) 0 (`self.Material`)))

(fn `UserConstructionScript`
  (`self.UpdateMesh`))