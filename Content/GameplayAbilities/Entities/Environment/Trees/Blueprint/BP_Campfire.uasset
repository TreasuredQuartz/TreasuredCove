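; BP_Campfire is an environment prop that procedurally builds a ring of campfire logs.
; Its construction script loops over NumLogs, adding one instance per log to an InstancedStaticMesh, evenly spaced around a circle of the given Radius.
; Each log's rotation follows its angle on the circle, with fixed rotator offsets to orient and tilt it.
; The event graph holds only disabled placeholder events, so it has no runtime logic.
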(fn `UserConstructionScript`
  (bind _numlogs (`self.NumLogs`))
  (for _index (range 1 (+ _numlogs 1))
    (bind _returnvalue (`KismetMathLibrary.RotatorFromAxisAndAngle` (0.0 0.0 1.0) (* 360.0 (/ _index _numlogs))))
    (`InstancedStaticMeshComponent.AddInstance` (`self.InstancedStaticMesh`) (`KismetMathLibrary.MakeTransform` (* (`KismetMathLibrary.Conv_RotatorToVector` _returnvalue) (`self.Radius`)) (`KismetMathLibrary.NormalizedDeltaRotator` (`KismetMathLibrary.NormalizedDeltaRotator` _returnvalue (struct :`Yaw` 90.0)) (struct :`Roll` -50.0))) false)))