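; Gadget vendor interactable that opens the Gadgetron shop menu for the player who interacts with it.
; Two rotating movement components spin its text widget and logo mesh; the label text is applied on construction and again shortly after BeginPlay.
; Interaction lazily creates and caches the shop widget, passing it the Vendor component, then shows it with UI-only input and a mouse cursor.
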(event `self.ReceiveBeginPlay`
  (`MovementComponent.SetUpdatedComponent` (`self.RotatingMovement_Widget`) (`self.Widget`))
  (`MovementComponent.SetUpdatedComponent` (`self.RotatingMovement_Logo`) (`self.SM_vendor_logo`))
  (`KismetSystemLibrary.Delay` 0.2)
  (`self.IntializeWidget`))

(event `IntializeWidget`
  (bind _text (`self.Text`))
  (bind _aswbp_custom_text (cast `/Game/GameplayAbilities/Blueprints/UI/Framework/CustomHUD/Custom/WBP_CustomText` (`WidgetComponent.GetWidget` (`self.Widget`))))
  (set `/Game/GameplayAbilities/Blueprints/UI/Framework/CustomHUD/Custom/WBP_CustomText.TextToDisplay` _text _aswbp_custom_text)
  (`TextBlock.SetText` (`/Game/GameplayAbilities/Blueprints/UI/Framework/CustomHUD/Custom/WBP_CustomText.Text` _aswbp_custom_text) _text))

(event `InteractionInterface.InteractedWith`
  (params (OtherActor :type "Actor Object Reference"))
  (bind _shopmenu (`self.ShopMenu`))
  (bind _asplayer_controller (cast `PlayerController` (`self.GetInstigatorController` OtherActor)))
  (`/Engine/EditorBlueprintResources/StandardMacros.IsValid` (`self.ShopMenu`)
    (:`Is Valid`
      _)
    (:`Is Not Valid`
      (bind _returnvalue (`|CreateWidget` "/Game/GameplayAbilities/Blueprints/UI/RatchetAndClank/WBP_Gadgetron_ShopMenu_V2.WBP_Gadgetron_ShopMenu_V2_C" _asplayer_controller (`self.Vendor`)))
      (set `self.ShopMenu` _returnvalue)))
  (`UserWidget.AddToViewport` _shopmenu 0)
  (`WidgetBlueprintLibrary.SetInputMode_UIOnlyEx` _asplayer_controller _shopmenu)
  (set `PlayerController.bShowMouseCursor` true _asplayer_controller))

(fn `UserConstructionScript`
  (`self.IntializeWidget`))