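; BP_ProjectileLauncher is an environment actor that fires projectiles automatically and repeatedly once play begins.
; On BeginPlay it starts a looping timer, with the interval derived from FireRate and an initial StartDelay.
; Each tick of that timer spawns ProjectileClass at the ProjectileSpawnLocation transform, owned by the launcher and ignoring collisions.
; Every spawned projectile gets a short fixed lifespan so it cleans itself up.
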(event `self.ReceiveBeginPlay`
  (`parent.ReceiveBeginPlay`)
  (`self.StartLaunching`))

(event `StartLaunching`
  (`KismetSystemLibrary.K2_SetTimerDelegate` (delegate `FireProjectile`) (/ 1.0 (`self.FireRate`)) true false (`self.StartDelay`)))

(event `FireProjectile`
  (bind _returnvalue (`|SpawnActorFromClass` (`self.ProjectileClass`) (`SceneComponent.K2_GetComponentToWorld` (`self.ProjectileSpawnLocation`)) "AlwaysSpawn" "MultiplyWithRoot" self null))
  (`self.SetLifeSpan` _returnvalue 5.0))

(fn `UserConstructionScript`)