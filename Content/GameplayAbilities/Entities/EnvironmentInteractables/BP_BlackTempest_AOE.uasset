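; BP_BlackTempest_AOE is a looping visual for a Black Tempest area-of-effect, built on an expanding sphere mesh.
; On BeginPlay it applies a dynamic instance of the Black Tempest material to the sphere.
; A timeline grows the sphere from tiny to large while raising the material's WPOIntensity in step, then resets the scale and restarts endlessly.
; The graph contains no damage or overlap logic.
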(event `self.ReceiveBeginPlay`
  (`self.AssignDynamicMaterial`)
  (`self.BeginScaling`))

(event `BeginScaling`
  (bind _returnvalue (`KismetMathLibrary.MakeVector` 0.1 0.1 0.1))
  (bind (_direction _durationtrack) (`Timeline|ScaleTimeline` :`NewTime` 0.1 :!via `PlayFromStart`)
    (:`Update`
      (`SceneComponent.SetWorldScale3D` (`self.Sphere`) (+ (* (30.0 30.0 30.0) _durationtrack) _returnvalue))
      (`MaterialInstanceDynamic.SetScalarParameterValue` (`self.MID`) "WPOIntensity" (* _durationtrack 100.0)))
    (:`Finished`
      (`SceneComponent.SetWorldScale3D` (`self.Sphere`) _returnvalue)
      (`self.BeginScaling`))))

(event `AssignDynamicMaterial`
  (`/Engine/EditorBlueprintResources/StandardMacros.IsValid` (`self.MID`)
    (:`Is Valid`
      _)
    (:`Is Not Valid`
      (bind _returnvalue (`PrimitiveComponent.CreateDynamicMaterialInstance` (`self.Sphere`) 0 "/Game/GameplayAbilities/Entities/EnvironmentInteractables/Mi_BlackTempest.Mi_BlackTempest" "None"))
      (set `self.MID` _returnvalue)))
  (`PrimitiveComponent.SetMaterial` (`self.Sphere`) 0 (`self.MID`)))

(fn `UserConstructionScript`)