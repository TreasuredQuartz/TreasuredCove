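; Master Blueprint for perk machines, which grant a perk to the interacting actor through a Gameplay Effect.
; On interaction, a valid Manager checks a pawn's points against PointsRequired before the effect is applied to that actor's AbilitySystemComponent.
; Without a valid Manager (Zombies inactive), or when the actor is not a Pawn, the perk is applied without a points check.
; CanBuyPerkMachine is an unimplemented stub.
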(event `InteractionInterface.InteractedWith`
  (params (OtherActor :type "Actor Object Reference"))
  (`KismetSystemLibrary.PrintString` "Interacted with Machine")
  (`/Engine/EditorBlueprintResources/StandardMacros.IsValid` (`self.Manager`)
    (:`Is Valid`
      (bind _aspawn (cast `Pawn` OtherActor)
        (:`then`
          (bind _returnvalue (`Zombie_Manager.CheckPoints` (`self.Manager`) _aspawn (`self.Points Required`)))
          (if _returnvalue
            (`KismetSystemLibrary.PrintString` "Bought Perk With Points")
            (`AbilitySystemComponent.BP_ApplyGameplayEffectToSelf` :`self` (`self.GetComponentByClass` OtherActor "/Script/GameplayAbilities.AbilitySystemComponent") :`GameplayEffectClass` (`self.Gameplay Effect Class`) :!label _label)))
        (:`CastFailed`
          (goto _label))))
    (:`Is Not Valid`
      (`KismetSystemLibrary.PrintString` "Zombies is not active; Gave Perk for free")
      (goto _label))))

(fn `Can Buy PerkMachine`
  (returns (Succeeded :type Boolean)))

(fn `UserConstructionScript`
  (`parent.UserConstructionScript`))