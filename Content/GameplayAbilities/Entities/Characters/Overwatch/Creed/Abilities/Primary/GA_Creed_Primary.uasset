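; Creed's primary ability: a combo melee attack that also fires a blade projection.
; The owner's ComboSystem picks the step, which selects the montage and blade tilt, with cooldown committed from the third step onward.
; A melee damage gameplay event applies GE_Creed_Primary to its target.
; The straight-flying projection spawns when the montage starts and carries its own effect spec; a SpawnProjectile alternative sits disconnected, noted as broken.
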(event `self.K2_ActivateAbility`
  (`self.K2_CommitAbilityCost` false)
  (bind _returnvalue (`self.GetOwningCharacter`))
  (bind _returnvalue_2 (`ComboComponent.DetermineCombo` (`GACharacter.ComboSystem` _returnvalue) (`self.ComboTag`)))
  (bind _output_get (set `self.ComboNum` _returnvalue_2))
  (`KismetSystemLibrary.PrintString` (`KismetStringLibrary.Conv_IntToString` (`self.ComboNum`)))
  (if (== _output_get -1)
    (`self.K2_EndAbility`)
    (else
      (if (not (< _output_get 2))
        (`self.K2_CommitAbilityCooldown` false))
      (`AbilityTask_PlayMontageAndWait.CreatePlayMontageAndWaitProxy` "None" (`|GetArrayItem` (`self.ComboMontages`) (`self.ComboNum`)) 1.0 "None" false
        (:`then`
          (bind (_asynctaskproxy _payload) (`AbilityTask_WaitGameplayEvent.WaitGameplayEvent` (struct :`TagName` "skills.creedPrimary.meleeDamage") null)
            (:`then`
              (bind (_asynctaskproxy_2 _spawnedactor) (`AbilityTask_SpawnActor.SpawnActor` (`.TargetData` (`self.TargetDataFromCamera` _returnvalue)) "/Game/GameplayAbilities/Entities/Items/Projectiles/LotusBladeProjectile/Blueprint/BladeProjection.BladeProjection_C" _returnvalue)
                (:`Success`
                  (`self.SpawnBladeProjection` _spawnedactor))))
            (:`EventReceived`
              (`self.BP_ApplyGameplayEffectToTarget` (`AbilitySystemBlueprintLibrary.AbilityTargetDataFromActor` (`.Target` (break `GameplayEventData` _payload))) "/Game/GameplayAbilities/Entities/Characters/Overwatch/Creed/Abilities/Primary/GE_Creed_Primary.GE_Creed_Primary_C"))))
        (:`OnCompleted`
          (`self.K2_EndAbility` :!label _label))
        (:`OnBlendOut`
          (goto _label))
        (:`OnInterrupted`
          (goto _label))
        (:`OnCancelled`
          (goto _label))))))

(fn `SpawnBladeProjection`
  (params (SpawnedActor :type "Actor Object Reference") (Sight :type "SenseComponent Object Reference"))
  (bind _asblade_projection (cast `/Game/GameplayAbilities/Entities/Items/Projectiles/LotusBladeProjectile/Blueprint/BladeProjection` SpawnedActor))
  (`Actor.K2_SetActorRotation` _asblade_projection (`SceneComponent.GetSocketRotation` Sight "None") false)
  (bind _staticmesh (`/Game/GameplayAbilities/Entities/Items/Projectiles/LotusBladeProjectile/Blueprint/BladeProjection.StaticMesh` _asblade_projection))
  (`SceneComponent.K2_SetWorldRotation` _staticmesh (`KismetMathLibrary.ComposeRotators` (`SceneComponent.K2_GetComponentRotation` _staticmesh) (select `int` (`self.ComboNum`) :`0` (struct :`Roll` 45.0) :`1` (struct :`Roll` -45.0) :`2` (struct) :!type "Rotator Structure")) false false)
  (`Actor.SetLifeSpan` _asblade_projection 1.2)
  (set `GAProjectile.EffectSpecHandleFromAbility` (`self.MakeOutgoingGameplayEffectSpec` "/Game/GameplayAbilities/Entities/Characters/Overwatch/Creed/Abilities/Primary/GE_Creed_Primary_Projectile.GE_Creed_Primary_Projectile_C") _asblade_projection)
  (bind _projectilemovementcomp (`GAProjectile.ProjectileMovementComp` _asblade_projection))
  (`ProjectileMovementComponent.SetVelocityInLocalSpace` _projectilemovementcomp (`self.Velocity`))
  (set `ProjectileMovementComponent.bRotationFollowsVelocity` true _projectilemovementcomp)
  (set `ProjectileMovementComponent.bShouldBounce` false _projectilemovementcomp)
  (set `ProjectileMovementComponent.ProjectileGravityScale` 0.0 _projectilemovementcomp))