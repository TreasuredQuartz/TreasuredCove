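; GA_Creed_Secondary is Creed's secondary gameplay ability, a barrier held for as long as the input is held.
; On activation it commits, spawns a CreedBarrier through a SpawnActor task and attaches it to the owning actor, snapped to location and rotation.
; Input release or a failed spawn ends the ability, and ending it destroys the spawned barrier.
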(event `self.K2_ActivateAbility`
  (`self.K2_CommitAbility`)
  (`AbilityTask_WaitInputRelease.WaitInputRelease` true
    (:`then`
      (bind (_asynctaskproxy _spawnedactor) (`AbilityTask_SpawnActor.SpawnActor` (struct) "/Game/GameplayAbilities/Entities/EnvirionmentInteractables/Barriers/CreedBarrier.CreedBarrier_C" null)
        (:`Success`
          (set `self.SpawnedActor` _spawnedactor)
          (`Actor.K2_AttachToActor` _spawnedactor (`self.GetOwningActorFromActorInfo`) "None" "SnapToTarget" "SnapToTarget" "KeepRelative" true))
        (:`DidNotSpawn`
          (`self.K2_EndAbility` :!label _label))))
    (:`OnRelease`
      (goto _label))))

(event `self.K2_OnEndAbility`
  (params (bWasCancelled :type Boolean))
  (bind _spawnedactor (`self.SpawnedActor`))
  (`/Engine/EditorBlueprintResources/StandardMacros.IsValid` _spawnedactor
    (:`Is Valid`
      (`Actor.K2_DestroyActor` _spawnedactor))))