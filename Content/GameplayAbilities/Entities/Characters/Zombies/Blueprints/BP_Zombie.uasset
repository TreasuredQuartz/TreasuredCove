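; Zombie enemy character that attacks with both arms through the Gameplay Ability System.
; On spawn it pauses its BP_ZombieController logic during a get-up montage, then restarts it unless dead.
; Arm notifies toggle per-hand hitbox overlaps, which apply GE_ZombieAttack to non-zombie actors, using an ignore list cleared on each notify to avoid repeat hits.
; Its voice cycles through random sounds, and death sets a lifespan for removal.
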(event `self.ReceiveBeginPlay`
  (bind _sound (`self.Sound`))
  (bind (_asbp_zombie_controller _bsuccess) (cast `/Game/GameplayAbilities/Entities/Characters/Zombies/Blueprints/BP_ZombieController` (`self.GetController`) :!pure true))
  ;[1 1 1] Don't think while spawning
  (`parent.ReceiveBeginPlay`)
  (if _bsuccess
    (`/Game/GameplayAbilities/Entities/Characters/Zombies/Blueprints/BP_ZombieController.StopLogic` _asbp_zombie_controller "Spawning")
    (`|PlayMontage` (`self.Mesh`) "/Game/Zombie_Pack/Animations/InPlace/Get_Up/IP_GetUp_01_Montage.IP_GetUp_01_Montage"
      (:`then`
        ;[1 1 1] Random Sound
        (`AudioComponent.SetSound` (`self.Voice`) (`|GetArrayItem` _sound (`KismetMathLibrary.RandomInteger` (- (`KismetArrayLibrary.Array_Length` _sound) 1)))))
      (:`OnCompleted`
        (if _bsuccess :!label _label
          (if (not (`self.GetIsDead`))
            (`/Game/GameplayAbilities/Entities/Characters/Zombies/Blueprints/BP_ZombieController.RestartLogic` _asbp_zombie_controller))))
      (:`OnBlendOut`
        (goto _label))
      (:`OnInterrupted`
        (goto _label)))))

(event `MeleeCombatInterface.RightArm_Notify`
  ;[1 1 1] Attacking
  (bind _isa (`/Engine/EditorBlueprintResources/StandardMacros.FlipFlop`)
    (:`A`
      _)
    (:`B`
      _))
  (`KismetArrayLibrary.Array_Clear` (`self.IgnoredActors`))
  (set `PrimitiveComponent.bGenerateOverlapEvents` _isa (`self.Hitbox_r`)))

(event `MeleeCombatInterface.LeftArm_Notify`
  ;[1 1 1] Attacking
  (bind _isa (`/Engine/EditorBlueprintResources/StandardMacros.FlipFlop`)
    (:`A`
      _)
    (:`B`
      _))
  (`KismetArrayLibrary.Array_Clear` (`self.IgnoredActors`))
  (set `PrimitiveComponent.bGenerateOverlapEvents` _isa (`self.Hitbox_l`)))

(event `self.Hitbox_l.OnComponentBeginOverlap`
  (params (OverlappedComponent :type "PrimitiveComponent Object Reference") (OtherActor :type "Actor Object Reference") (OtherComp :type "PrimitiveComponent Object Reference") (OtherBodyIndex :type Integer) (bFromSweep :type Boolean) (SweepResult :type "HitResult Structure (by ref)"))
  ;[1 1 1] Attacking
  (cast `/Game/GameplayAbilities/Entities/Characters/Zombies/Blueprints/BP_Zombie` OtherActor
    (:`CastFailed`
      (if (not (`KismetArrayLibrary.Array_Contains` (`self.IgnoredActors`) OtherActor))
        (`KismetArrayLibrary.Array_Add` (`self.IgnoredActors`) OtherActor)
        (`AbilitySystemComponent.BP_ApplyGameplayEffectToTarget` :`self` (`self.RenamedAbilitySystem`) :`GameplayEffectClass` "/Game/GameplayAbilities/Entities/Characters/Zombies/Blueprints/Abilities/GE_ZombieAttack.GE_ZombieAttack_C" :`Target` (`AbilitySystemBlueprintLibrary.GetAbilitySystemComponent` OtherActor) :`Level` 1.0)
        (`KismetSystemLibrary.PrintString` "Left")))))

(event `self.Hitbox_r.OnComponentBeginOverlap`
  (params (OverlappedComponent :type "PrimitiveComponent Object Reference") (OtherActor :type "Actor Object Reference") (OtherComp :type "PrimitiveComponent Object Reference") (OtherBodyIndex :type Integer) (bFromSweep :type Boolean) (SweepResult :type "HitResult Structure (by ref)"))
  ;[1 1 1] Attacking
  (cast `/Game/GameplayAbilities/Entities/Characters/Zombies/Blueprints/BP_Zombie` OtherActor
    (:`CastFailed`
      (if (not (`KismetArrayLibrary.Array_Contains` (`self.IgnoredActors`) OtherActor))
        (`KismetArrayLibrary.Array_Add` (`self.IgnoredActors`) OtherActor)
        (`AbilitySystemComponent.BP_ApplyGameplayEffectToTarget` :`self` (`self.RenamedAbilitySystem`) :`GameplayEffectClass` "/Game/GameplayAbilities/Entities/Characters/Zombies/Blueprints/Abilities/GE_ZombieAttack.GE_ZombieAttack_C" :`Target` (`AbilitySystemBlueprintLibrary.GetAbilitySystemComponent` OtherActor) :`Level` 1.0)
        (`KismetSystemLibrary.PrintString` "Right")))))

(event `self.Voice.OnAudioFinished`
  (bind _sound (`self.Sound`))
  ;[1 1 1] Make different sounds every time
  (`AudioComponent.SetSound` (`self.Voice`) (`|GetArrayItem` _sound (`KismetMathLibrary.RandomInteger` (- (`KismetArrayLibrary.Array_Length` _sound) 1)))))

(event `self.OnDeath`
  (`KismetSystemLibrary.PrintString` "Dead...")
  (`self.SetLifeSpan` (`self.DeathLifespan`)))

(fn `UserConstructionScript`
  (`parent.UserConstructionScript`))