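; AI controller for zombie characters that starts the BT_Zombie behavior tree on BeginPlay.
; StopLogic and RestartLogic events pass through to the brain component to halt or restart the AI.
; Run and Walk events start and stop sprinting on the pawn's GACharacterMovementComponent, both only when CanSprint is true.
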(event `self.ReceiveBeginPlay`
  (`self.RunBehaviorTree` "/Game/GameplayAbilities/Entities/Characters/Zombies/Blueprints/AI/BT_Zombie.BT_Zombie"))

(event `StopLogic`
  (params (Reason :type String))
  (`BrainComponent.StopLogic` (`self.BrainComponent`) Reason))

(event `RestartLogic`
  (`BrainComponent.RestartLogic` (`self.BrainComponent`)))

(event `Run`
  (bind (_asgacharacter_movement_component _bsuccess) (cast `GACharacterMovementComponent` (`Pawn.GetMovementComponent` (`self.K2_GetPawn`)) :!pure true))
  (if _bsuccess
    (if (`GACharacterMovementComponent.bCanSprint` _asgacharacter_movement_component)
      (`GACharacterMovementComponent.StartSprinting` _asgacharacter_movement_component))))

(event `Walk`
  (bind (_asgacharacter_movement_component _bsuccess) (cast `GACharacterMovementComponent` (`Pawn.GetMovementComponent` (`self.K2_GetPawn`)) :!pure true))
  (if _bsuccess
    (if (`GACharacterMovementComponent.bCanSprint` _asgacharacter_movement_component)
      (`GACharacterMovementComponent.StopSprinting` _asgacharacter_movement_component))))

(fn `UserConstructionScript`)