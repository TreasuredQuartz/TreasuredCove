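; BP_MovementTrail is a short-lived trail actor whose plane uses a snow brush subtraction material, apparently to mark movement in snow.
; BeginPlay gives the actor a fixed lifespan and creates a dynamic material instance on the plane.
; Each Tick scales the material's Radius by remaining lifespan, so the brush shrinks until the actor expires.
; Tick writes Radius twice, so the second, halved value takes effect.
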(event `self.ReceiveBeginPlay`
  (`self.SetLifeSpan` 5.0)
  (bind _returnvalue (`PrimitiveComponent.CreateDynamicMaterialInstance` (`self.Plane`) 0 "/Game/GameplayAbilities/Maps/MainWorld/QuartzDungeon/Blueprints/RuntimeSnowField/M_SnowBrush_Subtraction.M_SnowBrush_Subtraction" "None"))
  (set `self.MID` _returnvalue))

(event `self.ReceiveTick`
  (params (DeltaSeconds :type "Float (single-precision)"))
  (bind _returnvalue (/ (`self.GetLifeSpan`) (`self.InitialLifeSpan`)))
  (`MaterialInstanceDynamic.SetScalarParameterValue` (`self.MID`) "Radius" _returnvalue)
  (`MaterialInstanceDynamic.SetScalarParameterValue` (`self.MID`) "Radius" (* _returnvalue 0.5)))

(fn `UserConstructionScript`)