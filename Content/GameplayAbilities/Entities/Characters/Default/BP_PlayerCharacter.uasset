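; BP_PlayerCharacter is the player character Blueprint, which here mainly handles the camera when the player dies.
; OnDeath switches the FirstPerson component out of first-person view, then detaches CameraArm in place and disables its collision test.
; While IsDead, Tick steadily lengthens the arm and adds controller pitch input until the arm's pitch reaches a limit.
; Mesh dynamic-material setup and GrassAffector show-only logic are present but never run.
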(event `self.ReceiveBeginPlay`
  (`parent.ReceiveBeginPlay`)
  (`|ExecutionSequence`))

(event `self.OnDeath`
  (bind _cameraarm (`self.CameraArm`))
  (if (`FirstPersonComponent.IsFirstPerson` (`self.FirstPerson`))
    (`FirstPersonComponent.ChangeViewpoint` (`self.FirstPerson`) false))
  (`SceneComponent.K2_DetachFromComponent` _cameraarm "KeepWorld" "KeepWorld" "KeepWorld" true)
  (set `SpringArmComponent.bDoCollisionTest` false _cameraarm))

(event `self.ReceiveTick`
  (params (DeltaSeconds :type "Float (single-precision)"))
  (bind _cameraarm (`self.CameraArm`))
  (if (`self.bIsDead`)
    (set `SpringArmComponent.TargetArmLength` (+ (`SpringArmComponent.TargetArmLength` _cameraarm) (* DeltaSeconds 100.0)) _cameraarm)
    (if (< (.pitch (`SceneComponent.K2_GetComponentRotation` _cameraarm)) 85.0)
      (`self.AddControllerPitchInput` (* DeltaSeconds 10.0)))))

(fn `UserConstructionScript`)