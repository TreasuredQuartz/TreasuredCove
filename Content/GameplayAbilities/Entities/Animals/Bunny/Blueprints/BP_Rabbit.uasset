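; BP_Rabbit is a rabbit animal Blueprint that tracks nearby grass foliage as potential food.
; Overlap events on FoodDetectionSphere store the first valid foliage component using the GrassClipPlane mesh and maintain a list of overlapped instance indices.
; FindFood picks a random index from that list and returns the instance's transform in component-local space, treating individual foliage instances as food without separate actors.
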(event `self.FoodDetectionSphere.OnComponentBeginOverlap`
  (params (OverlappedComponent :type "PrimitiveComponent Object Reference") (OtherActor :type "Actor Object Reference") (OtherComp :type "PrimitiveComponent Object Reference") (OtherBodyIndex :type Integer) (bFromSweep :type Boolean) (SweepResult :type "HitResult Structure (by ref)"))
  (bind _asfoliage_instanced_static_mesh_component (cast `FoliageInstancedStaticMeshComponent` OverlappedComponent))
  (if (== (`StaticMeshComponent.StaticMesh` _asfoliage_instanced_static_mesh_component) "/Game/GameplayAbilities/Entities/Environment/Grass/Mesh/GrassClipPlane.GrassClipPlane")
    (`/Engine/EditorBlueprintResources/StandardMacros.IsValid` (`self.FoliageFoodInstance`)
      (:`Is Valid`
        _)
      (:`Is Not Valid`
        (set `self.FoliageFoodInstance` _asfoliage_instanced_static_mesh_component)))
    (`KismetArrayLibrary.Array_Add` (`self.Indecies`) OtherBodyIndex)))

(event `self.FoodDetectionSphere.OnComponentEndOverlap`
  (params (OverlappedComponent :type "PrimitiveComponent Object Reference") (OtherActor :type "Actor Object Reference") (OtherComp :type "PrimitiveComponent Object Reference") (OtherBodyIndex :type Integer))
  (bind _returnvalue (`KismetArrayLibrary.Array_Find` (`self.Indecies`) OtherBodyIndex))
  (bind _asfoliage_instanced_static_mesh_component (cast `FoliageInstancedStaticMeshComponent` OverlappedComponent))
  (if (== _asfoliage_instanced_static_mesh_component (`self.FoliageFoodInstance`))
    (if (> _returnvalue -1)
      (`KismetArrayLibrary.Array_Remove` (`self.Indecies`) _returnvalue))))

(fn `FindFood`
  (returns (OutInstanceTransform :type "Transform Structure"))
  (return (`InstancedStaticMeshComponent.GetInstanceTransform` (`self.FoliageFoodInstance`) (`|GetArrayItem` (`self.Indecies`) (`KismetMathLibrary.RandomIntegerInRange` 0 (- (`KismetArrayLibrary.Array_Length` (`self.Indecies`)) -1))) false)))

(fn `UserConstructionScript`)