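; Slime actor that tracks a movement-lagged center offset and feeds the ground position to its material, updating only from the Construction Script.
; Each update pushes the offset opposite to movement, clamped to the object's size.
; A vertical trace at the offset center finds static ground and writes the hit to the material's Ground parameter if the MID is valid.
; Tick is empty, and MID creation and component repositioning are disconnected.
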(event `InitializeMID`
  (bind _returnvalue (+ (`self.SlimeCenterOffset`) (`self.K2_GetActorLocation`)))
  (`/Engine/EditorBlueprintResources/StandardMacros.IsValid` (`self.MID`)
    (:`Is Valid`
      (bind (_outhit _returnvalue_2) (`KismetSystemLibrary.LineTraceSingleForObjects` (+ (* (`KismetMathLibrary.Vector_Up`) (`self.ObjectSize`)) _returnvalue) (+ _returnvalue (* (`KismetMathLibrary.Vector_Down`) (`self.ObjectSize`))) (`|MakeArray` "ObjectTypeQuery1" :!type "EObjectTypeQuery Enum")))
      (if _returnvalue_2
        (`self.SetGroundLocation` (`.Location` (`GameplayStatics.BreakHitResult` _outhit)))))))

(event `SetGroundLocation`
  (params (GroundLocation :type "Vector Structure"))
  (bind _output_get (set `self.GroundLocation` GroundLocation))
  (`MaterialInstanceDynamic.SetVectorParameterValue` (`self.MID`) "Ground" (`KismetMathLibrary.Conv_VectorToLinearColor` _output_get)))

(event `Update`
  (`|ExecutionSequence`
    (:`then_0`
      (set `self.SlimeCenterOffset` (`KismetMathLibrary.Conv_VectorToVector2D` (`KismetMathLibrary.ClampVectorSize` (+ (`self.SlimeCenterOffset`) (* (`KismetMathLibrary.Normal` (- (`self.PreviousLocation`) (`self.K2_GetActorLocation`))) (`self.CenterOffsetSpeed`))) 0.0 (`KismetMathLibrary.Conv_IntToDouble` (`self.ObjectSize`))))))
    (:`then_1`
      (`self.OnUpdated`))))

(event `OnUpdated`
  (set `self.PreviousLocation` (`self.K2_GetActorLocation`)))

(event `self.ReceiveTick`
  (params (DeltaSeconds :type "Float (single-precision)")))

(fn `UserConstructionScript`
  (`self.Update`)
  (`self.InitializeMID`))