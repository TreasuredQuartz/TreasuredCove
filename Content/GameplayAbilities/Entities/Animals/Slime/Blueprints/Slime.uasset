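; Slime actor Blueprint that turns on capsule physics at BeginPlay and holds experimental helpers for building a procedural spherical mesh.
; Fibonacci functions generate sphere points or a 2D lattice, which a nearest-neighbour pass can triangulate into an index buffer with winding checks.
; A Bowyer-Watson triangulation with a circumcircle test is disconnected from its entry.
; Debug functions draw points and edges, and no event calls any of these helpers.
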(event `self.ReceiveBeginPlay`
  (`parent.ReceiveBeginPlay`)
  (`PrimitiveComponent.SetSimulatePhysics` (`self.CapsuleComponent`) true))

(fn `BowyerWatson`
  (params (Points :type "Array of Vector Structure (by ref)"))
  (returns (Triangles :type "Array of Integer"))
  (locals (LocTriangles :type "Array of /Game/GameplayAbilities/Entities/Animals/Slime/Blueprints/Triangle_Helper Structure") (LocTriangleNum :type Integer) (LocBadTriangles :type "Array of /Game/GameplayAbilities/Entities/Animals/Slime/Blueprints/Triangle_Helper Structure") (LocPolygon :type "Array of Integer") (LocPointsToCkeck :type "Array of Vector Structure") (SuperTriangle :type "/Game/GameplayAbilities/Entities/Animals/Slime/Blueprints/Triangle_Helper Structure") (LocReturnTriangles :type "Array of Integer"))
  ;[0 1 0.07173] Initialize Local variables...
)

(fn `FormSphereFromLongLatCoords`
  (params (LongLatCoords :type "Array of Vector2D Structure (by ref)"))
  (locals (CurIndex :type Integer))
  (bind _radius (`self.Radius`))
  (set `local.CurIndex` (- (`self.NumVertices`) 1))
  (for (_array_element _array_index) LongLatCoords
    (bind (_x _y) (`KismetMathLibrary.BreakVector2D` _array_element))
    (`KismetArrayLibrary.Array_Set` (`self.VertexBuffer`) _array_index (`KismetMathLibrary.MakeVector` (* _x _radius) (* _y _radius)) true)))

(fn `Generate2DFibonacciLattice`
  (returns (NumVertices :type Integer) (`2DLattice` :type "Array of Vector2D Structure"))
  (locals (CurIndex :type Integer) (CurRadius :type "Float (double-precision)") (CurTheta :type "Float (double-precision)") (CurFibIndex :type "Float (double-precision)") (x :type "Float (double-precision)") (y :type "Float (double-precision)") (LongLatCoords :type "Array of Vector2D Structure") (GoldenRatio :type "Float (double-precision)"))
  (set `local.CurIndex` 0)
  (set `self.Resolution` (`self.NumVertices`))
  (set `local.GoldenRatio` (+ 1.0 (`KismetMathLibrary.Sqrt` 5.0)))
  (`KismetArrayLibrary.Array_Resize` (`local.LongLatCoords`) (`self.Resolution`))
  (while (< (`local.CurIndex`) (`self.Resolution`))
    (set `local.CurFibIndex` (+ (`KismetMathLibrary.Conv_IntToDouble` (`local.CurIndex`)) 0.5))
    (set `local.CurRadius` (`KismetMathLibrary.Sqrt` (/ (`local.CurFibIndex`) (`KismetMathLibrary.Conv_IntToDouble` (`self.Resolution`)))))
    (set `local.CurTheta` (* (`KismetMathLibrary.GetPI`) (`local.GoldenRatio`) (`local.CurFibIndex`)))
    ;[1 1 1] This is in radians
    (set `local.x` (* (`KismetMathLibrary.Cos` (`local.CurTheta`)) (`local.CurRadius`) 0.5))
    (set `local.y` (* (`KismetMathLibrary.Sin` (`local.CurTheta`)) (`local.CurRadius`) 0.5))
    (`KismetArrayLibrary.Array_Set` (`local.LongLatCoords`) (`local.CurIndex`) (`KismetMathLibrary.MakeVector2D` (`local.x`) (`local.y`)) true)
    (`/Engine/EditorBlueprintResources/StandardMacros.IncrementInt` (`local.CurIndex`)))
  (return (* (`local.CurIndex`) 2) (`local.LongLatCoords`)))

(fn `Generate3DFibonacciPoints`
  (for _index (range (`self.NumVertices`))
    (bind _returnvalue (+ (`KismetMathLibrary.Conv_IntToDouble` _index) 0.5))
    (bind _returnvalue_2 (`KismetMathLibrary.Acos` (- 1.0 (/ (* _returnvalue 2.0) (`KismetMathLibrary.Conv_IntToDouble` (`self.NumVertices`))))))
    (bind _returnvalue_3 (`KismetMathLibrary.Cos` _returnvalue_2))
    (if (== _returnvalue_3 0.0)
      (bind _returnvalue_4 (* _returnvalue (`KismetMathLibrary.MultiplyByPi` (+ 1.0 (`KismetMathLibrary.Sqrt` 5.0)))))
      (bind _returnvalue_5 (`KismetMathLibrary.Sin` _returnvalue_2))
      (bind _returnvalue_6 (* (`KismetMathLibrary.MakeVector` (* (`KismetMathLibrary.Cos` _returnvalue_4) _returnvalue_5) (* (`KismetMathLibrary.Sin` _returnvalue_4) _returnvalue_5) _returnvalue_3) (`self.Radius`)))
      (`KismetArrayLibrary.Array_Add` (`self.VertexBuffer`) _returnvalue_6))
    (`KismetArrayLibrary.Array_Add` (`self.VertexBuffer`) _returnvalue_6))
  (return))

(fn `InCircle`
  (params (Points :type "Array of Vector Structure (by ref)") (TriangleToCheck :type "/Game/GameplayAbilities/Entities/Animals/Slime/Blueprints/Triangle_Helper Structure (by ref)") (PointToCheck :type "Vector Structure (by ref)"))
  (returns (isInCircle :type Boolean))
  (locals (ax :type "Float (double-precision)") (ay :type "Float (double-precision)") (az :type "Float (double-precision)") (bx :type "Float (double-precision)") (by :type "Float (double-precision)") (bz :type "Float (double-precision)") (cx :type "Float (double-precision)") (cy :type "Float (double-precision)") (cz :type "Float (double-precision)"))
  (bind (_a _b _c) (break `/Game/GameplayAbilities/Entities/Animals/Slime/Blueprints/Triangle_Helper` TriangleToCheck))
  (bind _output (`|GetArrayItem` Points _a))
  (bind _returnvalue (- (`|GetArrayItem` Points _c) _output))
  (bind _returnvalue_2 (- (`|GetArrayItem` Points _b) _output))
  (bind _returnvalue_3 (`KismetMathLibrary.Cross_VectorVector` _returnvalue_2 _returnvalue))
  (bind _returnvalue_4 (/ (+ (* (`KismetMathLibrary.Cross_VectorVector` _returnvalue_3 _returnvalue_2) (`KismetMathLibrary.VSizeSquared` _returnvalue)) (* (`KismetMathLibrary.Cross_VectorVector` _returnvalue _returnvalue_3) (`KismetMathLibrary.VSizeSquared` _returnvalue_2))) (* (`KismetMathLibrary.VSizeSquared` _returnvalue_3) 2.0)))
  (return (< (`KismetMathLibrary.Vector_Distance` (+ _output _returnvalue_4) PointToCheck) (`KismetMathLibrary.VSizeSquared` _returnvalue_4))))

(fn `Is Clockwise (Vector)`
  (params (Points :type "Array of Vector Structure (by ref)") (Triangle :type "Array of Integer (by ref)"))
  (returns (IsClockwise :type Boolean))
  (locals (LocPoints :type "Array of Vector Structure"))
  (bind _locpoints (`local.LocPoints`))
  (bind (_output_x _output_y) (`KismetMathLibrary.BreakVector` (`|GetArrayItem` _locpoints 2)))
  (bind (_output_x_2 _output_y_2) (`KismetMathLibrary.BreakVector` (`|GetArrayItem` _locpoints)))
  (bind (_output_x_3 _output_y_3) (`KismetMathLibrary.BreakVector` (`|GetArrayItem` _locpoints 1)))
  (for _array_element Triangle
    (`KismetArrayLibrary.Array_Add` (`local.LocPoints`) (`|GetArrayItem` Points _array_element)))
  (return (> (- (* (- _output_x_3 _output_x_2) (- _output_y _output_y_2)) (* (- _output_x _output_x_2) (- _output_y_3 _output_y_2))) 0.0)))

(fn `Is Clockwise (Vector2D)`
  (params (Points :type "Array of Vector2D Structure (by ref)") (Triangle :type "Array of Integer (by ref)"))
  (returns (IsClockwise :type Boolean))
  (locals (LocPoints :type "Array of Vector2D Structure"))
  (bind _locpoints (`local.LocPoints`))
  (bind (_output_x _output_y) (`KismetMathLibrary.BreakVector2D` (`|GetArrayItem` _locpoints 2)))
  (bind (_output_x_2 _output_y_2) (`KismetMathLibrary.BreakVector2D` (`|GetArrayItem` _locpoints)))
  (bind (_output_x_3 _output_y_3) (`KismetMathLibrary.BreakVector2D` (`|GetArrayItem` _locpoints 1)))
  (for _array_element Triangle
    (`KismetArrayLibrary.Array_Add` (`local.LocPoints`) (`|GetArrayItem` Points _array_element)))
  (return (> (- (* (- _output_x_3 _output_x_2) (- _output_y _output_y_2)) (* (- _output_x _output_x_2) (- _output_y_3 _output_y_2))) 0.0)))

(fn `Triangles2DFibonacciLattice`
  (params (`2DCoords` :type "Array of Vector2D Structure (by ref)"))
  (locals (MinDistance :type "Float (double-precision)" :default 100.0) (Edges :type "Array of Integer"))
  (bind _edges (`local.Edges`))
  (bind _edges_2 (`local.Edges`))
  (for (_array_element _array_index) `2DCoords`
    (set `local.MinDistance` 100.0)
    (set `local.Edges` (`|MakeArray` _array_index))
    (for _array_element_2 `2DCoords`
      (bind _returnvalue (`KismetMathLibrary.Distance2D` _array_element _array_element_2))
      (if (< _returnvalue (`local.MinDistance`))
        (set `local.MinDistance` _returnvalue)))
    (for (_array_element_3 _array_index_2) `2DCoords`
      (if (<= (`KismetMathLibrary.Distance2D` _array_element _array_element_3) (* (`local.MinDistance`) 1.2))
        (if (not (`KismetArrayLibrary.Array_Contains` (`local.Edges`) _array_index_2))
          (`KismetArrayLibrary.Array_Add` (`local.Edges`) _array_index_2)
          (if (> (`KismetArrayLibrary.Array_Length` (`local.Edges`)) 2)
            (if (`self.Is Clockwise (Vector2D)` `2DCoords` (`local.Edges`))
              (`KismetArrayLibrary.Array_Swap` _edges 1 2))
            (`KismetArrayLibrary.Array_Append` (`self.TrianglesBuffer`) _edges)
            (`KismetArrayLibrary.Array_Remove` _edges_2 1)
            (`KismetArrayLibrary.Array_Remove` _edges_2 2))))))
  (return))

(fn `UserConstructionScript`
  (`parent.UserConstructionScript`))

(fn `VisualizeLattice`
  (params (Points :type "Array of Vector2D Structure"))
  (bind _radius (`self.Radius`))
  (bind _returnvalue (`|AddComponentByClass` "/Script/Engine.InstancedStaticMeshComponent"))
  (`StaticMeshComponent.SetStaticMesh` _returnvalue "/Engine/EngineMeshes/Sphere.Sphere")
  (for _array_element Points
    (`InstancedStaticMeshComponent.AddInstance` _returnvalue (`KismetMathLibrary.MakeTransform` (`KismetMathLibrary.MakeVector` (* (`KismetMathLibrary.BreakVector2D` _array_element) _radius) (* (`.Y` (`KismetMathLibrary.BreakVector2D` _array_element)) _radius)) (struct) (0.025 0.025 0.025)) false)))

(fn `VisualizeSphereEdges`
  (params (Points :type "Array of Vector Structure (by ref)") (Triangles :type "Array of Integer (by ref)"))
  (locals (LocPrevPoint :type "Vector Structure"))
  (for (_array_element _array_index) Triangles
    (if (!= _array_index 0)
      (bind _output (`|GetArrayItem` Points _array_element))
      (`KismetSystemLibrary.DrawDebugLine` (`local.LocPrevPoint`) _output (struct) 10.0 0.25))
    (set `local.LocPrevPoint` _output)))

(fn `VisualizeSpherePoints`
  (params (Points :type "Array of Vector Structure (by ref)"))
  (bind _returnvalue (`|AddComponentByClass` "/Script/Engine.InstancedStaticMeshComponent"))
  (`StaticMeshComponent.SetStaticMesh` _returnvalue "/Engine/EngineMeshes/Sphere.Sphere")
  (for _array_element Points
    (`InstancedStaticMeshComponent.AddInstance` _returnvalue (`KismetMathLibrary.MakeTransform` _array_element (struct) (0.025 0.025 0.025)) false)))