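; Player-enterable Arwing vehicle pawn that announces interactability through an overlap trigger and wakes its vehicle movement component when possessed.
; Inputs feed throttle, steering and look, while boosting adds physics force to the mesh each tick.
; Transition events switch between top-down, shooter and free-range modes, using a timeline to animate camera and mesh.
; Custom movement for those modes (clamped offsets, leaning, thrust-versus-gravity) remains, but its Tick dispatch is disconnected.
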(event `self.ReceiveBeginPlay`
  ;[0 0.1015 1] Begin Play
  (`TimelineComponent.SetPlayRate` (`self.TopDownTimeline`) (`self.TopDownTransitionSpeed`))
  (`ChaosVehicleMovementComponent.SetSleeping` (`self.VehicleMovementComponent`) true))

(event `self.EnterTrigger.OnComponentBeginOverlap`
  (params (OverlappedComponent :type "PrimitiveComponent Object Reference") (OtherActor :type "Actor Object Reference") (OtherComp :type "PrimitiveComponent Object Reference") (OtherBodyIndex :type Integer) (bFromSweep :type Boolean) (SweepResult :type "HitResult Structure (by ref)"))
  ;[0.7552 0.39 0.09379] Interaction  interface
  (message `InteractionInterface.NotifyCanInteract` OtherActor (`self.Name`) true))

(event `self.EnterTrigger.OnComponentEndOverlap`
  (params (OverlappedComponent :type "PrimitiveComponent Object Reference") (OtherActor :type "Actor Object Reference") (OtherComp :type "PrimitiveComponent Object Reference") (OtherBodyIndex :type Integer))
  ;[0.7552 0.39 0.09379] Interaction  interface
  (message `InteractionInterface.NotifyCanInteract` OtherActor (`self.Name`) false))

(event `self.ReceivePossessed`
  (params (NewController :type "Controller Object Reference"))
  ;[0 0.104 1] Possessed
  (`parent.ReceivePossessed` NewController)
  (`ChaosVehicleMovementComponent.SetSleeping` (`self.VehicleMovementComponent`) false))

(event `self.MoveForward`
  (params (AxisValue :type "Float (single-precision)"))
  ;[1 0.2344 0.2344] Inputs
  (`ChaosVehicleMovementComponent.SetThrottleInput` (`self.VehicleMovementComponent`) AxisValue))

(event `self.Throttle`
  ;[1 0.2344 0.2344] Inputs
  (set `self.bBoosting?` true))

(event `TransitionTopDown`
  (bind _mesh (`self.Mesh`))
  ;[0 0 0] Transition
  (set `self.Speed` 10000.0)
  (set `self.TopDown?` true)
  (bind _asplayer_controller (cast `PlayerController` (`self.GetController`)))
  (`self.DisableInput` _asplayer_controller)
  (bind (_direction _topdownfloatcurve) (`Timeline|TopDownTimeline` :!via `PlayFromStart` :!label _label)
    (:`Update`
      (`SceneComponent.K2_SetRelativeRotation` (`self.SpringArm`) (`KismetMathLibrary.RLerp` (struct) (struct :`Pitch` -90.0) _topdownfloatcurve) false false)
      (set `SpringArmComponent.TargetArmLength` (`KismetMathLibrary.Lerp` 1280.0 10000.0 _topdownfloatcurve) (`self.SpringArm`))
      (`SceneComponent.K2_SetRelativeLocation` _mesh (`KismetMathLibrary.VInterpTo` (`SceneComponent.RelativeLocation` (`self.Mesh`)) (0.0 0.0 0.0) _topdownfloatcurve 1.0) false false)
      (`SceneComponent.K2_SetRelativeRotation` _mesh (`KismetMathLibrary.RInterpTo` (`SceneComponent.RelativeRotation` _mesh) (struct :`Yaw` -90.0) _topdownfloatcurve 1.0) false false))
    (:`Finished`
      (set `self.CurrentLocOffset` (0.0 0.0))
      (bind _asplayer_controller_2 (cast `PlayerController` (`self.GetController`)))
      (`self.EnableInput` _asplayer_controller_2))))

(event `self.MoveRight`
  (params (AxisValue :type "Float (single-precision)"))
  ;[1 0.2344 0.2344] Inputs
  (`ChaosVehicleMovementComponent.SetSteeringInput` (`self.VehicleMovementComponent`) AxisValue))

(event `TransitionShooter`
  ;[0 0 0] Transition
  (set `self.Speed` 1000.0)
  (set `self.TopDown?` false)
  (bind _asplayer_controller (cast `PlayerController` (`self.GetController`) :!label _label_2))
  (`self.DisableInput` _asplayer_controller)
  (goto _label :!via `Reverse`))

(event `self.ReceiveTick`
  (params (DeltaSeconds :type "Float (single-precision)"))
  (if (`self.bBoosting?`)
    (`PhysicsThreadLibrary.AddForce` (`PrimitiveComponent.GetBodyInstanceAsyncPhysicsTickHandle` (`self.Mesh`) "None" true -1) (* (100000.0 0.0 0.0) DeltaSeconds))))

(event `self.LookUp`
  (params (AxisValue :type "Float (single-precision)"))
  ;[1 0.2344 0.2344] Inputs
  (`self.AddControllerPitchInput` AxisValue))

(event `PerformMove`
  ;[1 0.2344 0.2344] Inputs
  (bind _returnvalue (`self.ConsumeMovementInputVector`))
  (set `self.Velocity` (* _returnvalue (`self.Speed`))))

(event `TransitionFreeRange`
  ;[0 0 0] Transition
  (set `self.Speed` (`self.MinThrustToOvercomeGravity`))
  (set `self.bGrounded` false)
  (set `self.TopDown?` false)
  (goto _label_2))

(event `self.LookRight`
  (params (AxisValue :type "Float (single-precision)"))
  ;[1 0.2344 0.2344] Inputs
  (`self.AddControllerYawInput` AxisValue))

(event `ReplicateRotation`
  (params (DeltaSeconds :type "Float (double-precision)"))
  (bind (_returnvalue_x _returnvalue_y _returnvalue_z) (`KismetMathLibrary.BreakVector` (`KismetMathLibrary.Normal` (`self.Velocity`))))
  (bind (_returnvalue_roll _returnvalue_pitch) (`KismetMathLibrary.BreakRotator` (`KismetMathLibrary.RInterpTo` (`SceneComponent.RelativeRotation` (`self.Mesh`)) (`KismetMathLibrary.MakeRotFromYZ` (`self.AimTarget`) (`SceneComponent.GetUpVector` (`self.Camera`))) DeltaSeconds 10.0)))
  ;[0.4413 0 0.474] Shooter
  (set `self.AimTarget` (`KismetMathLibrary.MakeVector` 1.0 _returnvalue_y _returnvalue_z))
  (`SceneComponent.K2_SetRelativeRotation` (`self.Mesh`) (`KismetMathLibrary.MakeRotator` _returnvalue_roll _returnvalue_pitch -90.0) false false))

(event `FreeRangeMovement`
  (params (DeltaSeconds :type "Float (double-precision)"))
  (bind _returnvalue (`self.K2_GetActorLocation`))
  ;[0 0.0615 1] FreeRangeMovement
  (if (not (`KismetMathLibrary.NearlyEqual_FloatFloat` DeltaSeconds))
    (set `self.Speed` (select `bool` (< (`self.ThrustSpeed`) (`self.Speed`)) :`false` (`self.ThrustSpeed`) :`true` (`KismetMathLibrary.FInterpTo` (`self.Speed`) (`self.ThrustSpeed`) DeltaSeconds (`self.Drag`)) :!type "Float (double-precision)"))
    (if (`self.bGrounded`)
      (set `self.AppliedGravity` 980.0)
      (else
        (set `self.AppliedGravity` (`KismetMathLibrary.MapRangeClamped` (`self.Speed`) 0.0 (`self.MinThrustToOvercomeGravity`) 980.0))))
    (bind _output_get (set `self.Velocity` (+ (* (* (`self.Speed`) DeltaSeconds) (`self.GetActorForwardVector`)) (* (* (`self.AppliedGravity`) DeltaSeconds) (`KismetMathLibrary.Vector_Down`)) (`self.Velocity`))))
    (bind _returnvalue_2 (+ _returnvalue _output_get))
    (bind (_outhit _returnvalue_3) (`KismetSystemLibrary.BoxTraceSingle` _returnvalue _returnvalue_2 (250.0 250.0 100.0) (struct) "TraceTypeQuery1"))
    (`self.K2_SetActorLocation` _returnvalue_2)))

(event `HorizontalLean`
  (params (DeltaSeconds :type "Float (double-precision)"))
  (bind _mesh (`self.Mesh`))
  (bind (_relativerotation_roll _relativerotation_pitch _relativerotation_yaw) (`KismetMathLibrary.BreakRotator` (`SceneComponent.RelativeRotation` _mesh)))
  ;[0.4413 0 0.474] Shooter
  (`SceneComponent.K2_SetRelativeRotation` _mesh (`KismetMathLibrary.MakeRotator` _relativerotation_roll _relativerotation_pitch (`KismetMathLibrary.FInterpTo` _relativerotation_yaw (.y (`self.Velocity`)) DeltaSeconds 0.5)) false false))

(event `ShooterMovement`
  (params (DeltaSeconds :type "Float (double-precision)"))
  (bind (_clampedoffset_x _clampedoffset_y) (`KismetMathLibrary.BreakVector2D` (`self.ShooterClampedLocation` DeltaSeconds)))
  ;[0.4413 0 0.474] Shooter
  (if (not (`KismetMathLibrary.NearlyEqual_FloatFloat` DeltaSeconds 0.0 0.01))
    (`self.PerformMove`)
    (`self.ReplicateRotation` DeltaSeconds)
    (`self.HorizontalLean` DeltaSeconds)
    (if (not (`KismetMathLibrary.Vector_IsNearlyZero` (`self.Velocity`)))
      (`SceneComponent.K2_SetRelativeLocation` (`self.Mesh`) (`KismetMathLibrary.MakeVector` 0.0 _clampedoffset_x _clampedoffset_y) false false))))

(event `TopDownMovement`
  (params (DeltaSeconds :type "Float (double-precision)"))
  (bind (_x _y) (`KismetMathLibrary.BreakVector2D` (`self.TopDownClampedLocation` DeltaSeconds)))
  ;[0.5729 0 0] Top Down
  (if (not (`KismetMathLibrary.NearlyEqual_FloatFloat` DeltaSeconds 0.0 0.01))
    (`self.PerformMove`)
    (if (not (`KismetMathLibrary.Vector_IsNearlyZero` (`self.Velocity`)))
      (`SceneComponent.K2_SetRelativeLocation` (`self.Mesh`) (`KismetMathLibrary.MakeVector` _x _y) false false))))

(fn `ShooterClampedLocation`
  (params (DeltaSeconds :type "Float (single-precision)"))
  (returns (ClampedOffset :type "Vector2D Structure"))
  (locals (LocNewLocation :type "Vector Structure"))
  (bind _hlimit (`self.HLimit`))
  (bind _vlimit (`self.VLimit`))
  (bind (_returnvalue_x _returnvalue_y _returnvalue_z) (`KismetMathLibrary.BreakVector` (* (`self.Velocity`) DeltaSeconds)))
  (bind (_x _y) (`KismetMathLibrary.BreakVector2D` (+ (`self.CurrentLocOffset`) (`KismetMathLibrary.MakeVector2D` _returnvalue_y _returnvalue_z))))
  (bind _output_get (set `self.CurrentLocOffset` (`KismetMathLibrary.MakeVector2D` (`KismetMathLibrary.FClamp` _x (- 0.0 _hlimit) _hlimit) (`KismetMathLibrary.FClamp` _y (- 0.0 _vlimit) _vlimit))))
  (return _output_get))

(fn `TopDownClampedLocation`
  (params (DeltaSeconds :type "Float (single-precision)"))
  (returns (`Offset'` :type "Vector2D Structure"))
  (bind (_returnvalue_x _returnvalue_y) (`KismetMathLibrary.BreakVector` (* (`self.Velocity`) DeltaSeconds)))
  (bind _returnvalue (* (`self.VLimit`) 10.0))
  (bind _returnvalue_2 (* (`self.HLimit`) 10.0))
  (bind (_x _y) (`KismetMathLibrary.BreakVector2D` (+ (`self.CurrentLocOffset`) (`KismetMathLibrary.MakeVector2D` _returnvalue_x _returnvalue_y))))
  (bind _output_get (set `self.CurrentLocOffset` (`KismetMathLibrary.MakeVector2D` (`KismetMathLibrary.FClamp` _x (- 0.0 _returnvalue_2) _returnvalue_2) (`KismetMathLibrary.FClamp` _y (- 0.0 _returnvalue) _returnvalue))))
  (return _output_get))

(fn `UpdatePitch`)

(fn `UpdatePosition`)

(fn `UpdateRoll`)

(fn `UpdateYaw`)

(fn `UserConstructionScript`)