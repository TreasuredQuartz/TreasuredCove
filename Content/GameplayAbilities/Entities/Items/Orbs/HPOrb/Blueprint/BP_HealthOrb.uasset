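; Health orb pickup Blueprint that restores health to the actor that picks it up, then destroys itself.
; The construction script randomizes the pickup quantity and, with a separate roll, the mesh scale, so size does not reflect value.
; On pickup it builds a GE_HealthOrb effect spec, passes the quantity as a SetByCaller magnitude under the Stats.health tag, and applies it to the other actor's Ability System Component.
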(event `self.ReceiveBeginPlay`
  (`parent.ReceiveBeginPlay`))

(event `PickupInterface.OnPickedUp`
  (params (OtherActor :type "Actor Object Reference"))
  (bind _returnvalue (`|GenericCreateObject` "/Game/GameplayAbilities/Entities/Items/Orbs/HPOrb/Ability/GE_HealthOrb.GE_HealthOrb_C"))
  (bind _returnvalue_2 (`AbilitySystemBlueprintLibrary.AssignTagSetByCallerMagnitude` (`AbilitySystemBlueprintLibrary.MakeSpecHandle` _returnvalue (`self.GetInstigator`) self) (struct :`TagName` "stats.health") (`KismetMathLibrary.Conv_IntToDouble` (`.Quantity` (break `ItemKey` (`self.PickupInfo`))))))
  (`AbilitySystemComponent.BP_ApplyGameplayEffectSpecToSelf` (`AbilitySystemBlueprintLibrary.GetAbilitySystemComponent` OtherActor) _returnvalue_2)
  (`self.K2_DestroyActor`))

(fn `UserConstructionScript`
  (bind _returnvalue (`KismetMathLibrary.RandomIntegerInRange` 1 10))
  (`parent.UserConstructionScript`)
  (setmembers `ItemKey` :`StructRef` (`self.PickupInfo`) :`Quantity` _returnvalue)
  (`SceneComponent.SetWorldScale3D` (`self.Mesh`) (`KismetMathLibrary.Conv_DoubleToVector` (/ _returnvalue 10.0 2.0))))