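; Openable chest that, on first interaction, hands the contents of its repository, category by category, to an interacting actor that has a RepositoryComponent.
; A looping timer drives the lid's vertex animation through a dynamic material's frame parameter.
; Late in the animation it triggers a Niagara effect and fades a white-light cube, then stops the timer and hides the cube.
; The construction script applies an optional override material.
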(event `InteractionInterface.InteractedWith`
  (params (OtherActor :type "Actor Object Reference"))
  (if (not (`self.bHasBeenOpened`))
    (`/Engine/EditorBlueprintResources/StandardMacros.IsValid` (`self.GetComponentByClass` OtherActor "/Script/TreasuredCove.RepositoryComponent")
      (:`Is Valid`
        (bind _keys (`BlueprintMapLibrary.Map_Keys` (`RepositoryComponent.Repository` (`self.Repository`))))
        (for _array_element _keys
          (bind (_value _returnvalue) (`BlueprintMapLibrary.Map_Find` (`RepositoryComponent.Repository` (`self.Repository`)) _array_element))
          (if _returnvalue
            (for _array_element_2 (`.Repository` (break `Repository` _value))
              (message `InteractionInterface.AddItemToRepository` OtherActor _array_element _array_element_2))
            (set `self.bHasBeenOpened` true)
            (`self.SetDynamicMaterial`)
            (bind _returnvalue_2 (`KismetSystemLibrary.K2_SetTimerDelegate` (delegate `VertexAnimation`) 0.05 true))))))))

(event `VertexAnimation`
  (bind _output_get (set `self.VertexAnimationTime` (+ 0.05 (`self.VertexAnimationTime`))))
  (`MaterialInstanceDynamic.SetScalarParameterValue` (`self.MID`) "CurrentAnimationFrame" _output_get)
  (if (>= (`self.VertexAnimationTime`) 0.6)
    (`|ExecutionSequence`
      (:`then_0`
        (`/Engine/EditorBlueprintResources/StandardMacros.DoOnce` false
          (:`Completed`
            (`ActorComponent.Activate` (`self.NS_OpenKHChest`) true)
            (bind _returnvalue (`PrimitiveComponent.CreateDynamicMaterialInstance` (`self.Cube`) 0 "/Game/GameplayAbilities/Materials/Originals/MI_WhiteLight.MI_WhiteLight" "None")))))
      (:`then_1`
        (`MaterialInstanceDynamic.SetScalarParameterValue` _returnvalue "Intensity" (`KismetMathLibrary.Lerp` 100.0 0.0 (/ (- (`self.VertexAnimationTime`) 0.6) 0.3)))
        (if (>= (`self.VertexAnimationTime`) 0.9)
          (`KismetSystemLibrary.K2_ClearAndInvalidateTimerHandle` (stale `InteractionInterface.InteractedWith` _returnvalue_2))
          (`ActorComponent.Deactivate` (`self.NS_OpenKHChest`))
          (set `self.MID` null)
          (`SceneComponent.SetHiddenInGame` (`self.Cube`) true false))))))

(fn `SetDynamicMaterial`
  (`/Engine/EditorBlueprintResources/StandardMacros.IsValid` (`self.MID`)
    (:`Is Valid`
      _)
    (:`Is Not Valid`
      (bind _returnvalue (`KismetMaterialLibrary.CreateDynamicMaterialInstance` (`PrimitiveComponent.GetMaterial` (`self.SM_KH_Chest_Test`) 0)))
      (set `self.MID` _returnvalue)))
  (`PrimitiveComponent.SetMaterial` (`self.SM_KH_Chest_Test`) 0 (`self.MID`)))

(fn `UserConstructionScript`
  (bind _override_material (`self.Override_Material`))
  (`parent.UserConstructionScript`)
  (`/Engine/EditorBlueprintResources/StandardMacros.IsValid` _override_material
    (:`Is Valid`
      (`PrimitiveComponent.SetMaterial` (`self.SM_KH_Chest_Test`) 0 _override_material))))