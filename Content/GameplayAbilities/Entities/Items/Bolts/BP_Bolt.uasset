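; BP_Bolt is a bolt item actor that takes on one of eleven hardware meshes at random, such as bolts, nuts, gears, springs and cross fittings.
; Its construction script calls RandomizeType to roll BoltType, selects the matching static mesh and applies BoltMaterial to it.
; Because the roll happens during construction, the shape can change whenever the construction script reruns.
; BeginPlay only calls the parent implementation.
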(event `self.ReceiveBeginPlay`
  (`parent.ReceiveBeginPlay`))

(event `RandomizeType`
  (set `self.BoltType` (`KismetMathLibrary.Conv_IntToByte` (`KismetMathLibrary.RandomIntegerInRange` 0 10))))

(fn `UserConstructionScript`
  (bind _mesh (`self.Mesh`))
  (`parent.UserConstructionScript`)
  (`self.RandomizeType`)
  (`StaticMeshComponent.SetStaticMesh` _mesh (select `byte` (`self.BoltType`) :`0` "/Game/GameplayAbilities/Entities/Items/Bolts/SM_Bolt.SM_Bolt" :`1` "/Game/GameplayAbilities/Entities/Items/Bolts/Nuts/SM_NutHex.SM_NutHex" :`2` "/Game/GameplayAbilities/Entities/Items/Bolts/Nuts/SM_NutStar.SM_NutStar" :`3` "/Game/GameplayAbilities/Entities/Items/Bolts/Gears/SM_Gears_LOD_00.SM_Gears_LOD_00" :`4` "/Game/GameplayAbilities/Entities/Items/Bolts/Gears/SM_GearsSolid_LOD_00.SM_GearsSolid_LOD_00" :`5` "/Game/GameplayAbilities/Entities/Items/Bolts/Spring/SM_Spring.SM_Spring" :`6` "/Game/GameplayAbilities/Entities/Items/Bolts/CrossFittings/SM_CrossFittingThree.SM_CrossFittingThree" :`7` "/Game/GameplayAbilities/Entities/Items/Bolts/CrossFittings/SM_CrossFittingSix.SM_CrossFittingSix" :`8` "/Game/GameplayAbilities/Entities/Items/Bolts/Nuts/SM_NutAcorn.SM_NutAcorn" :`9` "/Game/GameplayAbilities/Entities/Items/Bolts/Nuts/SM_NutWing.SM_NutWing" :`10` "/Game/GameplayAbilities/Entities/Items/Bolts/SM_BoltDoubleCapped.SM_BoltDoubleCapped" :!type "StaticMesh Object Reference"))
  (`PrimitiveComponent.SetMaterial` _mesh 0 (`self.BoltMaterial`)))