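; BP_Blizzard is a zombie power-up shockwave that freezes the zombies it overlaps.
; Each inherited shockwave step feeds the current radius to the Niagara effect.
; On overlap it shortens the zombie's death lifespan and applies GE_Blizzard from the instigator's ability system.
; It then spawns a BP_FrozenZombie at the mesh transform, passing that mesh as reference.
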(event `self.Shockwave_Step`
  (`parent.Shockwave_Step`)
  (`NiagaraComponent.SetVariableFloat` (`self.Niagara`) "Radius" (`self.CurrentRadius`)))

(event `self.Overlap.OnComponentBeginOverlap`
  (params (OverlappedComponent :type "PrimitiveComponent Object Reference") (OtherActor :type "Actor Object Reference") (OtherComp :type "PrimitiveComponent Object Reference") (OtherBodyIndex :type Integer) (bFromSweep :type Boolean) (SweepResult :type "HitResult Structure (by ref)"))
  (bind _returnvalue (`AbilitySystemBlueprintLibrary.GetAbilitySystemComponent` (`self.Instigator`)))
  (bind _asbp_zombie (cast `/Game/GameplayAbilities/Entities/Characters/Zombies/Blueprints/BP_Zombie` OtherActor))
  (set `/Game/GameplayAbilities/Entities/Characters/Zombies/Blueprints/BP_Zombie.DeathLifespan` 0.15 _asbp_zombie)
  (`/Engine/EditorBlueprintResources/StandardMacros.IsValid` _returnvalue
    (:`Is Valid`
      (bind _returnvalue_2 (`AbilitySystemBlueprintLibrary.GetAbilitySystemComponent` _asbp_zombie))
      (`/Engine/EditorBlueprintResources/StandardMacros.IsValid` _returnvalue_2
        (:`Is Valid`
          (`AbilitySystemComponent.BP_ApplyGameplayEffectToTarget` :`self` _returnvalue :`GameplayEffectClass` "/Game/GameplayAbilities/Entities/Items/ZombiePowerUpDrops/GE_Blizzard.GE_Blizzard_C" :`Target` _returnvalue_2)
          (bind _mesh (`Character.Mesh` _asbp_zombie))
          (`|SpawnActorFromClass` "/Game/GameplayAbilities/Entities/Items/ZombiePowerUpDrops/BP_FrozenZombie.BP_FrozenZombie_C" (`SceneComponent.K2_GetComponentToWorld` _mesh) "Undefined" "OverrideRootScale" null _mesh null))))))

(fn `UserConstructionScript`
  (`parent.UserConstructionScript`))