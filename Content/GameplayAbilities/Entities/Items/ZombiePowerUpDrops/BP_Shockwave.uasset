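; Expanding shockwave actor, filed under zombie power-up drops, that grows until its lifespan runs out.
; A looping 0.05-second timer multiplies the current radius by an expansion rate, so growth is exponential.
; Each step applies that value as both the visible sphere's world scale and the overlap sphere's radius, updating overlaps.
; The graph itself contains no overlap response.
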(event `self.ReceiveBeginPlay`
  (`KismetSystemLibrary.K2_SetTimerDelegate` (delegate `Shockwave_Step`) 0.05 true)
  (`self.SetLifeSpan` (`self.Lifetime`)))

(event `Shockwave_Step`
  (set `self.CurrentRadius` (* (`self.CurrentRadius`) (`self.ExpansionRate`)))
  (`SceneComponent.SetWorldScale3D` (`self.Sphere`) (`KismetMathLibrary.Conv_DoubleToVector` (`self.CurrentRadius`)))
  (`SphereComponent.SetSphereRadius` (`self.Overlap`) (`self.CurrentRadius`) true))

(fn `UserConstructionScript`)