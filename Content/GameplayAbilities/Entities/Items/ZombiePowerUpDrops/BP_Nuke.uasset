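; BP_Nuke is a zombie power-up drop item that spawns a BP_Blizzard actor when a pawn picks it up.
; On BeginPlay it points its RotatingMovement component at the Mesh so the mesh spins.
; OnPickedUp spawns the Blizzard at the drop's transform with the pawn as Instigator, then runs the parent pickup logic, which is skipped for non-pawn actors.
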(event `self.ReceiveBeginPlay`
  (`parent.ReceiveBeginPlay`)
  (`MovementComponent.SetUpdatedComponent` (`self.RotatingMovement`) (`self.Mesh`)))

(event `PickupInterface.OnPickedUp`
  (params (OtherActor :type "Actor Object Reference"))
  (bind _aspawn (cast `Pawn` OtherActor))
  (`|SpawnActorFromClass` "/Game/GameplayAbilities/Entities/Items/ZombiePowerUpDrops/BP_Blizzard.BP_Blizzard_C" (`self.GetTransform`) "Undefined" "OverrideRootScale" null _aspawn)
  (`parent.OnPickedUp` OtherActor))

(fn `UserConstructionScript`
  (`parent.UserConstructionScript`))