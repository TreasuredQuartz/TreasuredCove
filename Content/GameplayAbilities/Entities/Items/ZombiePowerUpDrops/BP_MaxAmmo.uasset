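; Max Ammo zombie power-up drop, a child Blueprint that relies on its parent class for pickup behavior.
; On BeginPlay it runs the parent logic, then points RotatingMovement at Mesh so the mesh is the component that spins.
; OnPickedUp and the construction script only call their parents, so this graph contains no ammo refill logic of its own.
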(event `self.ReceiveBeginPlay`
  (`parent.ReceiveBeginPlay`)
  (`MovementComponent.SetUpdatedComponent` (`self.RotatingMovement`) (`self.Mesh`)))

(event `PickupInterface.OnPickedUp`
  (params (OtherActor :type "Actor Object Reference"))
  (`parent.OnPickedUp` OtherActor))

(fn `UserConstructionScript`
  (`parent.UserConstructionScript`))