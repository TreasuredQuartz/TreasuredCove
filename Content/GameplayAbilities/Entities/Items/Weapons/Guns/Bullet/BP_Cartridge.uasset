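; BP_Cartridge represents a gun cartridge made of a casing and one or more projectiles, and tracks its total mass.
; InitializeMass adds each projectile's mass to the casing's mass and stores the sum, but only when the projectile array is not empty.
; GetMass returns the stored value.
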(fn `GetMass`
  (returns (Mass :type "Float (double-precision)"))
  (return (`self.Mass`)))

(fn `InitializeMass`
  (locals (LocMass :type "Float (double-precision)"))
  (bind _projectile (`self.Projectile`))
  (set `local.LocMass` (`/Game/GameplayAbilities/Entities/Items/Weapons/Guns/Bullet/BP_Casing.GetMass` (`self.Casing`)))
  (if (`KismetArrayLibrary.Array_IsNotEmpty` _projectile)
    (for _array_element _projectile
      (set `local.LocMass` (+ (`local.LocMass`) (`/Game/GameplayAbilities/Entities/Items/Weapons/Guns/Bullet/BulletData.GetMass` _array_element))))
    (set `self.Mass` (`local.LocMass`))))