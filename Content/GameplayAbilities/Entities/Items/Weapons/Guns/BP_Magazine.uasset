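; BP_Magazine is a gun magazine that stores bullets as a last-in, first-out stack.
; Push adds a bullet after a capacity check against Size and Pop takes the last one, both firing a bullets-updated notification on change.
; GetMass adds projectile masses to the magazine's own mass, but its return sits inside the bullet loop, so only the first bullet counts.
; GetCurrentAmount reports the bullet count.
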(fn `GetCurrentAmount`
  (returns (Amount :type Integer))
  (return (`KismetArrayLibrary.Array_Length` (`self.Bullets`))))

(fn `GetMass`
  (returns (TotalMass :type "Float (double-precision)"))
  (locals (LocMass :type "Float (double-precision)"))
  (set `local.LocMass` (`self.Mass`))
  (for _array_element (`self.Bullets`)
    (for _array_element_2 (`/Game/GameplayAbilities/Entities/Items/Weapons/Guns/Bullet/BP_Cartridge.Projectile` _array_element)
      (set `local.LocMass` (+ (`local.LocMass`) (`/Game/GameplayAbilities/Entities/Items/Weapons/Guns/Bullet/BulletData.GetMass` _array_element_2))))
    (return (`local.LocMass`))))

(fn `Pop`
  (returns (`Popped Bullet` :type "/Game/GameplayAbilities/Entities/Items/Weapons/Guns/Bullet/BP_Cartridge Object Reference"))
  (locals (LocBullet :type "/Game/GameplayAbilities/Entities/Items/Weapons/Guns/Bullet/BP_Cartridge Object Reference"))
  (bind _returnvalue (`KismetArrayLibrary.Array_Length` (`self.Bullets`)))
  (bind _returnvalue_2 (- _returnvalue 1))
  (if (>= _returnvalue 1)
    (set `local.LocBullet` (`|GetArrayItem` (`self.Bullets`) _returnvalue_2))
    (`KismetArrayLibrary.Array_Remove` (`self.Bullets`) _returnvalue_2)
    (`self.OnBulletsUpdated`))
  (return (`local.LocBullet`)))

(fn `Push`
  (params (NewBullet :type "/Game/GameplayAbilities/Entities/Items/Weapons/Guns/Bullet/BP_Cartridge Object Reference"))
  (returns (Success :type Boolean))
  (if (>= (`self.Size`) (`KismetArrayLibrary.Array_Length` (`self.Bullets`)))
    (`KismetArrayLibrary.Array_Add` (`self.Bullets`) NewBullet)
    (`self.OnBulletsUpdated`)
    (return true)
    (else
      (return false))))

(fn `UserConstructionScript`)