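; Gun weapon actor that handles trigger-driven auto or burst fire, magazine reloading and projectile spawning, and builds attachment meshes on construction.
; Each shot pops a cartridge from the magazine, or starts a timed reload using a diameter-matched magazine from the owner's inventory.
; Primer force, barrel dimensions and bullet mass set muzzle velocity along the owner's view, and each projectile carries a GAS effect spec.
; Recoil and aim tracking are stubs, spread is zeroed, and debug output remains.
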(event `self.ReceiveBeginPlay`
  (if (`self.SpawnWithMag?`)
    _))

(event `self.ReceiveTick`
  (params (DeltaSeconds :type "Float (single-precision)"))
  (`self.AimWhereOwnerLooks`))

(event `PreFireBullet`)

(event `FireBullet`
  (`self.PreFireBullet`)
  (bind _outbullet (`self.CommitBullet`))
  (`/Engine/EditorBlueprintResources/StandardMacros.IsValid` _outbullet
    (:`Is Valid`
      (bind (_burndelay _forcecreated) (`/Game/GameplayAbilities/Entities/Items/Weapons/Guns/Bullet/BP_Casing.SetOffPrimer` (`/Game/GameplayAbilities/Entities/Items/Weapons/Guns/Bullet/BP_Cartridge.Casing` _outbullet)))
      (`GameplayStatics.PlaySoundAtLocation` (`self.TriggerPull_FireBullet_Sound`) (.location (`self.GetProjectileSpawnTransform`)) (struct) 1.0 1.0 0.0 null null null null)
      (if (`KismetArrayLibrary.Array_IsNotEmpty` (`/Game/GameplayAbilities/Entities/Items/Weapons/Guns/Bullet/BP_Cartridge.Projectile` _outbullet))
        (`KismetSystemLibrary.Delay` _burndelay)
        (for _array_element (`/Game/GameplayAbilities/Entities/Items/Weapons/Guns/Bullet/BP_Cartridge.Projectile` _outbullet)
          (`self.FireProjectile` _array_element _forcecreated)))
      (`self.PostFireBullet`))
    (:`Is Not Valid`
      (`GameplayStatics.PlaySoundAtLocation` (`self.TriggerPull_Empty_Sound`) (`self.K2_GetActorLocation`) (struct) 1.0 1.0 0.0 null null null null))))

(event `PostFireBullet`
  (`self.ApplyRecoil`))

(event `ApplyRecoil`)

(event `BurstFire`
  (`self.Burst` (`KismetMathLibrary.Conv_ByteToInt` (`self.BurstAmount`))
    (:`Burst`
      (`self.FireBullet`))))

(event `PullTrigger`
  (bind _returnvalue (> (`self.BurstAmount`) 1))
  (set `self.IsTriggerPulled` true)
  (if (`self.AutoFire?`)
    (bind _returnvalue_2 (`KismetSystemLibrary.K2_SetTimerDelegate` (select `bool` _returnvalue :`false` (`|CreateDelegate` :!event `FireBullet`) :`true` (`|CreateDelegate` :!event `BurstFire`)) (select `bool` _returnvalue :`false` (`self.FireRate`) :`true` (`self.BurstRate`)) true))
    (set `self.HoldingTrigger_Handle` _returnvalue_2)
    (else
      (`self.BurstFire`))))

(event `ReleaseTrigger`
  (`KismetSystemLibrary.K2_ClearAndInvalidateTimerHandle` (`self.HoldingTrigger_Handle`)))

(fn `AimWhereOwnerLooks`)

(fn `CalculateMuzzleVelocity`
  (params (BarrelDiameter :type "Float (double-precision)") (ForceApplied :type "Float (double-precision)") (BulletMass :type "Float (double-precision)") (BarrelLength :type "Float (double-precision)"))
  (returns (MuzzleVelocity :type "Float (double-precision)"))
  (return (* 2.0 (* (`local.BarrelLength`) (/ (* (`KismetMathLibrary.MultiplyByPi` (`KismetMathLibrary.Square` (* (* (`local.BarrelDiameter`) 0.1) 0.5))) (`local.ForceApplied`)) (`local.BulletMass`))))))

(fn `CanFireBullet`
  (returns (`Magazine is not empty` :type Boolean))
  (bind _magazine (`self.Magazine`))
  (`/Engine/EditorBlueprintResources/StandardMacros.IsValid` _magazine
    (:`Is Valid`
      (return (>= (`/Game/GameplayAbilities/Entities/Items/Weapons/Guns/BP_Magazine.GetCurrentAmount` _magazine) 1)))
    (:`Is Not Valid`
      (return false))))

(fn `CanReloadMagazine`
  (returns (`Owner has more magazines` :type Boolean))
  (locals (LocSucceded :type Boolean :default false))
  (bind _diameter (`self.Diameter`))
  (`KismetSystemLibrary.PrintString` "Check reload")
  (set `local.LocSucceded` false)
  (for _array_element (`InventoryComponent.Inventory` (`GACharacter.Inventory` (cast `GACharacter` (`self.GetOwner`) :!pure true)))
    (bind _asbp_magazine (cast `/Game/GameplayAbilities/Entities/Items/Weapons/Guns/BP_Magazine` _array_element))
    (bind _diameter_2 (`/Game/GameplayAbilities/Entities/Items/Weapons/Guns/BP_Magazine.Diameter` _asbp_magazine))
    (if (and (<= _diameter_2 (+ _diameter 0.1)) (>= _diameter_2 (- _diameter 0.1)))
      (set `local.LocSucceded` true)
      (`KismetSystemLibrary.PrintString` "Can reload")
      (break)))
  (return (`local.LocSucceded`)))

(fn `CommitBullet`
  (returns (OutBullet :type "/Game/GameplayAbilities/Entities/Items/Weapons/Guns/Bullet/BP_Cartridge Object Reference"))
  (bind _magazine_is_not_empty (`self.CanFireBullet`))
  (if _magazine_is_not_empty
    (bind _popped_bullet (`/Game/GameplayAbilities/Entities/Items/Weapons/Guns/BP_Magazine.Pop` (`self.Magazine`)))
    (return _popped_bullet)
    (else
      (`self.StartReload`)
      (return null))))

(fn `CommitReload`
  (bind _diameter (`self.Diameter`))
  (bind _inventory (`InventoryComponent.Inventory` (`GACharacter.Inventory` (cast `GACharacter` (`self.GetOwner`) :!pure true))))
  (for (_array_element _array_index) _inventory
    (bind _asbp_magazine (cast `/Game/GameplayAbilities/Entities/Items/Weapons/Guns/BP_Magazine` _array_element))
    (bind _diameter_2 (`/Game/GameplayAbilities/Entities/Items/Weapons/Guns/BP_Magazine.Diameter` _asbp_magazine))
    (if (and (<= _diameter_2 (+ _diameter 0.1)) (>= _diameter_2 (- _diameter 0.1)))
      (set `self.Magazine` _asbp_magazine)
      (`KismetArrayLibrary.Array_Remove` _inventory _array_index)
      (break)))
  (`self.OnReload`)
  (`KismetSystemLibrary.PrintString` (`KismetTextLibrary.Conv_TextToString` (`|FormatText` "Reloaded: \n Current Bullets {Amount} " (`KismetArrayLibrary.Array_Length` (`/Game/GameplayAbilities/Entities/Items/Weapons/Guns/BP_Magazine.Bullets` (`self.Magazine`)))))))

(fn `FireProjectile`
  (params (BulletData :type "/Game/GameplayAbilities/Entities/Items/Weapons/Guns/Bullet/BulletData Object Reference") (PropellantForce :type "Float (double-precision)"))
  (locals (LocVelocity :type "Float (double-precision)" :default 0.0))
  (bind _returnvalue (`self.K2_GetActorLocation`))
  (bind (_x _y) (`KismetMathLibrary.BreakVector2D` (`self.RandPointInCircle` (* (`KismetMathLibrary.DegTan` 5.0) 0.0))))
  (bind _returnvalue_2 (+ (* (`local.LocVelocity`) (`KismetMathLibrary.Conv_RotatorToVector` (`.OutRotation` (`self.GetActorEyesViewPoint` (`self.GetOwner`))))) (* (`self.GetActorRightVector`) _x) (* (`self.GetActorUpVector`) _y)))
  (bind _returnvalue_3 (+ _returnvalue _returnvalue_2))
  (bind _returnvalue_4 (`self.SpawnProjectile` BulletData))
  (bind _muzzlevelocity (`self.CalculateMuzzleVelocity` (`self.Diameter`) (`local.PropellantForce`) (`/Game/GameplayAbilities/Entities/Items/Weapons/Guns/Bullet/BulletData.GetMass` (`local.BulletData`)) (`self.BarrelLength`)))
  (set `local.LocVelocity` _muzzlevelocity)
  (`KismetSystemLibrary.DrawDebugLine` _returnvalue _returnvalue_3 (struct) 5.0)
  (`KismetSystemLibrary.DrawDebugSphere` _returnvalue_3 100.0 12 (struct :`R` 1.0 :`G` 1.0 :`B` 1.0 :`A` 1.0) 5.0)
  (set `MovementComponent.Velocity` _returnvalue_2 (`GAProjectile.ProjectileMovementComp` _returnvalue_4))
  (bind _returnvalue_5 (`AbilitySystemBlueprintLibrary.AssignTagSetByCallerMagnitude` (`AbilitySystemComponent.MakeOutgoingSpec` :`self` (`self.AbilitySystem`) :`GameplayEffectClass` "/Game/GameplayAbilities/Entities/Items/Weapons/Guns/Abilities/Primary/GE_SpawnBullet.GE_SpawnBullet_C" :`Level` 1.0) (struct :`TagName` "item.gun.InitialImpactPower") -1.0))
  (set `GAProjectile.EffectSpecHandleFromAbility` _returnvalue_5 _returnvalue_4)
  (`KismetSystemLibrary.PrintString` (`KismetTextLibrary.Conv_TextToString` (`|FormatText` "Velocity: ({VelX}, {VelY}, {VelZ}) \nOur Location: ({OurLocX}, {OurLocY}, {OurLocZ}) \nParent Location: ({X}, {Y}, {Z})" (.x _returnvalue_2) (.y _returnvalue_2) (.z _returnvalue_2) (.x (`self.K2_GetActorLocation`)) (.y (`self.K2_GetActorLocation`)) (.z (`self.K2_GetActorLocation`)) (.x (`self.K2_GetActorLocation` (`self.GetAttachParentActor`))) (.y (`self.K2_GetActorLocation` (`self.GetAttachParentActor`))) (.z (`self.K2_GetActorLocation` (`self.GetAttachParentActor`)))))))

(fn `Get Stability`
  (params (BulletLength :type "Float (double-precision)") (BulletDiameter :type "Float (double-precision)"))
  (returns (Varience :type "Float (double-precision)"))
  (return (`KismetMathLibrary.Lerp` 45.0 230.0)))

(fn `GetProjectileSpawnTransform`
  (returns (`Bullet Transform` :type "Transform Structure"))
  (bind (_outlocation _outrotation) (`self.GetActorEyesViewPoint` (`self.GetOwner`)))
  (return (`KismetMathLibrary.MakeTransform` _outlocation _outrotation)))

(fn `GetTwistRate`
  (returns (ReturnValue :type "Float (double-precision)"))
  (bind _riflingratio (`self.RiflingRatio`))
  (return (select `bool` (<= _riflingratio 0) :`false` (/ (`self.BarrelLength`) _riflingratio))))

(fn `RandPointInCircle`
  (params (Radius :type "Float (double-precision)"))
  (returns (Point :type "Vector2D Structure"))
  (locals (LocAngle :type "Float (double-precision)" :default 0.0) (LocDistance :type "Float (double-precision)" :default 0.0))
  (set `local.LocAngle` (`KismetMathLibrary.RandomFloatInRange` 0.0 360.0))
  (set `local.LocDistance` (`KismetMathLibrary.RandomFloatInRange` 0.0 (`local.Radius`)))
  (return (`KismetMathLibrary.MakeVector2D` (* (`local.LocDistance`) (`KismetMathLibrary.DegCos` (`local.LocAngle`))) (* (`local.LocDistance`) (`KismetMathLibrary.DegSin` (`local.LocAngle`))))))

(fn `SpawnProjectile`
  (params (BulletData :type "/Game/GameplayAbilities/Entities/Items/Weapons/Guns/Bullet/BulletData Object Reference"))
  (returns (ReturnValue :type "/Game/GameplayAbilities/Entities/Projectiles/Bullet Object Reference"))
  (bind _returnvalue (`|SpawnActorFromClass` "/Game/GameplayAbilities/Entities/Projectiles/Bullet.Bullet_C" (`KismetMathLibrary.MakeTransform` (`self.K2_GetActorLocation`) (`.OutRotation` (`self.GetActorEyesViewPoint` (`self.GetOwner`)))) "AlwaysSpawn" "OverrideRootScale" self (cast `Pawn` (`self.GetOwner`) :!pure true)))
  (bind _projectilemovementcomp (`GAProjectile.ProjectileMovementComp` _returnvalue))
  (set `GAProjectileMovementComponent.DragCoefficient` (`/Game/GameplayAbilities/Entities/Items/Weapons/Guns/Bullet/BulletData.DragCoefficient` (`local.BulletData`)) _projectilemovementcomp)
  (set `ProjectileMovementComponent.ProjectileGravityScale` (`/Game/GameplayAbilities/Entities/Items/Weapons/Guns/Bullet/BulletData.GetMass` (`local.BulletData`)) _projectilemovementcomp)
  (return _returnvalue))

(fn `StartReload`
  (bind _owner_has_more_magazines (`self.CanReloadMagazine`))
  (if _owner_has_more_magazines
    (if (`KismetSystemLibrary.K2_IsValidTimerHandle` (`self.ReloadTimerHandle`))
      (if (not (`KismetSystemLibrary.K2_IsTimerActiveHandle` (`self.ReloadTimerHandle`)))
        (bind _returnvalue (`KismetSystemLibrary.K2_SetTimer` null "CommitReload" (`self.ReloadDelay`) :!label _label))
        (set `self.ReloadTimerHandle` _returnvalue))
      (else
        (goto _label)))))

(fn `UserConstructionScript`
  (`parent.UserConstructionScript`)
  (for _array_element (`ShooterComponent.Attatchments` (`self.Shooter`))
    (`/Engine/EditorBlueprintResources/StandardMacros.IsValid` _array_element
      (:`Is Valid`
        (bind _mesh (`ShooterAttatchment.Mesh` _array_element))
        (`/Engine/EditorBlueprintResources/StandardMacros.IsValid` _mesh
          (:`Is Valid`
            (bind _returnvalue (`AddComponent|NODE_AddStaticMeshComponent-0` :`RelativeTransform` (`KismetMathLibrary.MakeTransform` (0.0 0.0 0.0) (struct :`Yaw` -90.0))))
            (`StaticMeshComponent.SetStaticMesh` _returnvalue _mesh)
            (bind _material (`ShooterAttatchment.Material` _array_element))
            (`/Engine/EditorBlueprintResources/StandardMacros.IsValid` _material
              (:`Is Valid`
                (`PrimitiveComponent.SetMaterial` _returnvalue 0 _material)))))))))