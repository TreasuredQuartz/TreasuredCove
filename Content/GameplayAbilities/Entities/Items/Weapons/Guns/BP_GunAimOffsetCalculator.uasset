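; BP_GunAimOffsetCalculator is a helper actor that calculates the aim-down-sights offset for a gun.
; Its construction script transforms the Weapon's Scope socket location into ADSLocation's local space, negates it and swaps X and Y.
; The result is stored in OffsetOutput, and the event graph holds no active logic.
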(fn `UserConstructionScript`
  (bind _returnvalue_location (`KismetMathLibrary.BreakTransform` (`SceneComponent.GetSocketTransform` (`self.Weapon`) "Scope" "RTS_World")))
  (bind (_returnvalue_x _returnvalue_y _returnvalue_z) (`KismetMathLibrary.BreakVector` (* (`KismetMathLibrary.InverseTransformLocation` (`SceneComponent.K2_GetComponentToWorld` (`self.ADS_Location`)) _returnvalue_location) (-1.0 -1.0 -1.0))))
  (set `self.OffsetOutput` (`KismetMathLibrary.MakeVector` _returnvalue_y _returnvalue_x _returnvalue_z)))