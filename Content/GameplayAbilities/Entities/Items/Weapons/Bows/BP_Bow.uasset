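; Bow weapon Blueprint that handles drawing, cancelling and firing a shot.
; With a valid Arrow, a timeline plays forward to write ChargeAmount on each update and reverses when the charge is cancelled.
; Stopping the charge halts the timeline and resets its time, while firing activates the GA_SpawnProjectile gameplay ability through the Ability System.
; The Reload event is empty.
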(event `BeginCharge`
  (`/Engine/EditorBlueprintResources/StandardMacros.IsValid` (`self.Arrow`)
    (:`Is Valid`
      (bind (_direction _chargeamounttrack) (`Timeline|ChargeTimeline` :!label _label)
        (:`Update`
          (set `self.ChargeAmount` _chargeamounttrack))))))

(event `StopCharge`
  (`|ExecutionSequence`
    (:`then_0`
      (goto _label :!via `Stop`))
    (:`then_1`
      (goto _label :!via `SetNewTime`))))

(event `CancelCharge`
  (`/Engine/EditorBlueprintResources/StandardMacros.IsValid` (`self.Arrow`)
    (:`Is Valid`
      (goto _label :!via `Reverse`))))

(event `Fire`
  (`AbilitySystemComponent.TryActivateAbilityByClass` (`self.AbilitySystem`) "/Script/TreasuredCove.GA_SpawnProjectile" true))

(event `Reload`)

(fn `UserConstructionScript`
  (`parent.UserConstructionScript`))