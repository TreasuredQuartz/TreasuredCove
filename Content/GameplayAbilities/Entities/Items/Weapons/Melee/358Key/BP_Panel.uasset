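; BP_Panel is a grid-placeable panel item, apparently modeled on the Kingdom Hearts 358/2 Days panel system.
; SetDataFromItemKey looks up the item name in DT_KHDays_Panels to fill display data, category, max, icon and shape.
; GetLinkZone turns the row's Value, as a one-based index, into link-zone tiles from ShapesDatabase.
; CanCohabitat lets panels of the same category share space, except at the panel's own location.
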(event `SetDataFromItemKey`
  (params (ItemKey :type "ItemKey Structure"))
  (set `self.ItemName` ItemKey_Name)
  (set `self.QuantityAvailable` ItemKey_Quantity)
  (bind _returnvalue (`|GetDataTableRow` "/Game/GameplayAbilities/Entities/Items/Weapons/Melee/358Key/DT_KHDays_Panels.DT_KHDays_Panels" (`self.ItemName`))
    (:`then`
      (bind (_name _category _description _max _value _texture) (break `ItemUIInfoRow` _returnvalue))
      (set `self.DisplayName` (`KismetTextLibrary.Conv_StringToText` _name))
      (set `self.Description` (`KismetTextLibrary.Conv_StringToText` _description))
      (set `self.Category` _category)
      (set `self.Max` _max)
      (set `self.Texture` _texture)
      (bind _linkzone (`self.GetLinkZone` _value))
      (set `self.Link Zone` _linkzone)
      (set `self.Name` (`self.ItemName`))
      (set `self.Shape` (`self.Link Zone`))
      (set `self.Icon` (`self.Texture`)))))

(fn `CanCohabitat`
  (params (Other :type "SpatialInventoryTileItem Object Reference") (InLocation :type "IntPoint Structure (by ref)"))
  (returns (ReturnValue :type Boolean))
  (if (!= InLocation (`self.Location`))
    (bind _asbp_panel (cast `/Game/GameplayAbilities/Entities/Items/Weapons/Melee/358Key/BP_Panel` Other))
    (return (`KismetStringLibrary.EqualEqual_StrStr` (`/Game/GameplayAbilities/Entities/Items/Weapons/Melee/358Key/BP_Panel.Category` _asbp_panel) (`self.Category`)))))

(fn `GetLinkZone`
  (params (LinkZoneType :type Integer))
  (returns (LinkZone :type "Array of IntPoint Structure"))
  (locals (LocLinkZone :type "Array of IntPoint Structure"))
  (bind _returnvalue (- LinkZoneType 1))
  (bind _shapesdatabase (`self.ShapesDatabase`))
  (bind _shapes (`SpatialInventoryShapeDatabase.Shapes` _shapesdatabase))
  (bind (_output_shapename _output_tiles) (break `SpatialInventoryShape` (`|GetArrayItem` _shapes _returnvalue)))
  (if (> LinkZoneType 0)
    (`/Engine/EditorBlueprintResources/StandardMacros.IsValid` _shapesdatabase
      (:`Is Valid`
        (if (`KismetArrayLibrary.Array_IsValidIndex` _shapes _returnvalue)
          (set `local.LocLinkZone` _output_tiles)))
      (:`Is Not Valid`
        _)))
  (return (`local.LocLinkZone`)))