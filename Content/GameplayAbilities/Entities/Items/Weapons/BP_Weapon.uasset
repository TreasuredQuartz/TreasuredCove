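; BP_Weapon is a weapon item Blueprint that shows a pickup effect colored by the weapon's rarity.
; The construction script looks up the rarity color in the RarityComponent's database and passes it to the FXPickup effect along with a fixed color intensity.
; When the weapon is picked up, it runs the parent's pickup logic and then deactivates the effect.
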(event `self.OnPickedUp`
  (`parent.OnPickedUp`)
  (`ActorComponent.Deactivate` (`self.FX_Pickup`)))

(fn `UserConstructionScript`
  (bind _fx_pickup (`self.FX_Pickup`))
  (bind _raritycomponent (`self.RarityComponent`))
  (bind _returnvalue (`RarityDatabase.GetRarityColor` (`RarityComponent.Database` _raritycomponent) (`RarityComponent.Rarity` _raritycomponent)))
  (`NiagaraComponent.SetVariableLinearColor` _fx_pickup "Color" _returnvalue)
  (`NiagaraComponent.SetVariableFloat` _fx_pickup "ColorIntensity" 10.0))