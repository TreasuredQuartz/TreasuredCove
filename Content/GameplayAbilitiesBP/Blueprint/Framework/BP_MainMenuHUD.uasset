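; Main menu HUD that spawns menu widgets and relays menu input to them.
; On BeginPlay it shows the ghost perk selection menu with UI-only input and a mouse cursor, without storing it as CurrentMenu.
; OpenMenu creates a given widget class and stores it as CurrentMenu, which receives navigation, confirm, return and cursor events.
; Both cursor events pass their single value as X and Y alike.
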(event `self.ReceiveBeginPlay`
  (bind _returnvalue (`self.GetOwningPlayerController`))
  (bind _returnvalue_2 (`|CreateWidget` "/Game/GameplayAbilitiesBP/Blueprint/UI/InfiniteWarfare/Perks/WBP_GhostPerkSelectionMenu.WBP_GhostPerkSelectionMenu_C"))
  (`UserWidget.AddToViewport` _returnvalue_2 0)
  (`WidgetBlueprintLibrary.SetInputMode_UIOnlyEx` _returnvalue _returnvalue_2)
  (set `PlayerController.bShowMouseCursor` true _returnvalue))

(event `self.SendNavigationRequest`
  (params (Val :type "ENavType Enum" :default "Up"))
  (`GAWidget.RecieveNavRequest` (`self.CurrentMenu`) Val))

(event `self.ConfirmPressed`
  (`GAWidget.ConfirmPressed` (`self.CurrentMenu`)))

(event `self.ReturnPressed`
  (`GAWidget.ReturnPressed` (`self.CurrentMenu`)))

(event `self.CursorMoveUp`
  (params (Val :type "Float (single-precision)"))
  (`GAWidget.OnCursorMove` (`self.CurrentMenu`) (`KismetMathLibrary.MakeVector2D` Val (stale `self.CursorMoveRight` Val)) :!label _label))

(event `self.CursorMoveRight`
  (params (Val :type "Float (single-precision)"))
  (goto _label))

(event `self.ConfirmReleased`
  (`GAWidget.ConfirmReleased` (`self.CurrentMenu`)))

(event `self.ReturnReleased`
  (`GAWidget.ReturnReleased` (`self.CurrentMenu`)))

(event `self.OpenMenu`
  (params (Menu :type "GAWidget Class Reference"))
  (bind _returnvalue (`|CreateWidget` Menu (`self.GetOwningPlayerController`)))
  (bind _output_get (set `self.CurrentMenu` _returnvalue))
  (`UserWidget.AddToViewport` _output_get 0))

(fn `UserConstructionScript`)