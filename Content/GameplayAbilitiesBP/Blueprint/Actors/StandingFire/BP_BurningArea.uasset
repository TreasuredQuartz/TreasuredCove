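; BP_BurningArea is a fire hazard area that applies the GE_Burning Gameplay Effect to overlapping actors that have an Ability System Component.
; On capsule begin overlap it prints a debug string, applies the effect and stores the returned handle in the ActiveBurningEffects map, keyed by component.
; On end overlap it looks up that handle and removes all stacks of the effect, leaving the map entry in place.
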(event `self.Capsule.OnComponentBeginOverlap`
  (params (OverlappedComponent :type "PrimitiveComponent Object Reference") (OtherActor :type "Actor Object Reference") (OtherComp :type "PrimitiveComponent Object Reference") (OtherBodyIndex :type Integer) (bFromSweep :type Boolean) (SweepResult :type "HitResult Structure (by ref)"))
  (bind _returnvalue (`AbilitySystemBlueprintLibrary.GetAbilitySystemComponent` OtherActor))
  (`/Engine/EditorBlueprintResources/StandardMacros.IsValid` _returnvalue
    (:`Is Valid`
      (`KismetSystemLibrary.PrintString` "Overlapped Ability System")
      (bind _returnvalue_2 (`AbilitySystemComponent.BP_ApplyGameplayEffectToSelf` :`self` _returnvalue :`GameplayEffectClass` "/Game/GameplayAbilitiesBP/Blueprint/Actors/StandingFire/GE_Burning.GE_Burning_C"))
      (`BlueprintMapLibrary.Map_Add` (`self.ActiveBurningEffects`) _returnvalue _returnvalue_2))))

(event `self.Capsule.OnComponentEndOverlap`
  (params (OverlappedComponent :type "PrimitiveComponent Object Reference") (OtherActor :type "Actor Object Reference") (OtherComp :type "PrimitiveComponent Object Reference") (OtherBodyIndex :type Integer))
  (bind _returnvalue (`AbilitySystemBlueprintLibrary.GetAbilitySystemComponent` OtherActor))
  (bind (_value _returnvalue_2) (`BlueprintMapLibrary.Map_Find` (`self.ActiveBurningEffects`) _returnvalue))
  (`/Engine/EditorBlueprintResources/StandardMacros.IsValid` _returnvalue
    (:`Is Valid`
      (if _returnvalue_2
        (`AbilitySystemComponent.RemoveActiveGameplayEffect` _returnvalue _value -1)))))

(fn `UserConstructionScript`)