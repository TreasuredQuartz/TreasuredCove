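; BP_GreatFox is the Great Fox vehicle Blueprint, which lets the player select and trigger warp points.
; On BeginPlay it gathers all WarpPoint actors, repeating the search after a delay until at least one exists.
; The mouse wheel steps the active index within a hard-coded range of three slots.
; Left click calls InteractedWith on the selected warp point, passing the Great Fox itself.
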(event `self.ReceiveBeginPlay`
  (bind _outactors (`GameplayStatics.GetAllActorsOfClass` "/Game/GameplayAbilitiesBP/Blueprint/Environment/Doors/WarpPoint.WarpPoint_C" :!label _label))
  (set `self.WarpPointCollection` _outactors)
  (`KismetSystemLibrary.Delay` 2.0)
  (if (not (`KismetArrayLibrary.Array_IsValidIndex` (`self.WarpPointCollection`)))
    (goto _label)))

(event `Key|LeftMouseButton`
  (params (Key :type "Key Structure"))
  (:`Pressed`
    (`/Game/GameplayAbilitiesBP/Blueprint/Environment/Doors/WarpPoint.InteractedWith` (`|GetArrayItem` (`self.WarpPointCollection`) (`self.ActiveWarpPoint`)) self)))

(event `Key|MouseScrollUp`
  (params (Key :type "Key Structure"))
  (:`Pressed`
    (set `self.ActiveWarpPoint` (`KismetMathLibrary.Clamp` (+ (`self.ActiveWarpPoint`) 1) 0 2))))

(event `Key|MouseScrollDown`
  (params (Key :type "Key Structure"))
  (:`Pressed`
    (set `self.ActiveWarpPoint` (`KismetMathLibrary.Clamp` (+ (`self.ActiveWarpPoint`) -1) 0 2))))

(fn `UserConstructionScript`)