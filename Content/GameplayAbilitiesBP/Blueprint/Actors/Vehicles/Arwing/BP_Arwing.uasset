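; Arwing vehicle pawn that flies in two modes, shooter or top-down, and offers itself as an interactable to actors overlapping its enter trigger.
; Each tick, consumed movement input becomes velocity that offsets the mesh within clamped bounds: Y/Z with banking in shooter mode, X/Y over a wider area in top-down.
; Mode switches change speed and play or reverse a timeline blending spring arm and mesh transforms, with input disabled until it finishes.
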(event `self.ReceiveBeginPlay`
  ;[0 0.1015 1] Begin Play
  (`TimelineComponent.SetPlayRate` (`self.TopDownTimeline`) (`self.TopDownTransitionSpeed`)))

(event `self.EnterTrigger.OnComponentBeginOverlap`
  (params (OverlappedComponent :type "PrimitiveComponent Object Reference") (OtherActor :type "Actor Object Reference") (OtherComp :type "PrimitiveComponent Object Reference") (OtherBodyIndex :type Integer) (bFromSweep :type Boolean) (SweepResult :type "HitResult Structure (by ref)"))
  ;[0.7552 0.39 0.09379] Interaction  interface
  (message `InteractionInterface.NotifyCanInteract` OtherActor "None" true self))

(event `self.EnterTrigger.OnComponentEndOverlap`
  (params (OverlappedComponent :type "PrimitiveComponent Object Reference") (OtherActor :type "Actor Object Reference") (OtherComp :type "PrimitiveComponent Object Reference") (OtherBodyIndex :type Integer))
  ;[0.7552 0.39 0.09379] Interaction  interface
  (message `InteractionInterface.NotifyCanInteract` OtherActor "None" false self))

(event `self.ReceiveTick`
  (params (DeltaSeconds :type "Float (single-precision)"))
  ;[0 0.1015 1] Tick
  (if (`self.TopDown?`)
    (`self.TopDownMovement` DeltaSeconds)
    (else
      (`self.ShooterMovement` DeltaSeconds))))

(event `self.MoveForward`
  (params (AxisValue :type "Float (single-precision)"))
  ;[1 0.2344 0.2344] Inputs
  (`self.AddMovementInput` (`KismetMathLibrary.SelectVector` (1.0 0.0 0.0) (0.0 0.0 1.0) (`self.TopDown?`)) AxisValue))

(event `PerformMove`
  ;[1 0.2344 0.2344] Inputs
  (bind _returnvalue (`self.ConsumeMovementInputVector`))
  (set `self.Velocity` (* _returnvalue (`self.Speed`))))

(event `TransitionTopDown`
  (bind _staticmesh (`self.StaticMesh`))
  (bind _staticmesh_2 (`self.StaticMesh`))
  ;[0.5729 0 0] Top Down
  (set `self.Speed` 10000)
  (set `self.TopDown?` true)
  (bind _asplayer_controller (cast `PlayerController` (`self.GetController`)))
  (`self.DisableInput` _asplayer_controller)
  (bind (_direction _topdownfloatcurve) (`Timeline|TopDownTimeline` :!via `PlayFromStart` :!label _label)
    (:`Update`
      (`SceneComponent.K2_SetRelativeRotation` (`self.SpringArm`) (`KismetMathLibrary.RLerp` (struct) (struct :`Pitch` -90.0) _topdownfloatcurve) false false)
      (set `SpringArmComponent.TargetArmLength` (`KismetMathLibrary.Lerp` 1280.0 10000.0 _topdownfloatcurve) (`self.SpringArm`))
      (`SceneComponent.K2_SetRelativeLocation` _staticmesh_2 (`KismetMathLibrary.VInterpTo` (`SceneComponent.RelativeLocation` _staticmesh_2) (0.0 0.0 0.0) _topdownfloatcurve 1.0) false false)
      (`SceneComponent.K2_SetRelativeRotation` _staticmesh (`KismetMathLibrary.RInterpTo` (`SceneComponent.RelativeRotation` _staticmesh) (struct :`Yaw` -90.0) _topdownfloatcurve 1.0) false false))
    (:`Finished`
      (set `self.CurrentLocOffset` (0.0 0.0))
      (bind _asplayer_controller_2 (cast `PlayerController` (`self.GetController`)))
      (`self.EnableInput` _asplayer_controller_2))))

(event `self.MoveRight`
  (params (AxisValue :type "Float (single-precision)"))
  ;[1 0.2344 0.2344] Inputs
  (`self.AddMovementInput` (0.0 1.0 0.0) AxisValue))

(event `TransitionShooter`
  ;[0.5729 0 0] Top Down
  (set `self.Speed` 1000)
  (set `self.TopDown?` false)
  (bind _asplayer_controller (cast `PlayerController` (`self.GetController`)))
  (`self.DisableInput` _asplayer_controller)
  (goto _label :!via `Reverse`))

(event `ReplicateRotation`
  (params (DeltaSeconds :type "Float (double-precision)"))
  (bind (_returnvalue_x _returnvalue_y _returnvalue_z) (`KismetMathLibrary.BreakVector` (`KismetMathLibrary.Normal` (`self.Velocity`))))
  (bind (_returnvalue_roll _returnvalue_pitch) (`KismetMathLibrary.BreakRotator` (`KismetMathLibrary.RInterpTo` (`SceneComponent.RelativeRotation` (`self.StaticMesh`)) (`KismetMathLibrary.MakeRotFromYZ` (`self.AimTarget`) (`SceneComponent.GetUpVector` (`self.Camera`))) DeltaSeconds 10.0)))
  ;[0.4413 0 0.474] Shooter
  (set `self.AimTarget` (`KismetMathLibrary.MakeVector` 1.0 _returnvalue_y _returnvalue_z))
  (`SceneComponent.K2_SetRelativeRotation` (`self.StaticMesh`) (`KismetMathLibrary.MakeRotator` _returnvalue_roll _returnvalue_pitch -90.0) false false))

(event `TopDownMovement`
  (params (DeltaSeconds :type "Float (double-precision)"))
  (bind (_x _y) (`KismetMathLibrary.BreakVector2D` (`self.TopDownClampedLocation` DeltaSeconds)))
  ;[0.5729 0 0] Top Down
  (if (not (`KismetMathLibrary.NearlyEqual_FloatFloat` DeltaSeconds 0.0 0.01))
    (`self.PerformMove`)
    (if (not (`KismetMathLibrary.Vector_IsNearlyZero` (`self.Velocity`)))
      (`SceneComponent.K2_SetRelativeLocation` (`self.StaticMesh`) (`KismetMathLibrary.MakeVector` _x _y) false false))))

(event `HorizontalLean`
  (params (DeltaSeconds :type "Float (double-precision)"))
  (bind (_relativerotation_roll _relativerotation_pitch _relativerotation_yaw) (`KismetMathLibrary.BreakRotator` (`SceneComponent.RelativeRotation` (`self.StaticMesh`))))
  ;[0.4413 0 0.474] Shooter
  (`SceneComponent.K2_SetRelativeRotation` (`self.StaticMesh`) (`KismetMathLibrary.MakeRotator` _relativerotation_roll _relativerotation_pitch (`KismetMathLibrary.FInterpTo` _relativerotation_yaw (.y (`self.Velocity`)) DeltaSeconds 0.5)) false false))

(event `ShooterMovement`
  (params (DeltaSeconds :type "Float (double-precision)"))
  (bind (_clampedoffset_x _clampedoffset_y) (`KismetMathLibrary.BreakVector2D` (`self.ShooterClampedLocation` DeltaSeconds)))
  ;[0.4413 0 0.474] Shooter
  (if (not (`KismetMathLibrary.NearlyEqual_FloatFloat` DeltaSeconds 0.0 0.01))
    (`self.PerformMove`)
    (`self.ReplicateRotation` DeltaSeconds)
    (`self.HorizontalLean` DeltaSeconds)
    (if (not (`KismetMathLibrary.Vector_IsNearlyZero` (`self.Velocity`)))
      (`SceneComponent.K2_SetRelativeLocation` (`self.StaticMesh`) (`KismetMathLibrary.MakeVector` 0.0 _clampedoffset_x _clampedoffset_y) false false))))

(fn `ShooterClampedLocation`
  (params (DeltaSeconds :type "Float (single-precision)"))
  (returns (ClampedOffset :type "Vector2D Structure"))
  (locals (LocNewLocation :type "Vector Structure"))
  (bind _hlimit (`self.HLimit`))
  (bind _vlimit (`self.VLimit`))
  (bind (_returnvalue_x _returnvalue_y _returnvalue_z) (`KismetMathLibrary.BreakVector` (* (`self.Velocity`) DeltaSeconds)))
  (bind (_x _y) (`KismetMathLibrary.BreakVector2D` (+ (`self.CurrentLocOffset`) (`KismetMathLibrary.MakeVector2D` _returnvalue_y _returnvalue_z))))
  (bind _output_get (set `self.CurrentLocOffset` (`KismetMathLibrary.MakeVector2D` (`KismetMathLibrary.FClamp` _x (- 0.0 _hlimit) _hlimit) (`KismetMathLibrary.FClamp` _y (- 0.0 _vlimit) _vlimit))))
  (return _output_get))

(fn `TopDownClampedLocation`
  (params (DeltaSeconds :type "Float (single-precision)"))
  (returns (`Offset'` :type "Vector2D Structure"))
  (bind (_returnvalue_x _returnvalue_y) (`KismetMathLibrary.BreakVector` (* (`self.Velocity`) DeltaSeconds)))
  (bind _returnvalue (* (`self.VLimit`) 10.0))
  (bind _returnvalue_2 (* (`self.HLimit`) 10.0))
  (bind (_x _y) (`KismetMathLibrary.BreakVector2D` (+ (`self.CurrentLocOffset`) (`KismetMathLibrary.MakeVector2D` _returnvalue_x _returnvalue_y))))
  (bind _output_get (set `self.CurrentLocOffset` (`KismetMathLibrary.MakeVector2D` (`KismetMathLibrary.FClamp` _x (- 0.0 _returnvalue_2) _returnvalue_2) (`KismetMathLibrary.FClamp` _y (- 0.0 _returnvalue) _returnvalue))))
  (return _output_get))

(fn `UserConstructionScript`)