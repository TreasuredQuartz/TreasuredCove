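; Player character Blueprint that switches between first and third person, run from the construction script and on camera type changes.
; Switching swaps arms and full mannequin meshes, rotates the mesh and sets camera arm length; death detaches the third-person camera.
; BeginPlay limits a scene capture to its SCPlane component, while Tick adds a static mesh component at the capsule location whenever moving.
; Dynamic material and GrassAffector capture registration logic is left unconnected.
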(event `self.ReceiveBeginPlay`
  (`parent.ReceiveBeginPlay`)
  (`|ExecutionSequence`
    (:`then_1`
      (`SceneCaptureComponent.ShowOnlyComponent` (`self.SceneCapture`) (`self.SC_Plane`)))))

(event `self.OnDeath`
  (if (not (`self.bFirstPerson`))
    (`SceneComponent.K2_DetachFromComponent` (`self.Camera_01`) "KeepWorld" "KeepWorld" "KeepWorld" true)))

(event `self.ReceiveTick`
  (params (DeltaSeconds :type "Float (single-precision)"))
  (if (> (`KismetMathLibrary.VSize` (`self.GetVelocity`)) 50.0)
    (`AddComponent|NODE_AddStaticMeshComponent-1` :`bManualAttachment` true :`RelativeTransform` (`KismetMathLibrary.Conv_VectorToTransform` (`SceneComponent.K2_GetComponentLocation` (`self.CapsuleComponent`))))))

(event `self.ChangeCameraType`
  (params (bInFirstPerson :type Boolean))
  (bind _bfirstperson (`self.bFirstPerson`))
  (bind _mesh (`self.Mesh`))
  (`parent.ChangeCameraType` bInFirstPerson)
  (`|ExecutionSequence`
    (:`then_0`
      (`SkinnedMeshComponent.SetSkinnedAssetAndUpdate` _mesh (select `bool` _bfirstperson :`false` "/Game/AnimStarterPack/UE4_Mannequin/Mesh/SK_Mannequin.SK_Mannequin" :`true` "/Game/AnimStarterPack/FirstPersonArms/Character/Mesh/SK_Mannequin_Arms.SK_Mannequin_Arms" :!type "SkeletalMesh Object Reference") true)
      (`SceneComponent.K2_SetRelativeRotation` _mesh (`KismetMathLibrary.SelectRotator` (struct) (struct :`Yaw` -90.0) _bfirstperson) false false))
    (:`then_1`
      (set `SpringArmComponent.TargetArmLength` (select `bool` _bfirstperson :`false` 300.0) (`self.CameraArm`)))))

(fn `UserConstructionScript`
  (`self.ChangeCameraType` (`self.bFirstPerson`)))