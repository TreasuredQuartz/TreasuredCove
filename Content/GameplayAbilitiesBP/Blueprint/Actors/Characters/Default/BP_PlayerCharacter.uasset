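; Player character Blueprint with switchable first- and third-person cameras and a death camera.
; On camera change, non-simulated roles in first person get the arms mesh, others the full mannequin, and the boom length follows the mode.
; On death the boom stops colliding, detaches in third person, then lengthens each tick while adding pitch input.
; BeginPlay limits the scene capture to SCPlane; GrassAffector capture and dynamic material nodes are unconnected.
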(event `self.ReceiveBeginPlay`
  (`parent.ReceiveBeginPlay`)
  (`|ExecutionSequence`
    (:`then_1`
      (`SceneCaptureComponent.ShowOnlyComponent` (`self.SceneCapture`) (`self.SC_Plane`)))))

(event `self.OnDeath`
  (bind _cameraarm (`self.CameraArm`))
  (if (not (`self.bFirstPerson`))
    (`SceneComponent.K2_DetachFromComponent` _cameraarm "KeepWorld" "KeepWorld" "KeepWorld" true))
  (set `SpringArmComponent.bDoCollisionTest` false _cameraarm))

(event `self.ReceiveTick`
  (params (DeltaSeconds :type "Float (single-precision)"))
  (bind _cameraarm (`self.CameraArm`))
  (if (`self.bIsDead`)
    (set `SpringArmComponent.TargetArmLength` (+ (`SpringArmComponent.TargetArmLength` _cameraarm) (* DeltaSeconds 100.0)) _cameraarm)
    (if (< (.pitch (`SceneComponent.K2_GetComponentRotation` _cameraarm)) 85.0)
      (`self.AddControllerPitchInput` (* DeltaSeconds 10.0)))))

(event `self.OnChangeCameraType`
  (params (bInFirstPerson :type Boolean))
  (bind _bfirstperson (`self.bFirstPerson`))
  (bind _mesh (`self.Mesh`))
  (bind _returnvalue (and _bfirstperson (> (`self.GetLocalRole`) 1)))
  (`|ExecutionSequence`
    (:`then_0`
      (`SkinnedMeshComponent.SetSkinnedAssetAndUpdate` _mesh (select `bool` _returnvalue :`false` "/Game/AnimStarterPack/UE4_Mannequin/Mesh/SK_Mannequin.SK_Mannequin" :`true` "/Game/AnimStarterPack/FirstPersonArms/Character/Mesh/SK_Mannequin_Arms.SK_Mannequin_Arms" :!type "SkeletalMesh Object Reference") true)
      (`SceneComponent.K2_SetRelativeRotation` _mesh (`KismetMathLibrary.SelectRotator` (struct) (struct :`Yaw` -90.0) _returnvalue) false false))
    (:`then_1`
      (set `SpringArmComponent.TargetArmLength` (select `bool` _bfirstperson :`false` 300.0) (`self.CameraArm`)))))

(fn `UserConstructionScript`)