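; BP_Footprint is a short-lived footprint actor with a mesh and a sphere that can react to being heard.
; Each tick it scales the sphere uniformly by the actor's elapsed lifespan plus a small offset, so the sphere grows steadily like an expanding ripple.
; OnHeardBP turns on custom depth rendering for both the sphere and footprint mesh, with no logic here to turn it off.
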(event `self.ReceiveBeginPlay`)

(event `self.ReceiveTick`
  (params (DeltaSeconds :type "Float (single-precision)"))
  (`SceneComponent.SetWorldScale3D` (`self.Sphere`) (`KismetMathLibrary.Conv_DoubleToVector` (- (`self.InitialLifeSpan`) (`self.GetLifeSpan`) -0.1))))

(event `self.OnHeard_BP`
  (`PrimitiveComponent.SetRenderCustomDepth` (`self.Sphere`) true)
  (`PrimitiveComponent.SetRenderCustomDepth` (`self.FootprintMesh`) true))

(fn `UserConstructionScript`)