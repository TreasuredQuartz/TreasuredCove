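; BP_Character is a character Blueprint that sets up footprint and equipment placement from placeholder components at BeginPlay.
; The relative locations of the right and left footprint placeholders are added to the FootprintComponent's location list.
; The held and stowed item placeholders supply relative location and rotation, with unit scale, to initialize the Equipment component's slot transforms.
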(event `self.ReceiveBeginPlay`
  (bind (_returnvalue_location _returnvalue_rotation) (`KismetMathLibrary.BreakTransform` (`SceneComponent.GetRelativeTransform` (`self.StowedItem_placeholder`))))
  (bind (_returnvalue_location_2 _returnvalue_rotation_2) (`KismetMathLibrary.BreakTransform` (`SceneComponent.GetRelativeTransform` (`self.HeldItem_placeholder`))))
  (bind _footprintlocations (`FootprintComponent.FootprintLocations` (`self.FootprintComponent`)))
  (`KismetArrayLibrary.Array_Add` _footprintlocations (`SceneComponent.RelativeLocation` (`self.Footprint_r_placeholder`)))
  (`KismetArrayLibrary.Array_Add` _footprintlocations (`SceneComponent.RelativeLocation` (`self.Footprint_l_placeholder`)))
  (`EquipmentComponent.InitializeEquipmentSlotTransforms` (`self.Equipment`) (`|MakeArray` (`KismetMathLibrary.MakeTransform` _returnvalue_location_2 _returnvalue_rotation_2) (`KismetMathLibrary.MakeTransform` _returnvalue_location _returnvalue_rotation) :!type "Transform Structure")))

(fn `UserConstructionScript`)