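; BP_PauseStudio is a pawn for a pause mode that takes over the player's controller and hands it back on exit.
; OnEnter possesses it through the owner's instigator controller and, if none exists, spawns a hex grid manager far below and attaches it.
; The mouse wheel zooms the spring-arm camera within limits, and the Pause action repossesses the owning pawn.
; Move and look inputs are unimplemented stubs.
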(event `self.OnEnter`
  (`Controller.Possess` (`self.GetInstigatorController` (`self.GetOwner`)) self)
  (`/Engine/EditorBlueprintResources/StandardMacros.IsValid` (`self.HexGridManager`)
    (:`Is Not Valid`
      (bind _returnvalue (`|SpawnActorFromClass` "/Game/GameplayAbilitiesBP/Blueprint/Abilities/HexTiles/BP_HexGridManager.BP_HexGridManager_C" (`KismetMathLibrary.MakeTransform` (+ (`self.K2_GetActorLocation`) (0.0 0.0 -10000.0))) "Undefined" "OverrideRootScale" null null))
      (bind _output_get (set `self.HexGridManager` _returnvalue))
      (`self.K2_AttachToActor` _output_get self "None" "KeepRelative" "KeepRelative" "KeepRelative" true))))

(event `self.OnExit`
  (`Controller.Possess` (`self.GetController`) (cast `Pawn` (`self.GetOwner`) :!pure true)))

(event `InputAxis|Move Forward / Backward`
  (params (AxisValue :type "Float (single-precision)"))
  (if (!= AxisValue 0.0)
    _))

(event `InputAction|Pause`
  (params (Key :type "Key Structure"))
  (:`Pressed`
    (`self.OnExit`)))

(event `InputAxisKey|MouseWheelAxis`
  (params (AxisValue :type "Float (single-precision)"))
  (if (!= AxisValue 0.0)
    (set `SpringArmComponent.TargetArmLength` (`KismetMathLibrary.FClamp` (+ (* AxisValue (`self.CameraZoomSpeed`) -1.0) (`SpringArmComponent.TargetArmLength` (`self.SpringArm`))) (`self.MinCameraDistance`) (`self.MaxCameraDistance`)) (`self.SpringArm`))))

(event `InputAxis|LookRight`
  (params (AxisValue :type "Float (single-precision)"))
  (if (!= AxisValue 0.0)
    _))

(event `InputAxis|LookUp`
  (params (AxisValue :type "Float (single-precision)"))
  (if (!= AxisValue 0.0)
    _))

(fn `UserConstructionScript`)