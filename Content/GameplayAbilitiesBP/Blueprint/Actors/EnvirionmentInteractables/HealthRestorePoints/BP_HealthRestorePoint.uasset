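; Health restore point actor that heals any overlapping actor with an Ability System Component while it stays inside the capsule.
; On begin overlap, its own ability system applies GE_HealthRestore to that actor and stores the effect handle in a map keyed by the target's component.
; On end overlap, it looks up the handle and removes all stacks of the effect, leaving the map entry in place.
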(event `self.Capsule.OnComponentBeginOverlap`
  (params (OverlappedComponent :type "PrimitiveComponent Object Reference") (OtherActor :type "Actor Object Reference") (OtherComp :type "PrimitiveComponent Object Reference") (OtherBodyIndex :type Integer) (bFromSweep :type Boolean) (SweepResult :type "HitResult Structure (by ref)"))
  (bind _returnvalue (`AbilitySystemBlueprintLibrary.GetAbilitySystemComponent` OtherActor))
  (`/Engine/EditorBlueprintResources/StandardMacros.IsValid` _returnvalue
    (:`Is Valid`
      (`KismetSystemLibrary.PrintString` "Overlapped Ability System")
      (bind _returnvalue_2 (`AbilitySystemComponent.BP_ApplyGameplayEffectToTarget` :`self` (`self.AbilitySystem`) :`GameplayEffectClass` "/Game/GameplayAbilitiesBP/Blueprint/Actors/EnvirionmentInteractables/HealthRestorePoints/GE_HealthRestore.GE_HealthRestore_C" :`Target` _returnvalue))
      (`BlueprintMapLibrary.Map_Add` (`self.ActiveHeallingEffects`) _returnvalue _returnvalue_2))))

(event `self.Capsule.OnComponentEndOverlap`
  (params (OverlappedComponent :type "PrimitiveComponent Object Reference") (OtherActor :type "Actor Object Reference") (OtherComp :type "PrimitiveComponent Object Reference") (OtherBodyIndex :type Integer))
  (bind _returnvalue (`AbilitySystemBlueprintLibrary.GetAbilitySystemComponent` OtherActor))
  (bind (_value _returnvalue_2) (`BlueprintMapLibrary.Map_Find` (`self.ActiveHeallingEffects`) _returnvalue))
  (`/Engine/EditorBlueprintResources/StandardMacros.IsValid` _returnvalue
    (:`Is Valid`
      (if _returnvalue_2
        (`AbilitySystemComponent.RemoveActiveGameplayEffect` _returnvalue _value -1)))))

(fn `UserConstructionScript`)