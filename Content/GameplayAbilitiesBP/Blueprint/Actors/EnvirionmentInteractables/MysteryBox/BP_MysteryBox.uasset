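; BP_MysteryBox is an interactable mystery box that offers a random weapon to the pawn that opens it.
; Opening plays a montage while looping timers respawn random PossibleWeapons, each higher than the last, then sink the final one during a timed claim window.
; Only that customer can pick it up; pickup or timeout closes and resets the box.
; CanBuyMysteryBox always returns true, so no cost is checked.
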(event `InteractionInterface.InteractedWith`
  (params (OtherActor :type "Actor Object Reference"))
  (bind _customer (`self.Customer`))
  (`/Engine/EditorBlueprintResources/StandardMacros.IsValid` OtherActor
    (:`Is Valid`
      (if (`self.CanInteractWith`)
        (`/Engine/EditorBlueprintResources/StandardMacros.IsValid` _customer
          (:`Is Valid`
            (if (== OtherActor _customer)
              (`GACharacter.PickupItem` (cast `GACharacter` _customer :!pure true) (`self.MysteryWeapon`))
              (`self.MysteryBoxGunAccepted`)))
          (:`Is Not Valid`
            (bind _aspawn (cast `Pawn` OtherActor))
            (bind _succeded (`self.CanBuyMysteryBox` _aspawn))
            (if _succeded
              (set `self.Customer` _aspawn)
              (`|PlayMontage` null "/Game/GameplayAbilities/Items/MysteryBox/Animations/AM_OpenMysteryBox.AM_OpenMysteryBox"
                (:`then`
                  (bind _returnvalue (`KismetSystemLibrary.K2_SetTimerDelegate` (delegate `MysteryBoxAnim`) 0.1 true))
                  (set `self.MysteryAnimTimerHandle` _returnvalue)
                  (`KismetSystemLibrary.K2_SetTimerDelegate` (delegate `FinishMysteryAnim`) 5.0)
                  (set `self.CanInteractWith` false))))))))))

(event `FinishMysteryAnim`
  (`KismetSystemLibrary.K2_ClearAndInvalidateTimerHandle` (`self.MysteryAnimTimerHandle`))
  (bind _returnvalue (`KismetSystemLibrary.K2_SetTimerDelegate` (delegate `MysteryCountdownAnim`) 0.1 true))
  (set `self.RejectMysteryCountdownAnimTimerHandle` _returnvalue)
  (set `self.CanInteractWith` true)
  (bind _returnvalue_2 (`KismetSystemLibrary.K2_SetTimerDelegate` (delegate `MysteryBoxGunRejection`) 5.0))
  (set `self.RejectMysteryBoxTimerHandle` _returnvalue_2))

(event `MysteryBoxAnim`
  (bind _mysteryweapon (`self.MysteryWeapon`))
  (bind _possibleweapons (`self.PossibleWeapons`))
  (bind _output (`|GetArrayItem` _possibleweapons (`KismetMathLibrary.RandomIntegerInRange` 0 (- (`KismetArrayLibrary.Array_Length` _possibleweapons) 1))))
  (bind _returnvalue (`KismetMathLibrary.MakeRotator` (.roll (.rotation (`SceneComponent.K2_GetComponentToWorld` (`self.OtherMesh`)))) (.pitch (.rotation (`SceneComponent.K2_GetComponentToWorld` (`self.OtherMesh`)))) (+ (.yaw (.rotation (`SceneComponent.K2_GetComponentToWorld` (`self.OtherMesh`)))) 90.0)))
  (`/Engine/EditorBlueprintResources/StandardMacros.IsValid` _mysteryweapon
    (:`Is Valid`
      (bind _returnvalue_2 (`|SpawnActorFromClass` _output (`KismetMathLibrary.MakeTransform` (`KismetMathLibrary.MakeVector` (.x (.location (`self.GetTransform` (`self.MysteryWeapon`)))) (.y (.location (`self.GetTransform` (`self.MysteryWeapon`)))) (+ (.z (.location (`self.GetTransform` (`self.MysteryWeapon`)))) 3.0)) _returnvalue (.scale (`self.GetTransform` (`self.MysteryWeapon`)))) "AlwaysSpawn" "OverrideRootScale" self null))
      (`self.K2_DestroyActor` _mysteryweapon)
      (set `self.MysteryWeapon` _returnvalue_2))
    (:`Is Not Valid`
      (bind _returnvalue_3 (`|SpawnActorFromClass` _output (`KismetMathLibrary.MakeTransform` (.location (`SceneComponent.K2_GetComponentToWorld` (`self.OtherMesh`))) _returnvalue (.scale (`SceneComponent.K2_GetComponentToWorld` (`self.OtherMesh`)))) "AlwaysSpawn" "OverrideRootScale" self null))
      (set `self.MysteryWeapon` _returnvalue_3))))

(event `MysteryCountdownAnim`
  (bind _mysteryweapon (`self.MysteryWeapon`))
  (`self.K2_SetActorLocation` _mysteryweapon (`KismetMathLibrary.MakeVector` (.x (`self.K2_GetActorLocation` _mysteryweapon)) (.y (`self.K2_GetActorLocation` _mysteryweapon)) (+ (.z (`self.K2_GetActorLocation` _mysteryweapon)) -1.0)) false false))

(event `MysteryBoxGunRejection`
  (`self.K2_DestroyActor` (`self.MysteryWeapon`))
  (set `self.MysteryWeapon` null :!label _label)
  (`|PlayMontage` null "/Game/GameplayAbilities/Items/MysteryBox/Animations/AM_CloseMysteryBox.AM_CloseMysteryBox"
    (:`then`
      (`KismetSystemLibrary.K2_ClearAndInvalidateTimerHandle` (`self.RejectMysteryCountdownAnimTimerHandle`))
      (set `self.Customer` null)
      (`KismetSystemLibrary.K2_ClearAndInvalidateTimerHandle` (`self.RejectMysteryBoxTimerHandle`)))))

(event `MysteryBoxGunAccepted`
  (goto _label))

(fn `CanBuyMysteryBox`
  (params (Activator :type "Actor Object Reference"))
  (returns (Succeded :type Boolean))
  (return true))

(fn `UserConstructionScript`
  (`parent.UserConstructionScript`))