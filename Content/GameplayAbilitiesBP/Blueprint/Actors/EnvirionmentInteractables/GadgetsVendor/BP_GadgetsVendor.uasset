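; Gadgets vendor actor that displays a rotating text widget and a rotating logo mesh; no vending logic is in its graphs.
; Two rotating movement components are bound on BeginPlay, one to the widget and one to the logo.
; A shared initialize event pushes the actor's Text into the WBP_CustomText widget, running from the construction script and again after a short delay on BeginPlay.
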(event `self.ReceiveBeginPlay`
  (`MovementComponent.SetUpdatedComponent` (`self.RotatingMovement_Widget`) (`self.Widget`))
  (`MovementComponent.SetUpdatedComponent` (`self.RotatingMovement_Logo`) (`self.SM_vendor_logo`))
  (`KismetSystemLibrary.Delay` 0.2)
  (`self.IntializeWidget`))

(event `IntializeWidget`
  (bind _text (`self.Text`))
  (bind _aswbp_custom_text (cast `/Game/GameplayAbilitiesBP/Blueprint/UI/Framework/CustomHUD/Custom/WBP_CustomText` (`WidgetComponent.GetWidget` (`self.Widget`))))
  (set `/Game/GameplayAbilitiesBP/Blueprint/UI/Framework/CustomHUD/Custom/WBP_CustomText.TextToDisplay` _text _aswbp_custom_text)
  (`TextBlock.SetText` (`/Game/GameplayAbilitiesBP/Blueprint/UI/Framework/CustomHUD/Custom/WBP_CustomText.Text` _aswbp_custom_text) _text))

(fn `UserConstructionScript`
  (`self.IntializeWidget`))