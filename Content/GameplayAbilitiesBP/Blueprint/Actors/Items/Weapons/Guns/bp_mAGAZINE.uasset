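; Gun magazine Blueprint that stores bullets in an array as a last-in, first-out stack.
; Push appends a bullet while the count is at or below Size, so it can hold one more than Size, and reports success.
; Pop removes and returns the last bullet, if any.
; GetMass adds every bullet's mass to the magazine's own, and GetCurrentAmount returns the bullet count.
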(fn `GetCurrentAmount`
  (returns (Amount :type Integer))
  (return (`KismetArrayLibrary.Array_Length` (`self.Bullets`))))

(fn `GetMass`
  (returns (TotalMass :type "Float (double-precision)"))
  (locals (LocMass :type "Float (double-precision)"))
  (set `local.LocMass` (`self.Mass`))
  (for _array_element (`self.Bullets`)
    (set `local.LocMass` (+ (`local.LocMass`) (`/Game/GameplayAbilitiesBP/Blueprint/Actors/Items/Weapons/Guns/Bullet/BulletData.GetMass` _array_element))))
  (return (`local.LocMass`)))

(fn `Pop`
  (returns (`Popped Bullet` :type "/Game/GameplayAbilitiesBP/Blueprint/Actors/Items/Weapons/Guns/Bullet/BulletData Object Reference"))
  (locals (LocBullet :type "/Game/GameplayAbilitiesBP/Blueprint/Actors/Items/Weapons/Guns/Bullet/BulletData Object Reference"))
  (bind _returnvalue (`KismetArrayLibrary.Array_LastIndex` (`self.Bullets`)))
  (if (>= _returnvalue 0)
    (set `local.LocBullet` (`|GetArrayItem` (`self.Bullets`) _returnvalue))
    (`KismetArrayLibrary.Array_Remove` (`self.Bullets`) _returnvalue))
  (return (`local.LocBullet`)))

(fn `Push`
  (params (NewBullet :type "/Game/GameplayAbilitiesBP/Blueprint/Actors/Items/Weapons/Guns/Bullet/BulletData Object Reference"))
  (returns (Success :type Boolean))
  (if (>= (`self.Size`) (`KismetArrayLibrary.Array_Length` (`self.Bullets`)))
    (`KismetArrayLibrary.Array_Add` (`self.Bullets`) NewBullet)
    (return true)
    (else
      (return false))))

(fn `UserConstructionScript`)