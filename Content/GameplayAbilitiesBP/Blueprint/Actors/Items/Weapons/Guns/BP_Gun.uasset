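; Gun weapon actor that aims along its owner's view and feeds projectiles from a magazine.
; Tick traces from the owner's eyes and, on a hit, rotates the gun toward the trace end.
; CommitProjectile pops the magazine or, when it is empty or missing (CanFireProjectile returns true), reloads with the first diameter-matched magazine from the GACharacter's inventory.
; Projectile transform and variance functions are empty stubs.
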(event `self.ReceiveTick`
  (params (DeltaSeconds :type "Float (single-precision)"))
  (bind _returnvalue (`self.GetOwner`))
  (bind (_outlocation _outrotation) (`self.GetActorEyesViewPoint` _returnvalue))
  (`/Engine/EditorBlueprintResources/StandardMacros.IsValid` _returnvalue
    (:`Is Valid`
      (bind (_outhit _returnvalue_2) (`KismetSystemLibrary.LineTraceSingle` :`Start` _outlocation :`End` (+ _outlocation (* (`KismetMathLibrary.GetForwardVector` _outrotation) (`self.PointMaxEffectiveRange`))) :`TraceChannel` "TraceTypeQuery1" :`DrawDebugType` "ForDuration"))
      (if _returnvalue_2
        (`self.K2_SetActorRotation` (`KismetMathLibrary.FindLookAtRotation` (`self.K2_GetActorLocation`) (`.TraceEnd` (`GameplayStatics.BreakHitResult` _outhit))))))))

(fn `CanFireProjectile`
  (returns (`Magazine is empty` :type Boolean))
  (bind _magazine (`self.Magazine`))
  (`/Engine/EditorBlueprintResources/StandardMacros.IsValid` _magazine
    (:`Is Valid`
      (return (<= (`/Game/GameplayAbilitiesBP/Blueprint/Actors/Items/Weapons/Guns/bp_mAGAZINE.GetCurrentAmount` _magazine) 0)))
    (:`Is Not Valid`
      (return true))))

(fn `CanReloadMagazine`
  (returns (`Owner has more magazines` :type Boolean))
  (locals (LocSucceded :type Boolean :default false))
  (bind _diameter (`self.Diameter`))
  (`KismetSystemLibrary.PrintString` "Check reload")
  (for _array_element (`InventoryComponent.Inventory` (`GACharacter.Inventory` (cast `GACharacter` (`self.GetOwner`) :!pure true)))
    (bind _asbp_magazine (cast `/Game/GameplayAbilitiesBP/Blueprint/Actors/Items/Weapons/Guns/bp_mAGAZINE` _array_element))
    (bind _diameter_2 (`/Game/GameplayAbilitiesBP/Blueprint/Actors/Items/Weapons/Guns/bp_mAGAZINE.Diameter` _asbp_magazine))
    (if (and (<= _diameter_2 (+ _diameter 0.1)) (>= _diameter_2 (- _diameter 0.1)))
      (set `local.LocSucceded` true)
      (`KismetSystemLibrary.PrintString` "Can reload")
      (break)))
  (return (`local.LocSucceded`)))

(fn `CommitProjectile`
  (returns (OutBullet :type "/Game/GameplayAbilitiesBP/Blueprint/Actors/Items/Weapons/Guns/Bullet/BP_Cartridge Object Reference"))
  (bind _magazine_is_empty (`self.CanFireProjectile`))
  (if (not _magazine_is_empty)
    (bind _popped_bullet (`/Game/GameplayAbilitiesBP/Blueprint/Actors/Items/Weapons/Guns/bp_mAGAZINE.Pop` (`self.Magazine`)))
    (return _popped_bullet)
    (else
      (`self.CommitReload`)
      (return null))))

(fn `CommitReload`
  (bind _diameter (`self.Diameter`))
  (bind _inventory (`InventoryComponent.Inventory` (`GACharacter.Inventory` (cast `GACharacter` (`self.GetOwner`) :!pure true))))
  (bind _owner_has_more_magazines (`self.CanReloadMagazine`))
  (if _owner_has_more_magazines
    (for (_array_element _array_index) _inventory
      (bind _asbp_magazine (cast `/Game/GameplayAbilitiesBP/Blueprint/Actors/Items/Weapons/Guns/bp_mAGAZINE` _array_element))
      (bind _diameter_2 (`/Game/GameplayAbilitiesBP/Blueprint/Actors/Items/Weapons/Guns/bp_mAGAZINE.Diameter` _asbp_magazine))
      (if (and (<= _diameter_2 (+ _diameter 0.1)) (>= _diameter_2 (- _diameter 0.1)))
        (set `self.Magazine` _asbp_magazine)
        (`KismetArrayLibrary.Array_Remove` _inventory _array_index)
        (break)))))

(fn `GetProjectileTransform`
  (returns (`Bullet Transform` :type "Transform Structure"))
  (return))

(fn `GetVarrience`)

(fn `UserConstructionScript`
  (`parent.UserConstructionScript`))