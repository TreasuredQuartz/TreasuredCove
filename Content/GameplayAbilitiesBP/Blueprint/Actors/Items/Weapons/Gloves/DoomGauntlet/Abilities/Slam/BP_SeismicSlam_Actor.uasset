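; Short-lived visual actor for the Doom Gauntlet's Seismic Slam ability, showing animated ground cracks and expiring one second after BeginPlay.
; The construction script puts a dynamic instance of the tiling cracks decal material on the Triangle component and starts a looping timer.
; The timer advances Time and writes it to the material's Time parameter.
; Tick also adds delta seconds to the same Time variable, so both sources accumulate.
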(event `self.ReceiveBeginPlay`
  (`self.SetLifeSpan` 1.0))

(event `self.ReceiveTick`
  (params (DeltaSeconds :type "Float (single-precision)"))
  (set `self.Time` (+ DeltaSeconds (`self.Time`))))

(fn `SlamLoopTime`
  (set `self.Time` (+ (`self.Time`) 0.05))
  (`MaterialInstanceDynamic.SetScalarParameterValue` (`self.MID`) "Time" (`self.Time`)))

(fn `UserConstructionScript`
  (`/Engine/EditorBlueprintResources/StandardMacros.IsValid` (`self.MID`)
    (:`Is Valid`
      _)
    (:`Is Not Valid`
      (bind _returnvalue (`PrimitiveComponent.CreateDynamicMaterialInstance` (`self.Triangle`) 0 "/Game/GameplayAbilitiesBP/Blueprint/Actors/Items/Weapons/Gloves/DoomGauntlet/Mesh/M_TilingCracksDecal.M_TilingCracksDecal" "None"))
      (set `self.MID` _returnvalue)
      (`PrimitiveComponent.SetMaterial` (`self.Triangle`) 0 (`self.MID`))))
  (`KismetSystemLibrary.K2_SetTimer` null "SlamLoopTime" 0.05 true))