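; BP_358Key is a melee weapon Blueprint that tracks equipped panels under the Kingdom Hearts Days category.
; Its EquippedPanels component acts as the item repository, with events that add or subtract one item by name.
; Functions look up an item's index by name, read quantity by index and expose the component itself.
; The construction script only calls its parent.
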(event `SubtractFromEquipped`
  (params (Name :type Name))
  (`RepositoryComponent.SubtractItem` (`self.EquippedPanels`) "KingdomHearts|Days" Name 1))

(event `AddToEquipped`
  (params (Name :type Name))
  (`RepositoryComponent.AddItem` (`self.EquippedPanels`) "KingdomHearts|Days" Name 1))

(fn `FindEquipped`
  (params (Name :type Name))
  (returns (Index :type Integer))
  (return (`RepositoryComponent.GetItemIndex` (`self.EquippedPanels`) "KingdomHearts|Days" Name)))

(fn `GetEquippedQuantity`
  (params (Index :type Integer))
  (returns (Quantity :type Integer))
  (return (`RepositoryComponent.GetItemQuantity` (`self.EquippedPanels`) "KingdomHearts|Days" (`KismetMathLibrary.Conv_IntToByte` Index))))

(fn `GetRepositoryComponent`
  (returns (ReturnValue :type "RepositoryComponent Object Reference"))
  (return (`self.EquippedPanels`)))

(fn `UserConstructionScript`
  (`parent.UserConstructionScript`))