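; BP_DoomfistGauntlet is a melee weapon Blueprint that handles the charge-up state of a Doomfist-style gauntlet.
; StartCharging runs a fast looping timer that increments ChargeAmount, prints it for debugging, and stops the timer once full charge is reached.
; StopCharging clears the timer and keeps the accumulated charge, while ClearChargeAmount zeroes it and stops charging.
; The charge is not consumed within this Blueprint, and construction defers to the parent.
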(event `StartCharging`
  (bind _returnvalue (`KismetSystemLibrary.K2_SetTimerDelegate` (delegate `ChargingLoop`) 0.05 true))
  (set `self.ChargeTimerHandle` _returnvalue))

(event `ChargingLoop`
  (bind _output_get (set `self.ChargeAmount` (+ (`self.ChargeAmount`) 0.05)))
  (`KismetSystemLibrary.PrintString` (`KismetStringLibrary.Concat_StrStr` "Charging: " (`KismetStringLibrary.Conv_DoubleToString` _output_get)))
  (if (>= _output_get 1.0)
    (`self.StopCharging`)))

(event `StopCharging`
  (`KismetSystemLibrary.K2_ClearAndInvalidateTimerHandle` (`self.ChargeTimerHandle`)))

(event `ClearChargeAmount`
  (set `self.ChargeAmount` 0.0)
  (`self.StopCharging`))

(fn `UserConstructionScript`
  (`parent.UserConstructionScript`))