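; BP_Nuke is a zombie power-up drop pickup that spawns a BP_Blizzard actor when a pawn picks it up.
; On BeginPlay it assigns the static mesh to its RotatingMovement component, so only the mesh rotates.
; On pickup it spawns the blizzard at its own transform with the pawn as Instigator, then defers to the parent pickup logic, which non-pawn actors never reach.
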(event `self.ReceiveBeginPlay`
  (`parent.ReceiveBeginPlay`)
  (`MovementComponent.SetUpdatedComponent` (`self.RotatingMovement`) (`self.StaticMesh`)))

(event `PickupInterface.OnPickedUp`
  (params (OtherActor :type "Actor Object Reference"))
  (bind _aspawn (cast `Pawn` OtherActor))
  (`|SpawnActorFromClass` "/Game/GameplayAbilitiesBP/Blueprint/Actors/Items/ZombiePowerUpDrops/BP_Blizzard.BP_Blizzard_C" (`self.GetTransform`) "Undefined" "OverrideRootScale" null _aspawn)
  (`parent.OnPickedUp` OtherActor))

(fn `UserConstructionScript`
  (`parent.UserConstructionScript`))