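; BP_FrozenZombie is a short-lived actor that shows a static, posed copy of a skeletal mesh, apparently a frozen zombie.
; On BeginPlay, if MeshRef is valid, it copies that component's mesh asset and materials onto a PoseableMesh.
; It then snapshots the current pose by applying each socket name's world transform as a bone transform, and sets a lifespan to remove itself after a few seconds.
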(event `self.ReceiveBeginPlay`
  (bind _meshref (`self.MeshRef`))
  (bind _meshref_2 (`self.MeshRef`))
  (`/Engine/EditorBlueprintResources/StandardMacros.IsValid` (`self.MeshRef`)
    (:`Is Valid`
      (`|ExecutionSequence`
        (:`then_0`
          ;[1 1 1] Set mesh and material
          (`SkinnedMeshComponent.SetSkinnedAssetAndUpdate` (`self.PoseableMesh`) (`SkeletalMeshComponent.SkeletalMeshAsset` _meshref_2) false)
          (for (_array_element _array_index) (`MeshComponent.GetMaterials` _meshref_2)
            (`PrimitiveComponent.SetMaterial` (`self.PoseableMesh`) _array_index _array_element)))
        (:`then_1`
          ;[1 1 1] Copy current pose
          (for _array_element_2 (`SceneComponent.GetAllSocketNames` _meshref)
            (`PoseableMeshComponent.SetBoneTransformByName` (`self.PoseableMesh`) _array_element_2 (`SceneComponent.GetSocketTransform` _meshref _array_element_2 "RTS_World") "WorldSpace")))
        (:`then_2`
          ;[1 1 1] Set lifespan
          (`self.SetLifeSpan` 5.0))))))

(fn `UserConstructionScript`)