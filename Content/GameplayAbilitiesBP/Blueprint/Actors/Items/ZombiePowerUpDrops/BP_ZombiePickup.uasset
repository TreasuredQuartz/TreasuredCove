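; BP_ZombiePickup is a pickup actor for zombie power-up drops that only the first player's character can collect.
; Its OnCanBePickedUp check accepts an overlapping actor only if it matches player character 0.
; Each tick, it sets the Plane's relative location along the normalized camera-to-pickup direction, scaled by PlaneDistance, to keep the plane behind the pickup mesh from the player's view.
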(event `self.ReceiveTick`
  (params (DeltaSeconds :type "Float (single-precision)"))
  (`parent.ReceiveTick` DeltaSeconds)
  (`SceneComponent.K2_SetRelativeLocation` (`self.Plane`) (* (`KismetMathLibrary.Normal` (- (`self.K2_GetActorLocation`) (`PlayerCameraManager.GetCameraLocation` (`GameplayStatics.GetPlayerCameraManager` 0)))) (`self.PlaneDistance`)) false false))

(fn `OnCanBePickedUp`
  (params (OtherActor :type "Actor Object Reference"))
  (returns (ReturnValue :type Boolean))
  (return (== OtherActor (`GameplayStatics.GetPlayerCharacter` 0))))

(fn `UserConstructionScript`
  (`parent.UserConstructionScript`))