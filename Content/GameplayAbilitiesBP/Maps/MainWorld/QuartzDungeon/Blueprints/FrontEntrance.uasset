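; Double front entrance door for the Quartz Dungeon that swings open or closed each time it is interacted with.
; BeginPlay caches the starting yaw of the Left and Right doors.
; A FlipFlop on interaction sets the Open flag and plays or reverses a timeline, whose lerped angle swings the doors in opposite directions to nearly a right angle.
; Rotation is applied in world space as yaw only, zeroing pitch and roll.
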(event `self.ReceiveBeginPlay`
  (bind (_returnvalue_roll _returnvalue_pitch _returnvalue_yaw) (`KismetMathLibrary.BreakRotator` (`SceneComponent.K2_GetComponentRotation` (`self.Right`))))
  (bind (_returnvalue_roll_2 _returnvalue_pitch_2 _returnvalue_yaw_2) (`KismetMathLibrary.BreakRotator` (`SceneComponent.K2_GetComponentRotation` (`self.Left`))))
  (set `self.OGDoorRightRotation` _returnvalue_yaw)
  (set `self.OGDoorLeftRotation` _returnvalue_yaw_2))

(event `InteractionInterface.InteractedWith`
  (params (OtherActor :type "Actor Object Reference"))
  (bind _isa (`/Engine/EditorBlueprintResources/StandardMacros.FlipFlop`)
    (:`A`
      (set `self.Open?` _isa)
      (bind (_direction _floattrack) (`Timeline|Timeline_0` :!label _label)
        (:`Update`
          (set `self.ActiveDoorValue` (`KismetMathLibrary.Lerp` 0.0 89.0 _floattrack))
          (`self.Open/CloseDoor`))))
    (:`B`
      (set `self.Open?` _isa)
      (goto _label :!via `Reverse`))))

(event `self.Open/CloseDoor`
  (bind _activedoorvalue (`self.ActiveDoorValue`))
  (`SceneComponent.K2_SetWorldRotation` (`self.Right`) (`KismetMathLibrary.MakeRotator` 0.0 0.0 (+ (`self.OGDoorRightRotation`) _activedoorvalue)) false false)
  (`SceneComponent.K2_SetWorldRotation` (`self.Left`) (`KismetMathLibrary.MakeRotator` 0.0 0.0 (+ (`self.OGDoorLeftRotation`) (* -1 _activedoorvalue))) false false))

(fn `UserConstructionScript`
  (`parent.UserConstructionScript`))