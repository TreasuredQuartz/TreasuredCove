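; BP_QuartzSnowField is a snow field actor for the Quartz dungeon, tiled from instanced snow planes.
; Initialization adds a Width by Length grid of instances, sizes an overlap box to match and creates a dynamic brush material on SnowBrush.
; Update pushes SnowStrength into that material's Strength parameter.
; The box toggles actor spawning on any overlapping actor's MovementTrailComponent, enabling it on entry and disabling it on exit.
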(event `self.ReceiveBeginPlay`
  (`self.InitializeSnowPlane`))

(event `Update`
  (params (SnowStrength :type "Float (double-precision)"))
  (bind _output_get (set `self.SnowStrength` SnowStrength))
  (`MaterialInstanceDynamic.SetScalarParameterValue` (`self.BrushMID`) "Strength" _output_get))

(event `self.Box.OnComponentBeginOverlap`
  (params (OverlappedComponent :type "PrimitiveComponent Object Reference") (OtherActor :type "Actor Object Reference") (OtherComp :type "PrimitiveComponent Object Reference") (OtherBodyIndex :type Integer) (bFromSweep :type Boolean) (SweepResult :type "HitResult Structure (by ref)"))
  (bind _returnvalue (`self.GetComponentByClass` OtherActor "/Script/TreasuredCove.MovementTrailComponent"))
  (`/Engine/EditorBlueprintResources/StandardMacros.IsValid` _returnvalue
    (:`Is Valid`
      (`MovementTrailComponent.SetSpawnActors` _returnvalue true))))

(event `self.Box.OnComponentEndOverlap`
  (params (OverlappedComponent :type "PrimitiveComponent Object Reference") (OtherActor :type "Actor Object Reference") (OtherComp :type "PrimitiveComponent Object Reference") (OtherBodyIndex :type Integer))
  (bind _returnvalue (`self.GetComponentByClass` OtherActor "/Script/TreasuredCove.MovementTrailComponent"))
  (`/Engine/EditorBlueprintResources/StandardMacros.IsValid` _returnvalue
    (:`Is Valid`
      (`MovementTrailComponent.SetSpawnActors` _returnvalue false))))

(fn `InitializeSnowPlane`
  (bind _returnvalue (/ (`self.Length`) 2))
  (bind _returnvalue_2 (/ (`self.Width`) 2))
  (`KismetArrayLibrary.Array_Clear` (`self.SnowPlanes`))
  (for _index (range (* _returnvalue_2 -1) (+ _returnvalue_2 1))
    (for _index_2 (range (* _returnvalue -1) (+ _returnvalue 1))
      (`InstancedStaticMeshComponent.AddInstance` (`self.SnowInstances`) (`KismetMathLibrary.MakeTransform` (`KismetMathLibrary.MakeVector` (`KismetMathLibrary.Conv_IntToDouble` (* _index_2 200)) (`KismetMathLibrary.Conv_IntToDouble` (* _index 200)))) false)))
  (`BoxComponent.SetBoxExtent` (`self.Box`) (`KismetMathLibrary.MakeVector` (`KismetMathLibrary.Conv_IntToDouble` (* (`self.Length`) 100)) (`KismetMathLibrary.Conv_IntToDouble` (* (`self.Width`) 100)) 200.0) true)
  (`/Engine/EditorBlueprintResources/StandardMacros.IsValid` (`self.BrushMID`)
    (:`Is Valid`
      _)
    (:`Is Not Valid`
      (bind _returnvalue_3 (`KismetMaterialLibrary.CreateDynamicMaterialInstance` "/Game/GameplayAbilitiesBP/Maps/MainWorld/QuartzDungeon/Blueprints/RuntimeSnowField/M_SnowBrush_Addition.M_SnowBrush_Addition"))
      (bind _output_get (set `self.BrushMID` _returnvalue_3))
      (`PrimitiveComponent.SetMaterial` (`self.SnowBrush`) 0 _output_get)))
  (`self.Update` (`self.SnowStrength`)))

(fn `UserConstructionScript`
  (if (`self.bRunConstruction`)
    (`self.InitializeSnowPlane`)
    (else
      (set `self.bRunConstruction` false))))