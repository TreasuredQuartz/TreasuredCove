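; Base room for the Tower of Owen map that animates an actor moving into and out of it.
; Enter and exit timelines lerp the actor between start and end transforms from stub getters, ignoring move input for player controllers meanwhile.
; Returns play the same timelines in reverse.
; Finishing a forward exit calls the move to the next room, while finishing a reversed entry calls the move to the previous one.
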(event `EnterRoom`
  (params (Actor :type "Actor Object Reference"))
  (bind (_asplayer_controller _bsuccess) (cast `PlayerController` (`self.GetInstigatorController` (`self.MovingActor`)) :!pure true))
  (set `self.MovingActor` Actor)
  (`self.OnRoom_BeginEnter`)
  (if _bsuccess
    (`Controller.SetIgnoreMoveInput` _asplayer_controller true)
    (bind (_direction _leveltransitiontrack) (`Timeline|LevelEnterTimeline` :!via `PlayFromStart` :!label _label)
      (:`Update`
        (`self.K2_SetActorTransform` (`self.MovingActor`) (`KismetMathLibrary.TLerp` (`self.GetEnterStartTransform`) (`self.GetEnterEndTransform`) _leveltransitiontrack) false false))
      (:`Finished`
        (`Controller.SetIgnoreMoveInput` (cast `PlayerController` (`self.GetInstigatorController` (`self.MovingActor`)) :!pure true) false)
        (switch `ETimelineDirection` _direction
          (:`Forward`
            _)
          (:`Backward`
            (`self.MoveToPreviousRoom` (`self.MovingActor`))))
        (set `self.MovingActor` null)
        (`self.OnRoom_EndEntered`)))
    (else
      (goto _label :!via `PlayFromStart`))))

(event `OnRoom_BeginEnter`)

(event `OnRoom_EndEntered`)

(event `ReturnFrom`
  (params (Actor :type "Actor Object Reference"))
  (bind (_asplayer_controller _bsuccess) (cast `PlayerController` (`self.GetInstigatorController` (`self.MovingActor`)) :!pure true))
  (set `self.MovingActor` Actor)
  (`self.OnRoom_BeginEnter`)
  (if _bsuccess
    (`Controller.SetIgnoreMoveInput` _asplayer_controller true)
    (goto _label :!via `ReverseFromEnd`)
    (else
      (goto _label :!via `ReverseFromEnd`))))

(event `ExitRoom`
  (params (Actor :type "Actor Object Reference"))
  (bind (_asplayer_controller _bsuccess) (cast `PlayerController` (`self.GetInstigatorController` (`self.MovingActor`)) :!pure true))
  (set `self.MovingActor` Actor)
  (set `self.bPerformingTransition` true)
  (if _bsuccess
    (`Controller.SetIgnoreMoveInput` _asplayer_controller true)
    (bind (_direction _leveltransitiontrack) (`Timeline|LevelExitTimeline` :!via `PlayFromStart` :!label _label_2)
      (:`Update`
        (`self.K2_SetActorTransform` (`self.MovingActor`) (`KismetMathLibrary.TLerp` (`self.GetExitStartTransform`) (`self.GetExitEndTransform`) _leveltransitiontrack) false true))
      (:`Finished`
        (`Controller.SetIgnoreMoveInput` (cast `PlayerController` (`self.GetInstigatorController` (`self.MovingActor`)) :!pure true) false)
        (switch `ETimelineDirection` _direction
          (:`Forward`
            (`self.MoveToNextRoom` (`self.MovingActor`)))
          (:`Backward`
            _))
        (set `self.MovingActor` null)))
    (else
      (goto _label_2 :!via `PlayFromStart`))))

(event `ReturnTo`
  (params (Actor :type "Actor Object Reference"))
  (bind (_asplayer_controller _bsuccess) (cast `PlayerController` (`self.GetInstigatorController` (`self.MovingActor`)) :!pure true))
  (set `self.MovingActor` Actor)
  (set `self.bPerformingTransition` true)
  (if _bsuccess
    (`Controller.SetIgnoreMoveInput` _asplayer_controller true)
    (goto _label_2 :!via `ReverseFromEnd`)
    (else
      (goto _label_2 :!via `ReverseFromEnd`))))

(fn `GetEnterEndTransform`
  (returns (Transform :type "Transform Structure"))
  (return))

(fn `GetEnterStartTransform`
  (returns (Transform :type "Transform Structure"))
  (return))

(fn `GetExitEndTransform`
  (returns (Transform :type "Transform Structure"))
  (return))

(fn `GetExitStartTransform`
  (returns (Transform :type "Transform Structure"))
  (return))

(fn `UserConstructionScript`)