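; A Mega Man-style double sliding door Blueprint that opens and closes on interaction or when something enters or leaves its collision volume.
; Interaction toggles the door through a FlipFlop, while overlap begin and end play or reverse the same timeline.
; The timeline drives a lerped offset that slides the two panels apart along world X from positions cached at BeginPlay, so movement ignores actor rotation.
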(event `self.ReceiveBeginPlay`
  (bind _returnvalue_x (`KismetMathLibrary.BreakVector` (`SceneComponent.K2_GetComponentLocation` (`self.MegaManDoorRight`))))
  (bind _returnvalue_x_2 (`KismetMathLibrary.BreakVector` (`SceneComponent.K2_GetComponentLocation` (`self.MegaManDoorLeft`))))
  (set `self.OGDoorLeftLocation` _returnvalue_x_2)
  (set `self.OGDoorRightLocation` _returnvalue_x))

(event `self.InteractedWith`
  (params (OtherActor :type "Actor Object Reference"))
  (bind _isa (`/Engine/EditorBlueprintResources/StandardMacros.FlipFlop`)
    (:`A`
      (set `self.Open?` _isa)
      (bind (_direction _floattrack) (`Timeline|FloatTimeline` :!label _label)
        (:`Update`
          (set `self.ActiveDoorValue` (`KismetMathLibrary.Lerp` 0.0 200.0 _floattrack))
          (`self.Open/CloseDoor`))))
    (:`B`
      (set `self.Open?` _isa)
      (goto _label :!via `Reverse`))))

(event `self.Collision.OnComponentBeginOverlap`
  (params (OverlappedComponent :type "PrimitiveComponent Object Reference") (OtherActor :type "Actor Object Reference") (OtherComp :type "PrimitiveComponent Object Reference") (OtherBodyIndex :type Integer) (bFromSweep :type Boolean) (SweepResult :type "HitResult Structure (by ref)"))
  (set `self.Open?` true)
  (goto _label))

(event `self.Collision.OnComponentEndOverlap`
  (params (OverlappedComponent :type "PrimitiveComponent Object Reference") (OtherActor :type "Actor Object Reference") (OtherComp :type "PrimitiveComponent Object Reference") (OtherBodyIndex :type Integer))
  (set `self.Open?` false)
  (goto _label :!via `Reverse`))

(event `self.Open/CloseDoor`
  (bind _activedoorvalue (`self.ActiveDoorValue`))
  (`SceneComponent.K2_SetWorldLocation` (`self.MegaManDoorRight`) (`KismetMathLibrary.MakeVector` (+ _activedoorvalue (`self.OGDoorRightLocation`))) false false)
  (`SceneComponent.K2_SetWorldLocation` (`self.MegaManDoorLeft`) (`KismetMathLibrary.MakeVector` (+ (* -1 _activedoorvalue) (`self.OGDoorLeftLocation`))) false false))

(fn `UserConstructionScript`
  (`parent.UserConstructionScript`))