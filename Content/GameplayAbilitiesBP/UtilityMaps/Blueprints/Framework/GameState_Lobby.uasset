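; Lobby GameState that runs a map vote countdown and moves the match to the winning map.
; The server ticks a one-second timer, tallies PlayerState votes, locks voting, then server-travels after a short delay.
; New players trigger a delayed player-list refresh across lobby controllers.
; Preference pool and option generation are empty stubs; weighted map-picking helpers exist, but the code filling the vote pool is disconnected.
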(event `self.ReceiveBeginPlay`
  (`self.GenerateLobbyPreferrenceMapPool`)
  (`self.GenerateMapOptions`)
  (`/Engine/EditorBlueprintResources/ActorMacros.Switch Has Authority`
    (:`Authority`
      (bind _returnvalue (`KismetSystemLibrary.K2_SetTimerDelegate` (delegate `MapVoteCountdown`) 1.0 true))
      (set `self.MapVoteTimerHandle` _returnvalue)
      (set `self.MapVoteTime` 60))))

(event `MapVoteCountdown`
  (`/Engine/EditorBlueprintResources/StandardMacros.DecrementInt` (`self.MapVoteTime`)
    (:`  `
      (if (<= (`self.MapVoteTime`) 0)
        (`KismetSystemLibrary.K2_ClearAndInvalidateTimerHandle` (`self.MapVoteTimerHandle`))
        (`self.EndVoting`)))))

(event `EndVoting`
  (`KismetSystemLibrary.K2_SetTimerDelegate` (delegate `InitiateTravel`) 10.0)
  (bind _asgame_state_lobby (cast `/Game/GameplayAbilitiesBP/UtilityMaps/Blueprints/Framework/GameState_Lobby` (`GameplayStatics.GetGameState`)))
  (bind _winningmap (`self.FinishMapVoting` _asgame_state_lobby))
  (set `self.CurrentMap` _winningmap))

(event `InitiateTravel`
  (bind (_mapname _maplevel) (break `MultiplayerMapInfo` (`self.CurrentMap`)))
  (`/Engine/EditorBlueprintResources/ActorMacros.Switch Has Authority`
    (:`Authority`
      (`KismetSystemLibrary.ExecuteConsoleCommand` (`KismetStringLibrary.Concat_StrStr` "servertravel /Game/Multiplayer/MultiplayerMaps/" (`KismetStringLibrary.Conv_NameToString` _mapname) _maplevel) (`GameplayStatics.GetPlayerController` 0)))))

(event `NewPlayerAddedToLobby`
  (params (NewController :type "/Game/GameplayAbilitiesBP/UtilityMaps/Blueprints/Framework/PlayerController_Lobby Object Reference"))
  (`|ExecutionSequence`
    (:`then_0`
      (`self.UpdateCurrentPlayers`))
    (:`then_1`
      (`/Game/GameplayAbilitiesBP/UtilityMaps/Blueprints/Framework/PlayerController_Lobby.UpdateCurrentPlayers` NewController))))

(event `UpdateCurrentPlayers`
  (`KismetSystemLibrary.Delay` (* 0.4 (`GameplayStatics.GetNumPlayerStates`)))
  (for _index (range (`GameplayStatics.GetNumPlayerStates`))
    (`/Game/GameplayAbilitiesBP/UtilityMaps/Blueprints/Framework/PlayerController_Lobby.UpdateCurrentPlayers` (cast `/Game/GameplayAbilitiesBP/UtilityMaps/Blueprints/Framework/PlayerController_Lobby` (`GameplayStatics.GetPlayerController` _index) :!pure true))))

(event `GenerateMapOptions`)

(fn `ChooseWeightedMap`
  (returns (SelectedMap :type "MultiplayerMapInfo Structure"))
  (locals (RandomValue :type Integer :default 0))
  (bind _sum (`self.MapPoolSum`))
  (set `local.RandomValue` (`KismetMathLibrary.RandomIntegerInRange` 0 _sum))
  (bind _keys (`BlueprintMapLibrary.Map_Keys` (`/Game/GameplayAbilitiesBP/UtilityMaps/Blueprints/Framework/GameMode_Lobby.GetCurrentMapPool` (cast `/Game/GameplayAbilitiesBP/UtilityMaps/Blueprints/Framework/GameMode_Lobby` (`GameplayStatics.GetGameMode`) :!pure true))))
  (for _array_element _keys
    (bind (_value _returnvalue) (`BlueprintMapLibrary.Map_Find` (`/Game/GameplayAbilitiesBP/UtilityMaps/Blueprints/Framework/GameMode_Lobby.GetCurrentMapPool` (cast `/Game/GameplayAbilitiesBP/UtilityMaps/Blueprints/Framework/GameMode_Lobby` (`GameplayStatics.GetGameMode`) :!pure true)) _array_element))
    (if _returnvalue
      (if (< (`local.RandomValue`) _value)
        (return _array_element)))))

(fn `FinishMapVoting`
  (returns (WinningMap :type "MultiplayerMapInfo Structure"))
  (bind _indexofmaxvalue (`self.GetPlayerMapVotes`))
  (return (`|GetArrayItem` (`self.MapVotePool`) _indexofmaxvalue)))

(fn `GenerateLobbyPreferrenceMapPool`)

(fn `GenerateNextMap`
  (params (OtherMap :type "MultiplayerMapInfo Structure"))
  (returns (SelectedMap :type "MultiplayerMapInfo Structure"))
  (bind _selectedmap (`self.ChooseWeightedMap` :!label _label))
  (if (== _selectedmap OtherMap)
    (goto _label)
    (else
      (return _selectedmap))))

(fn `GetMapVoteTimeRemaining`
  (returns (TimeLeft :type Integer))
  (return (`self.MapVoteTime`)))

(fn `GetPlayerMapVotes`
  (returns (IndexOfMaxValue :type Integer))
  (locals (LocMapVotes :type "Array of Integer"))
  (bind _locmapvotes (`local.LocMapVotes`))
  (for _array_element (`self.PlayerArray`)
    (bind _asbp_player_state_lobby (cast `/Game/GameplayAbilitiesBP/UtilityMaps/Blueprints/Framework/BP_PlayerState_Lobby` _array_element))
    (bind _mapvote (`/Game/GameplayAbilitiesBP/UtilityMaps/Blueprints/Framework/BP_PlayerState_Lobby.MapVote` _asbp_player_state_lobby))
    (`KismetArrayLibrary.Array_Set` _locmapvotes _mapvote (+ (`|GetArrayItem` _locmapvotes _mapvote) 1))
    (`/Game/GameplayAbilitiesBP/UtilityMaps/Blueprints/Framework/BP_PlayerState_Lobby.SetCanVote` _asbp_player_state_lobby false))
  (return (`KismetMathLibrary.MaxOfIntArray` (`local.LocMapVotes`))))

(fn `MapPoolSum`
  (returns (Sum :type Integer))
  (locals (TotalValue :type Integer))
  (bind _values (`BlueprintMapLibrary.Map_Values` (`self.LobbyMapPool`)))
  (for _array_element _values
    (set `local.TotalValue` (+ _array_element (`local.TotalValue`))))
  (return (`local.TotalValue`)))

(fn `UserConstructionScript`)