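; Lobby game mode that tracks joining players and tallies their map preferences for multiplayer.
; On post login it notifies GameState_Lobby and adds the player state's preferences to MultiplayerMapPool, a map of vote counts exposed through GetCurrentMapPool.
; Logout only refreshes the game state's current players.
; A removal function decrements counts and drops emptied entries, but nothing in this file calls it.
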(event `self.ReceiveBeginPlay`)

(event `self.K2_PostLogin`
  (params (NewPlayer :type "PlayerController Object Reference"))
  (`KismetSystemLibrary.PrintString` "Game Mode: On Post Login")
  (bind _asplayer_controller_lobby (cast `/Game/GameplayAbilitiesBP/UtilityMaps/Blueprints/Framework/PlayerController_Lobby` NewPlayer))
  (`/Game/GameplayAbilitiesBP/UtilityMaps/Blueprints/Framework/GameState_Lobby.NewPlayerAddedToLobby` (cast `/Game/GameplayAbilitiesBP/UtilityMaps/Blueprints/Framework/GameState_Lobby` (`GameplayStatics.GetGameState`) :!pure true) _asplayer_controller_lobby)
  (`self.AddPlayerMapPoolToLobby` (`Controller.PlayerState` _asplayer_controller_lobby)))

(event `self.K2_OnLogout`
  (params (ExitingController :type "Controller Object Reference"))
  (`/Game/GameplayAbilitiesBP/UtilityMaps/Blueprints/Framework/GameState_Lobby.UpdateCurrentPlayers` (cast `/Game/GameplayAbilitiesBP/UtilityMaps/Blueprints/Framework/GameState_Lobby` (`GameplayStatics.GetGameState`) :!pure true))
  (`/Engine/EditorBlueprintResources/StandardMacros.IsValid` (`Controller.PlayerState` ExitingController)))

(event `self.K2_OnSetMatchState`
  (params (NewState :type Name)))

(fn `AddPlayerMapPoolToLobby`
  (params (NewPlayerState :type "PlayerState Object Reference"))
  (for _array_element (`/Game/GameplayAbilitiesBP/UtilityMaps/Blueprints/Framework/BP_PlayerState_Lobby.GetMapPreferences` (cast `/Game/GameplayAbilitiesBP/UtilityMaps/Blueprints/Framework/BP_PlayerState_Lobby` NewPlayerState :!pure true))
    (bind (_value _returnvalue) (`BlueprintMapLibrary.Map_Find` (`self.MultiplayerMapPool`) _array_element))
    (if _returnvalue
      (`BlueprintMapLibrary.Map_Add` (`self.MultiplayerMapPool`) _array_element (+ _value 1))
      (else
        (`BlueprintMapLibrary.Map_Add` (`self.MultiplayerMapPool`) _array_element 1)))))

(fn `GetCurrentMapPool`
  (returns (MapPool :type "Map of MultiplayerMapInfo Structure to Integer"))
  (return (`self.MultiplayerMapPool`)))

(fn `RemovePlayerMapPoolFromLobby`
  (params (LeavingPlayer :type "PlayerState Object Reference"))
  (for _array_element (`/Game/GameplayAbilitiesBP/UtilityMaps/Blueprints/Framework/BP_PlayerState_Lobby.GetMapPreferences` (cast `/Game/GameplayAbilitiesBP/UtilityMaps/Blueprints/Framework/BP_PlayerState_Lobby` LeavingPlayer :!pure true))
    (bind (_value _returnvalue) (`BlueprintMapLibrary.Map_Find` (`self.MultiplayerMapPool`) _array_element))
    (if _returnvalue
      (bind _returnvalue_2 (+ _value -1))
      (if (> _returnvalue_2 0)
        (`BlueprintMapLibrary.Map_Add` (`self.MultiplayerMapPool`) _array_element _returnvalue_2)
        (else
          (`BlueprintMapLibrary.Map_Remove` (`self.MultiplayerMapPool`) _array_element))))))

(fn `UserConstructionScript`)