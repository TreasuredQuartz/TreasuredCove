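; Lobby player controller that loads the player's account profile and shows the lobby menu.
; On BeginPlay it registers five default class loadouts with GISSMultiplayer, then looks up the user account by net ID to fill lobby player info (name, background, level, rank) and saved loadouts.
; It creates WBP_LobbyMenu with the mouse cursor shown and forwards current-player updates to that widget.
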(event `self.ReceiveBeginPlay`
  (`/Engine/EditorBlueprintResources/ActorMacros.Switch Has Authority`
    (:`Authority`
      _)
    (:`Remote`
      _))
  (`self.GetAllUserAttributes`)
  (`self.CreateLobbyMenu`))

(event `CreateLobbyMenu`
  (set `self.bShowMouseCursor` true)
  (bind _returnvalue (`|CreateWidget` "/Game/GameplayAbilitiesBP/UtilityMaps/Blueprints/UI/WBP_LobbyMenu.WBP_LobbyMenu_C" self))
  (bind _output_get (set `self.LobbyMenu` _returnvalue))
  (`UserWidget.AddToViewport` _output_get 0))

(event `UpdateCurrentPlayers`
  (`/Game/GameplayAbilitiesBP/UtilityMaps/Blueprints/UI/WBP_LobbyMenu.UpdateCurrentPlayers` (`self.LobbyMenu`)))

(fn `GetAllUserAttributes`
  (locals (AccountInfo :type "BPUserOnlineAccount Structure"))
  (`GISS_Multiplayer.SetDefaultLoadouts` (subsystem `GISS_Multiplayer`) (`|MakeArray` "/Game/GameplayAbilitiesBP/Blueprint/UI/InfiniteWarfare/Loadout/DefaultLoadouts/Loadout_Assault.Loadout_Assault_C" "/Game/GameplayAbilitiesBP/Blueprint/UI/InfiniteWarfare/Loadout/DefaultLoadouts/Loadout_Predator.Loadout_Predator_C" "/Game/GameplayAbilitiesBP/Blueprint/UI/InfiniteWarfare/Loadout/DefaultLoadouts/Loadout_Phantom.Loadout_Phantom_C" "/Game/GameplayAbilitiesBP/Blueprint/UI/InfiniteWarfare/Loadout/DefaultLoadouts/Loadout_Stronghold.Loadout_Stronghold_C" "/Game/GameplayAbilitiesBP/Blueprint/UI/InfiniteWarfare/Loadout/DefaultLoadouts/Loadout_Outlaw.Loadout_Outlaw_C" :!type "MultiplayerLoadout Class Reference"))
  (bind _accountinfo (`AdvancedIdentityLibrary.GetUserAccount` (`AdvancedSessionsLibrary.GetUniqueNetID` null))
    (:`OnSuccess`
      (bind _attributes (`GISS_Multiplayer.GetUserAccountAttributes` (subsystem `GISS_Multiplayer`)))
      (bind (_displayname _clanname _title _experience _level _prestige _rankicon _background _portrait _emblemicon _equippedcallingcards _loadouts) (break `AccountAttributes` _attributes))
      (setmembers `/Game/GameplayAbilitiesBP/UtilityMaps/Blueprints/Framework/ST_LobbyPlayerInfo` :`StructRef` (`self.PlayerLobbyInfo`) :`Name` (`KismetTextLibrary.Conv_StringToText` (`AdvancedIdentityLibrary.GetUserAccountDisplayName` _accountinfo)) :`PlayerBackground` _background :`Level` _level :`Rank` _rankicon)
      (set `self.Loadouts` _loadouts)
      (return))))

(fn `UserConstructionScript`)