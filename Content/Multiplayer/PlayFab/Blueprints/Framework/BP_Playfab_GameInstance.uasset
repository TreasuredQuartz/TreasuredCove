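; PlayFab game instance that handles player account registration and email login for the multiplayer framework.
; Init sets the PlayFab title ID, then SignUp and Login send client requests to register a new user or sign in with email and password.
; Success callbacks for both open the main menu level, while OnLoginFailure, bound to registration failure, logs the error name, message and details.
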(event `self.ReceiveInit`
  (`PlayFabUtilities.setPlayFabSettings` (`self.Game Id`)))

(event `SignUp`
  (params (Username :type String) (Password :type String) (Email :type String))
  ;[1 1 1] Registerring for a new account
  (`PlayFabClientAPI.RegisterPlayFabUser` (make `ClientRegisterPlayFabUserRequest` null Username Email "" null Password "" false Username) (delegate `OnRegisterSuccess`) (delegate `OnLoginFailure`)))

(event `OnRegisterSuccess`
  (params (result :type "ClientRegisterPlayFabUserResult Structure") (customData :type "Object Object Reference"))
  ;[1 1 1] Registerring for a new account
  (`GameplayStatics.OpenLevelBySoftObjectPtr` "/Game/GameplayAbilities/Maps/UtilityMaps/MainMenu.MainMenu"))

(event `OnLoginFailure`
  (params (error :type "PlayFabError Structure") (customData :type "Object Object Reference"))
  ;[1 1 1] Registerring for a new account
  (`KismetSystemLibrary.LogString` (`KismetTextLibrary.Conv_TextToString` (`|FormatText` "Error Name: {Name} \nError Message: {Message} \nError Details: {Details}" error_ErrorName error_ErrorMessage error_ErrorDetails))))

(event `Login`
  (params (Email :type String) (Password :type String))
  ;[1 1 1] Log into account
  (`PlayFabClientAPI.LoginWithEmailAddress` (make `ClientLoginWithEmailAddressRequest` null Email null Password) (delegate `OnLoginSuccess`) (`|CreateDelegate` :!event `OnLoginFailure`)))

(event `OnLoginSuccess`
  (params (result :type "ClientLoginResult Structure") (customData :type "Object Object Reference"))
  ;[1 1 1] Log into account
  (`GameplayStatics.OpenLevelBySoftObjectPtr` "/Game/GameplayAbilities/Maps/UtilityMaps/MainMenu.MainMenu"))