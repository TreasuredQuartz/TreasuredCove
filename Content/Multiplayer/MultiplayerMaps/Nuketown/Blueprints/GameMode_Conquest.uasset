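; Conquest game mode that fills empty match slots with AI bots, starts the match and tracks kills and deaths.
; On WaitingToStart it spawns bots at player starts up to the match player count, then calls StartMatch.
; Default pawn spawn overrides bind HealthComponent events, and player deaths update both PlayerStates only when both controllers are PlayerControllers.
; UpdateGamestateInfo copies mode, duration and team lives into GameState_Conquest.
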(event `self.ReceiveBeginPlay`)

(event `PlayerKilled`
  (params (Player :type "PlayerController Object Reference") (ResponsiblePlayer :type "PlayerController Object Reference"))
  (`|ExecutionSequence`
    (:`then_0`
      (`/Engine/EditorBlueprintResources/StandardMacros.IncrementInt` (`/Game/Multiplayer/MultiplayerMaps/Nuketown/Blueprints/PlayerState_Conquest.Deaths` (cast `/Game/Multiplayer/MultiplayerMaps/Nuketown/Blueprints/PlayerState_Conquest` (`Controller.PlayerState` Player) :!pure true))))
    (:`then_1`
      (`/Engine/EditorBlueprintResources/StandardMacros.IncrementInt` (`/Game/Multiplayer/MultiplayerMaps/Nuketown/Blueprints/PlayerState_Conquest.Kills` (cast `/Game/Multiplayer/MultiplayerMaps/Nuketown/Blueprints/PlayerState_Conquest` (`Controller.PlayerState` ResponsiblePlayer) :!pure true))))))

(event `UpdateGamestateInfo`
  (bind _totallives (`self.TotalLives`))
  (bind _asgame_state_conquest (cast `/Game/Multiplayer/MultiplayerMaps/Nuketown/Blueprints/GameState_Conquest` (`GameplayStatics.GetGameState`) :!pure true))
  (set `/Game/Multiplayer/MultiplayerMaps/Nuketown/Blueprints/GameState_Conquest.CurrentGamemode` "Conquest" _asgame_state_conquest)
  (set `/Game/Multiplayer/MultiplayerMaps/Nuketown/Blueprints/GameState_Conquest.MatchDuration` (`self.MatchDuration`) _asgame_state_conquest)
  (set `/Game/Multiplayer/MultiplayerMaps/Nuketown/Blueprints/GameState_Conquest.TeamLives` (`|MakeArray` _totallives _totallives) _asgame_state_conquest))

(event `self.K2_OnSetMatchState`
  (params (NewState :type Name))
  (if (== NewState "WaitingToStart")
    (for _ (range 1 (+ (- (`self.MatchPlayerCount`) (`self.NumPlayers`)) 1))
      (`self.SpawnPlayerBot`))
    (`self.StartMatch`)))

(fn `BindEventsToDefaultPawn`
  (params (Pawn :type "Actor Object Reference"))
  (bind _returnvalue (`self.GetComponentByClass` Pawn "/Script/TreasuredCove.HealthComponent"))
  (`/Engine/EditorBlueprintResources/StandardMacros.IsValid` _returnvalue
    (:`Is Valid`
      (add `HealthComponent.OnHealthModified` _returnvalue (`|CreateDelegate` :!event `On Player Health Modified`))
      (add `HealthComponent.OnHealthZeroed` _returnvalue (`|CreateDelegate` :!event `On Player Death`)))))

(fn `On Player Death`
  (params (Victim :type "Actor Object Reference") (ResponsibleActor :type "Actor Object Reference"))
  (bind _asplayer_controller (cast `PlayerController` (`self.GetInstigatorController` ResponsibleActor)))
  (bind _asplayer_controller_2 (cast `PlayerController` (`self.GetInstigatorController` Victim)))
  (`self.PlayerKilled` _asplayer_controller_2 _asplayer_controller))

(fn `On Player Health Modified`
  (params (Payload :type "OnAttributeModifiedPayload Structure"))
  (return))

(fn `ReadyToStartMatch`
  (returns (ReturnValue :type Boolean))
  (return (== (`GameplayStatics.GetNumPlayerStates`) (`self.MatchPlayerCount`))))

(fn `SpawnDefaultPawnAtTransform`
  (params (NewPlayer :type "Controller Object Reference") (SpawnTransform :type "Transform Structure (by ref)"))
  (returns (ReturnValue :type "Pawn Object Reference"))
  (bind _returnvalue (`parent.SpawnDefaultPawnAtTransform` NewPlayer SpawnTransform))
  (`|ExecutionSequence`
    (:`then_0`
      (`self.BindEventsToDefaultPawn` _returnvalue))
    (:`then_1`
      (return _returnvalue))))

(fn `SpawnDefaultPawnFor`
  (params (NewPlayer :type "Controller Object Reference") (StartSpot :type "Actor Object Reference"))
  (returns (ReturnValue :type "Pawn Object Reference"))
  (bind _returnvalue (`parent.SpawnDefaultPawnFor` NewPlayer StartSpot))
  (`|ExecutionSequence`
    (:`then_0`
      (`self.BindEventsToDefaultPawn` _returnvalue))
    (:`then_1`
      (return _returnvalue))))

(fn `SpawnPlayerBot`
  (`|ExecutionSequence`
    (:`then_0`
      (bind _returnvalue (`AIBlueprintHelperLibrary.SpawnAIFromClass` (`self.DefaultPawnClass`) null (0.0 0.0 0.0) (struct) true null))
      (bind _returnvalue_2 (`Pawn.GetController` _returnvalue))
      (`/Engine/EditorBlueprintResources/StandardMacros.IsValid` _returnvalue_2
        (:`Is Valid`
          (bind _returnvalue_3 (`self.K2_FindPlayerStart` _returnvalue_2))
          (`self.K2_TeleportTo` _returnvalue (`self.K2_GetActorLocation` _returnvalue_3) (`self.K2_GetActorRotation` _returnvalue_3)))))
    (:`then_1`
      (`/Engine/EditorBlueprintResources/StandardMacros.IncrementInt` (`self.BotCount`)))))

(fn `UserConstructionScript`)